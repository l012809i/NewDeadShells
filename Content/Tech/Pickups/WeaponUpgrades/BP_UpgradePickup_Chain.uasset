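; BP_UpgradePickup_Chain is a weapon upgrade pickup that rolls a random upgrade on BeginPlay, skipping the first enum entry.
; When BP_Player overlaps its box, it looks up that upgrade's row in DT_Upgrades by enum name.
; It passes the row's upgrade Blueprint and the player's weapon slot through an interface message, prints debug text, and destroys itself.
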(event `self.ReceiveBeginPlay`
  (set `self.Upgrade Info` (cast `/Game/Tech/Upgrades/E_Upgradenames` (`KismetMathLibrary.Conv_IntToByte` (`KismetMathLibrary.RandomIntegerInRange` 1 (- (enumcount `/Game/Tech/Upgrades/E_Upgradenames`) 1))))))

(event `self.Box.OnComponentBeginOverlap`
  (params (OverlappedComponent :type "PrimitiveComponent Object Reference") (OtherActor :type "Actor Object Reference") (OtherComp :type "PrimitiveComponent Object Reference") (OtherBodyIndex :type Integer) (bFromSweep :type Boolean) (SweepResult :type "HitResult Structure (by ref)"))
  (bind _weaponslot (`/Game/Tech/Character/BP_Player.WeaponSlot` (cast `/Game/Tech/Character/BP_Player` OtherActor :!pure true)))
  (`KismetSystemLibrary.PrintString` "Overlap happened")
  (if (== (`GameplayStatics.GetObjectClass` OtherActor) "/Game/Tech/Character/BP_Player.BP_Player_C")
    (bind _returnvalue (`|GetDataTableRow` "/Game/Tech/Upgrades/DT_Upgrades.DT_Upgrades" (`KismetStringLibrary.Conv_StringToName` (`|GetEnumeratorNameAsString` (`self.Upgrade Info`))))
      (:`then`
        (bind (_upgradename _upgradeblueprint) (break `/Game/Tech/Upgrades/S_Upgrades` _returnvalue))
        (message `/Game/Tech/Upgrades/BPI_upgradeComponents.I_InitialiseComponent` OtherActor _upgradeblueprint _weaponslot)
        (`KismetSystemLibrary.PrintText` (`|FormatText` "Upgrade {upgrade} applied to slot {x}" (`|GetEnumeratorNameAsString` _upgradename) _weaponslot))
        (`self.K2_DestroyActor`)))))

(fn `UserConstructionScript`)