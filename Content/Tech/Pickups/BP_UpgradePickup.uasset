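; Upgrade pickup that grants the player a random upgrade component when they overlap its box.
; On BeginPlay it picks a random upgrade enum value, skipping the first entry.
; On overlap, that name keys a DT_Upgrades row, whose component class goes to the player through an interface message with a random slot 0 or 1.
; Debug prints re-roll the slot, and the pickup is never destroyed here.
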(event `self.ReceiveBeginPlay`
  (bind _output_get (set `self.Upgrade Info` (cast `/Game/Tech/Upgrades/E_Upgradenames` (`KismetMathLibrary.Conv_IntToByte` (`KismetMathLibrary.RandomIntegerInRange` 1 (- (enumcount `/Game/Tech/Upgrades/E_Upgradenames`) 1))))))
  (`KismetSystemLibrary.PrintString` (`|GetEnumeratorNameAsString` _output_get)))

(event `self.Box.OnComponentBeginOverlap`
  (params (OverlappedComponent :type "PrimitiveComponent Object Reference") (OtherActor :type "Actor Object Reference") (OtherComp :type "PrimitiveComponent Object Reference") (OtherBodyIndex :type Integer) (bFromSweep :type Boolean) (SweepResult :type "HitResult Structure (by ref)"))
  (bind _returnvalue (`KismetMathLibrary.RandomIntegerInRange` 0 1))
  (cast `/Game/Tech/Character/BP_Player` OtherActor)
  (bind _returnvalue_2 (`|GetDataTableRow` "/Game/Tech/Upgrades/DT_Upgrades.DT_Upgrades" (`KismetStringLibrary.Conv_StringToName` (`|GetEnumeratorNameAsString` (`self.Upgrade Info`))))
    (:`then`
      (bind (_upgradename _upgradeblueprint) (break `/Game/Tech/Upgrades/S_Upgrades` _returnvalue_2))
      (message `/Game/Tech/Upgrades/BPI_upgradeComponents.I_InitialiseComponent` OtherActor _upgradeblueprint _returnvalue)
      (`KismetSystemLibrary.PrintString` (`KismetStringLibrary.Concat_StrStr` (`KismetSystemLibrary.GetClassDisplayName` _upgradeblueprint) (`KismetStringLibrary.Conv_IntToString` _returnvalue))))))

(fn `UserConstructionScript`)