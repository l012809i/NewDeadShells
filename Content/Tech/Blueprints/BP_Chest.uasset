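; Chest actor that randomly spawns a weapon pickup shortly after play begins.
; After a short delay, BeginPlay calls SpawnItem, where a random boolean decides whether a BP_WeaponPickup spawns at the Sphere component's world location.
; A disconnected lookup that switches on an existing pickup's Weapon value never runs.
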(event `self.ReceiveBeginPlay`
  (`KismetSystemLibrary.Delay` 2.0)
  (`self.SpawnItem`))

(event `SpawnItem`
  (if (`KismetMathLibrary.RandomBool`)
    (`|SpawnActorFromClass` "/Game/Tech/Weapons/BP_WeaponPickup.BP_WeaponPickup_C" (`KismetMathLibrary.MakeTransform` (`SceneComponent.K2_GetComponentLocation` (`self.Sphere`))) "Undefined" "OverrideRootScale" null null)))

(fn `UserConstructionScript`)