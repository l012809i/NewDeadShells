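; BP_Vendor2 is a hub world vendor that blends the player's camera to itself when interacted with.
; Its Interact event alternates via FlipFlop between blending the view to the vendor and back to the BP_Player found at BeginPlay, while the Interact input action also blends back.
; One-second timers call Posses and Unposses after blends, but both events are empty and the possession nodes are disconnected.
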(event `self.ReceiveBeginPlay`
  (bind _returnvalue (`GameplayStatics.GetActorOfClass` "/Game/Tech/Character/BP_Player.BP_Player_C"))
  (set `self.Player` _returnvalue))

(event `/Game/Tech/HubWorld/BPI_Interact.Interact`
  (`/Engine/EditorBlueprintResources/StandardMacros.FlipFlop`
    (:`A`
      (`PlayerController.SetViewTargetWithBlend` (`GameplayStatics.GetPlayerController` 0) self 1.0 "VTBlend_Linear" 0.0 false)
      (`KismetSystemLibrary.K2_SetTimerDelegate` (delegate `Posses`) 1.0))
    (:`B`
      (`PlayerController.SetViewTargetWithBlend` (`GameplayStatics.GetPlayerController` 0) (`self.Player`) 1.0 "VTBlend_Linear" 0.0 false))))

(event `Posses`)

(event `InputAction|Interact`
  (params (Key :type "Key Structure"))
  (:`Pressed`
    (`PlayerController.SetViewTargetWithBlend` (`GameplayStatics.GetPlayerController` 0) (`self.Player`) 1.0 "VTBlend_Linear" 0.0 false)
    (`KismetSystemLibrary.K2_SetTimerDelegate` (delegate `Unposses`) 1.0)))

(event `Unposses`)

(fn `UserConstructionScript`)