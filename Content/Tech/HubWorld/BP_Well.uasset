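; BP_Well is a hub world well that acts as a camera-driven exit to MainWorld.
; On BeginPlay, a timeline moves the Cube platform toward the Billboard's location.
; When the player first leaves Box, the view blends to the player, Cube collision turns off and exiting is enabled.
; A BPI_Currency actor entering Box1 then blends the view to the well, and chained timers show a transition widget before loading the level.
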(event `self.ReceiveBeginPlay`
  (bind _cube (`self.Cube`))
  (bind (_direction _newtrack_0) (`Timeline|Raise Platform`)
    (:`Update`
      (`SceneComponent.K2_SetWorldLocation` _cube (`KismetMathLibrary.VLerp` (`SceneComponent.K2_GetComponentLocation` _cube) (`SceneComponent.K2_GetComponentLocation` (`self.Billboard`)) _newtrack_0) false false))))

(event `self.Box.OnComponentEndOverlap`
  (params (OverlappedComponent :type "PrimitiveComponent Object Reference") (OtherActor :type "Actor Object Reference") (OtherComp :type "PrimitiveComponent Object Reference") (OtherBodyIndex :type Integer))
  (if (not (`self.CanExit?`))
    (bind _asbp_player (cast `/Game/Tech/Character/BP_Player` OtherActor))
    (`PlayerController.SetViewTargetWithBlend` (`GameplayStatics.GetPlayerController` 0) _asbp_player 1.0 "VTBlend_Linear" 0.0 false)
    (set `self.CanExit?` true)
    (`PrimitiveComponent.SetCollisionEnabled` (`self.Cube`) "NoCollision")))

(event `self.Box1.OnComponentBeginOverlap`
  (params (OverlappedComponent :type "PrimitiveComponent Object Reference") (OtherActor :type "Actor Object Reference") (OtherComp :type "PrimitiveComponent Object Reference") (OtherBodyIndex :type Integer) (bFromSweep :type Boolean) (SweepResult :type "HitResult Structure (by ref)"))
  (if (`KismetSystemLibrary.DoesImplementInterface` OtherActor "/Game/Tech/Currency/BPI_Currency.BPI_Currency_C")
    (if (`self.CanExit?`)
      (`self.chage to well cam`))))

(event `chage to well cam`
  (`PlayerController.SetViewTargetWithBlend` (`GameplayStatics.GetPlayerController` 0) self 2.0 "VTBlend_Linear" 0.0 false)
  (`KismetSystemLibrary.K2_SetTimerDelegate` (delegate `fadeout`) 2.0))

(event `Load Level`
  (`GameplayStatics.OpenLevel` "MainWorld"))

(event `fadeout`
  (bind _returnvalue (`|CreateWidget` "/Game/Tech/UI/W_LevelTransitionOut.W_LevelTransitionOut_C"))
  (`UserWidget.AddToViewport` _returnvalue 0)
  (`KismetSystemLibrary.K2_SetTimerDelegate` (delegate `Load Level`) 1.5))

(fn `UserConstructionScript`)