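; Maestrophone player weapon that grabs an enemy in its aim, drags it at trace range and damages it.
; Activate and deactivate toggle a firing flag, read by a fast looping timer that sphere-traces from the player's projectile spawn.
; A hit enemy switches to swimming movement and snaps to the trace end.
; The miss branch attempts NavWalking restore using the missed trace's hit actor; the multi-trace Hold event is old code.
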(event `Hold`
  (bind _location (.location (`SceneComponent.K2_GetComponentToWorld` (`/Game/Tech/Character/BP_Player.Projectilespawn` (cast `/Game/Tech/Character/BP_Player` (`self.GetOwner`) :!pure true)))))
  (bind _rotation (.rotation (`SceneComponent.K2_GetComponentToWorld` (`/Game/Tech/Character/BP_Player.Projectilespawn` (cast `/Game/Tech/Character/BP_Player` (`self.GetOwner`) :!pure true)))))
  ;[0.2448 0.007135 0] OLD CODE
  (bind _output_get (set `self.Start trace` (+ _location (* _rotation 50.0))))
  (bind _output_get_2 (set `self.EndTrace` (+ _location (* _rotation 1000.0))))
  (bind _outhits (`KismetSystemLibrary.SphereTraceMultiForObjects` :`Start` _output_get :`End` _output_get_2 :`Radius` 50.0 :`ObjectTypes` (`|MakeArray` "ObjectTypeQuery3" :!type "EObjectTypeQuery Enum") :`DrawDebugType` "ForDuration" :`DrawTime` 3.0))
  (for _array_element _outhits
    (bind (_bblockinghit _binitialoverlap _time _distance _location_2 _impactpoint _normal _impactnormal _physmat _hitactor _hitcomponent _hitbonename _bonename _hititem _elementindex _faceindex _tracestart _traceend) (`GameplayStatics.BreakHitResult` _array_element))
    (bind _output_get_3 (set `self.Hit Actor` _hitactor))
    (`self.K2_SetActorLocation` _output_get_3 (+ _tracestart (* (`KismetMathLibrary.Normal` (- _traceend _tracestart)) _distance)) true false)))

(event `self.AlternateActivate`
  ;[0 1 1] Alternate Firing nodes
)

(event `self.AlternateDeactivate`
  ;[0 1 1] Alternate Firing nodes
)

(event `self.ActivateWeapon`
  ;[0 1 1] Add custom firing mechanics here
  (`parent.ActivateWeapon`)
  (set `self.isFiringWeapon` true))

(event `self.DeactivateWeapon`
  (params (`Weapon Switch?` :type Boolean))
  ;[0 1 1] Add custom firing mechanics here
  (`parent.DeactivateWeapon` `Weapon Switch?`)
  (set `self.isFiringWeapon` false))

(event `self.WeaponFunctionality`
  ;[0 0.02951 0.07812] Weapon Functionality
  ; -On Activate set isFiringWeapon bool to True and On Deactivate set isFiringWeapon to False.
  ; -SetTimerByEvent is on Loop acts as event tick and checks if the isFiringWeapon T or F
  ; -Shoots out a SphereLineTraceByChannel from BP_Player > Projectile Spawn Location
  ; -If Enemy hit, Set Enemy Actor Location to End Location of SphereTraceByChannel + Set Movement to Swimming/Flying
  ; -Otherwise put the enemy back to its Last Location and his is back to his Walking Movement
  ;
  ; Now, we need to do it for multiple enemies
  (`KismetSystemLibrary.K2_SetTimerDelegate` (delegate `DrawSphereTrace`) 0.01 true))

(event `DrawSphereTrace`
  (bind _projectilespawn (`/Game/Tech/Character/BP_Player.Projectilespawn` (cast `/Game/Tech/Character/BP_Player` (`self.GetOwner`) :!pure true)))
  (bind _returnvalue (`SceneComponent.K2_GetComponentLocation` _projectilespawn))
  (bind _returnvalue_2 (`KismetMathLibrary.MakeVector` (.x (+ _returnvalue (* (`SceneComponent.GetForwardVector` _projectilespawn) (`self.TraceLength`)))) (.y (+ _returnvalue (* (`SceneComponent.GetForwardVector` _projectilespawn) (`self.TraceLength`)))) (+ (.z (+ _returnvalue (* (`SceneComponent.GetForwardVector` _projectilespawn) (`self.TraceLength`)))) 200.0)))
  ;[0 0.02951 0.07812] Weapon Functionality
  ; -On Activate set isFiringWeapon bool to True and On Deactivate set isFiringWeapon to False.
  ; -SetTimerByEvent is on Loop acts as event tick and checks if the isFiringWeapon T or F
  ; -Shoots out a SphereLineTraceByChannel from BP_Player > Projectile Spawn Location
  ; -If Enemy hit, Set Enemy Actor Location to End Location of SphereTraceByChannel + Set Movement to Swimming/Flying
  ; -Otherwise put the enemy back to its Last Location and his is back to his Walking Movement
  ;
  ; Now, we need to do it for multiple enemies
  (if (`self.isFiringWeapon`)
    (bind (_outhit _returnvalue_3) (`KismetSystemLibrary.SphereTraceSingle` :`Start` (`KismetMathLibrary.MakeVector` (.x _returnvalue) (.y _returnvalue) (+ (.z _returnvalue) 200.0)) :`End` _returnvalue_2 :`Radius` 100.0 :`TraceChannel` "TraceTypeQuery1" :`DrawDebugType` "ForOneFrame" :`DrawTime` 3.0))
    (if _returnvalue_3
      (bind (_bblockinghit _binitialoverlap _time _distance _location _impactpoint _normal _impactnormal _physmat _hitactor) (`GameplayStatics.BreakHitResult` _outhit))
      (bind _returnvalue_4 (`KismetSystemLibrary.DoesImplementInterface` _hitactor "/Game/Tech/Character/Enemies/BPI_BaseEnemy.BPI_BaseEnemy_C"))
      (if _returnvalue_4
        ;;[1 1 1] Take enemy location and set it to End Location of sphereTraceByChannel and it should follow the aim of the player.
        (bind _enemy (message `/Game/Tech/Character/Enemies/BPI_BaseEnemy.I Get BP Base Enemy` _hitactor))
        (set `self.LastLocation` (`self.K2_GetActorLocation` _enemy))
        (`CharacterMovementComponent.SetMovementMode` (`Character.CharacterMovement` _enemy) "MOVE_Swimming" 0)
        (`self.K2_SetActorLocation` _enemy _returnvalue_2 false false)
        (message `/Game/Tech/HealthSystem/BPI_DamageHandling.I_ApplyDamage` _enemy (`self.Damage`) (`self.GetOwner`)))
      (else
        ;;[1 1 1] Leave the enemy alone
        (if _returnvalue_4
          (bind _enemy_2 (message `/Game/Tech/Character/Enemies/BPI_BaseEnemy.I Get BP Base Enemy` _hitactor)) ; Getting EnemyRef
          (`CharacterMovementComponent.SetMovementMode` (`Character.CharacterMovement` _enemy_2) "MOVE_NavWalking" 0)
          (`self.K2_SetActorLocation` _enemy_2 (`self.LastLocation`) false false))))))

(fn `UserConstructionScript`
  (`parent.UserConstructionScript`))