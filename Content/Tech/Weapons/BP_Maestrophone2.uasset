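; Weapon Blueprint for the Maestrophone 2, a child weapon that fires a grab projectile.
; Its firing event spawns BP_Grabprojectile at the owning BP_Player's Projectilespawn transform, ignoring collisions.
; Activation and deactivation defer to the parent class, and alternate fire is empty.
; Damage, healing and horn sound nodes are leftover template pieces that never run.
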(event `self.ActivateWeapon`
  ;[0 1 1] Add custom firing mechanics here
  (`parent.ActivateWeapon`))

(event `self.AlternateActivate`
  ;[0 1 1] Alternate Firing nodes
)

(event `self.AlternateDeactivate`
  ;[0 1 1] Alternate Firing nodes
)

(event `self.DeactivateWeapon`
  (params (`Weapon Switch?` :type Boolean))
  ;[0 1 1] Add custom firing mechanics here
  (`parent.DeactivateWeapon` `Weapon Switch?`))

(event `self.WeaponFunctionality`
  (`|SpawnActorFromClass` "/Game/Tech/Projectiles/BP_Grabprojectile.BP_Grabprojectile_C" (`SceneComponent.K2_GetComponentToWorld` (`/Game/Tech/Character/BP_Player.Projectilespawn` (cast `/Game/Tech/Character/BP_Player` (`self.GetOwner`) :!pure true))) "AlwaysSpawn" "OverrideRootScale" null null))

(fn `UserConstructionScript`
  (`parent.UserConstructionScript`))