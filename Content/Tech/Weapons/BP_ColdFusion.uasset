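; Cold Fusion charge-up weapon that fires only if the trigger is held until the charge completes.
; Activation starts a one-shot timer of 1/FireRate seconds, while deactivation cancels it, with debug prints for both.
; Firing calls UpgradeProjectileShoot on every BPC_BaseUpgrade component, passing projectile type, damage and the BPC_ChainLightning components.
; A DoOnce gates the charge sound and resets only after a shot, so cancelled charges do not re-arm it.
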(event `self.ActivateWeapon`
  ;[0 1 1] On left click - start charging the weapon shot (left click must be held) - shoot if charge completes
  (`KismetSystemLibrary.PrintText` (`|FormatText` "Charge of {time}s started" (/ 1.0 (`.FireRate_27_CAE65EA0450609A315897D810B56FE4E` (break `/Game/Tech/Weapons/WeaponInfo/WeaponInformation` (`self.WeaponInformation`))))) true true (struct :`G` 0.66 :`B` 1.0 :`A` 1.0) 3.0)
  (bind _returnvalue (`KismetSystemLibrary.K2_SetTimerDelegate` (`|CreateDelegate` :!event `WeaponFunctionality`) (/ 1.0 (`.FireRate_27_CAE65EA0450609A315897D810B56FE4E` (break `/Game/Tech/Weapons/WeaponInfo/WeaponInformation` (`self.WeaponInformation`))))))
  (set `self.ChargeTimer` _returnvalue)
  (`/Engine/EditorBlueprintResources/StandardMacros.DoOnce` false :!label _label
    (:`Completed`
      (`GameplayStatics.PlaySound2D` "/Game/Tech/Sounds/ColdFusion/charge_up2.charge_up2" 1.0 1.0 0.0 null null))))

(event `self.DeactivateWeapon`
  (params (`Weapon Switch?` :type Boolean))
  (bind _chargetimer (`self.ChargeTimer`))
  ;[0 1 1] On release left click/swap weapon - cancel all charge
  (if (`KismetSystemLibrary.K2_IsValidTimerHandle` _chargetimer)
    (`KismetSystemLibrary.PrintText` (`|FormatText` "Charge cancelled at {time}s" (`KismetSystemLibrary.K2_GetTimerElapsedTimeHandle` _chargetimer)) true true (struct :`G` 0.66 :`B` 1.0 :`A` 1.0) 3.0))
  (`KismetSystemLibrary.K2_ClearAndInvalidateTimerHandle` (`self.ChargeTimer`)))

(event `self.WeaponFunctionality`
  ;[0 1 1] Shoot
  (`KismetSystemLibrary.K2_ClearAndInvalidateTimerHandle` (`self.ChargeTimer`))
  (`self.ChargeShot`)
  (goto _label :!via `Reset`))

(event `ChargeShot`
  ;[0 1 1] ChargeShot Graph
  (for _array_element (`self.K2_GetComponentsByClass` "/Game/Tech/Upgrades/BPC_BaseUpgrade.BPC_BaseUpgrade_C")
    (`/Game/Tech/Upgrades/BPC_BaseUpgrade.Upgrade_ProjectileShoot` _array_element 0.0 (`self.ProjectileType`) (`self.F_GetDamage`) (`self.K2_GetComponentsByClass` "/Game/Tech/Upgrades/BPC_ChainLightning.BPC_ChainLightning_C"))))

(fn `UserConstructionScript`
  (`parent.UserConstructionScript`))