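; Sea Katana weapon Blueprint, a child weapon that runs a melee combo of two basic attacks followed by a long-range one.
; An attack counter picks the attack and its reach, and both share one debug-drawn forward sphere trace from the player.
; Every hit receives damage through an interface message, then the player teleports just beyond the last actor hit.
; Alternate fire is empty.
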(event `self.ActivateWeapon`
  ;[0 1 1] Add custom firing mechanics here
  (`parent.ActivateWeapon`))

(event `self.AlternateActivate`
  ;[0 1 1] Alternate Firing nodes
)

(event `self.AlternateDeactivate`
  ;[0 1 1] Alternate Firing nodes
)

(event `self.DeactivateWeapon`
  (params (`Weapon Switch?` :type Boolean))
  ;[0 1 1] Add custom firing mechanics here
  (`parent.DeactivateWeapon` `Weapon Switch?`))

(event `self.WeaponFunctionality`
  (bind _returnvalue (`GameplayStatics.GetActorOfClass` "/Game/Tech/Character/BP_Player.BP_Player_C"))
  (set `self.Player` _returnvalue)
  (if (>= (`self.AttackCount`) 2)
    (set `self.Distance` 500.0)
    (`self.LongAttack`)
    (else
      (set `self.Distance` 250.0)
      (`self.BasicAttack`))))

(event `BasicAttack`
  (bind _rootcomponent (`Actor.RootComponent` (`self.Player`)))
  (bind _rootcomponent_2 (`Actor.RootComponent` (`self.Player`)))
  (bind _returnvalue (`SceneComponent.K2_GetComponentLocation` _rootcomponent_2))
  (set `self.AttackCount` (+ (`self.AttackCount`) 1))
  (`KismetSystemLibrary.PrintString` "BasicAttack")
  (bind _outhits (`KismetSystemLibrary.SphereTraceMultiForObjects` _returnvalue (+ _returnvalue (* (`SceneComponent.GetForwardVector` _rootcomponent_2) (`self.Distance`))) 125.0 (`self.Object Types`) false (`|MakeArray` (`self.Player`) :!type "Actor Object Reference") "ForDuration" :!label _label))
  (for (_array_element _array_index) _outhits
    (bind (_bblockinghit _binitialoverlap _time _distance _location _impactpoint _normal _impactnormal _physmat _hitactor) (`GameplayStatics.BreakHitResult` _array_element))
    (message `/Game/Tech/HealthSystem/BPI_DamageHandling.I_ApplyDamage` _hitactor (`self.F_GetDamage`) null)
    (if (== _array_index (`KismetArrayLibrary.Array_LastIndex` _outhits))
      (`SceneComponent.K2_SetWorldLocation` _rootcomponent (+ (`self.K2_GetActorLocation` _hitactor) (* (`SceneComponent.GetForwardVector` _rootcomponent) 150.0)) false true))))

(event `LongAttack`
  (set `self.AttackCount` 0)
  (`KismetSystemLibrary.PrintString` "Long attack")
  (goto _label))

(fn `UserConstructionScript`
  (`parent.UserConstructionScript`))