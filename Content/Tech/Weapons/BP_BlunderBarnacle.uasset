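; Blunderbarnacle player weapon, a child weapon Blueprint with primary and alternate fire inputs that both pass to the parent's activate and deactivate logic.
; WeaponFunctionality ignores the SingleShot flag and flip-flops between six inaccurate buckshot rounds splitting the damage and one full-damage piercing projectile.
; Projectiles fire through BPC_BaseUpgrade components, passing chain lightning components as shot upgrades.
; Debug-drawn hitscan single and spread shot events also exist, uncalled within this graph.
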(event `self.ActivateWeapon`
  ;[0 1 1] On fire - do shot type
  (set `self.SingleShot?` true)
  (`parent.ActivateWeapon` :!label _label))

(event `self.DeactivateWeapon`
  (params (`Weapon Switch?` :type Boolean))
  ;[0 1 1] Deactivate to start cooldown
  (`parent.DeactivateWeapon` false :!label _label_2))

(event `self.AlternateDeactivate`
  ;[0 1 1] Deactivate to start cooldown
  (goto _label_2))

(event `self.AlternateActivate`
  ;[0 1 1] On fire - do shot type
  (set `self.SingleShot?` false)
  (goto _label))

(event `SingleShot`
  (bind _projectilespawn (`/Game/Tech/Character/BP_Player.Projectilespawn` (cast `/Game/Tech/Character/BP_Player` (`self.GetOwner`) :!pure true)))
  (bind _returnvalue (`SceneComponent.K2_GetComponentLocation` _projectilespawn))
  (bind _outhits (`KismetSystemLibrary.LineTraceMultiForObjects` _returnvalue (+ _returnvalue (* (`SceneComponent.GetForwardVector` _projectilespawn) 1000.0)) (`|MakeArray` "ObjectTypeQuery3" "ObjectTypeQuery1" "ObjectTypeQuery2" :!type "EObjectTypeQuery Enum") false (`|MakeArray` (`self.GetOwner`)) "ForDuration" true (struct :`R` 1.0 :`A` 1.0) (struct :`G` 1.0 :`A` 1.0) 2.0))
  (for _array_element _outhits
    (bind (_bblockinghit _binitialoverlap _time _distance _location _impactpoint _normal _impactnormal _physmat _hitactor _hitcomponent) (`GameplayStatics.BreakHitResult` _array_element))
    (if (`|EnumInequality` (`PrimitiveComponent.GetCollisionObjectType` _hitcomponent) "ECC_Pawn")
      (break)
      (elif (== (`KismetArrayLibrary.Array_Find` (`self.Hit Actor`) _hitactor) -1)
        (`KismetArrayLibrary.Array_Add` (`self.Hit Actor`) _hitactor)
        (message `/Game/Tech/HealthSystem/BPI_DamageHandling.I_ApplyDamage` _hitactor (`self.F_GetDamage`) (`self.GetOwner`)))))
  (`KismetArrayLibrary.Array_Clear` (`self.Hit Actor`)))

(event `Spreadshot`
  (bind _projectilespawn (`/Game/Tech/Character/BP_Player.Projectilespawn` (cast `/Game/Tech/Character/BP_Player` (`self.GetOwner`) :!pure true)))
  (bind (_returnvalue_x _returnvalue_y _returnvalue_z) (`KismetMathLibrary.BreakVector` (`SceneComponent.K2_GetComponentLocation` _projectilespawn)))
  (bind _returnvalue (`SceneComponent.K2_GetComponentLocation` _projectilespawn))
  (bind (_returnvalue_x_2 _returnvalue_y_2) (`KismetMathLibrary.BreakVector` (+ _returnvalue (* (`KismetMathLibrary.RandomUnitVectorInConeInDegrees` (`SceneComponent.GetForwardVector` _projectilespawn) 30.0) 500.0))))
  (for _ (range 1 11)
    (bind _outhits (`KismetSystemLibrary.LineTraceMultiForObjects` _returnvalue (`KismetMathLibrary.MakeVector` _returnvalue_x_2 _returnvalue_y_2 _returnvalue_z) (`|MakeArray` "ObjectTypeQuery3" "ObjectTypeQuery1" "ObjectTypeQuery2" :!type "EObjectTypeQuery Enum") false (`|MakeArray` (`self.GetOwner`)) "ForDuration" true (struct :`R` 1.0 :`A` 1.0) (struct :`G` 1.0 :`A` 1.0) 2.0))
    (for _array_element _outhits
      (bind (_bblockinghit _binitialoverlap _time _distance _location _impactpoint _normal _impactnormal _physmat _hitactor _hitcomponent) (`GameplayStatics.BreakHitResult` _array_element))
      (if (`|EnumInequality` (`PrimitiveComponent.GetCollisionObjectType` _hitcomponent) "ECC_Pawn")
        (break)
        (elif (== (`KismetArrayLibrary.Array_Find` (`self.Hit Actor`) _hitactor) -1)
          (`KismetArrayLibrary.Array_Add` (`self.Hit Actor`) _hitactor)
          (message `/Game/Tech/HealthSystem/BPI_DamageHandling.I_ApplyDamage` _hitactor (`self.F_GetDamage`) (`self.GetOwner`)))))
    (`KismetArrayLibrary.Array_Clear` (`self.Hit Actor`))))

(event `self.WeaponFunctionality`
  (`/Engine/EditorBlueprintResources/StandardMacros.FlipFlop`
    (:`A`
      (bind _output_get (set `self.ProjectileType` "/Game/Tech/Projectiles/NewProjectiles/BP_Buckshot.BP_Buckshot_C"))
      (for _ (range 1 7)
        (for _array_element (`self.K2_GetComponentsByClass` "/Game/Tech/Upgrades/BPC_BaseUpgrade.BPC_BaseUpgrade_C")
          (`/Game/Tech/Upgrades/BPC_BaseUpgrade.Upgrade_ProjectileShoot` _array_element 15.0 _output_get (/ (`self.F_GetDamage`) 6.0) (`self.K2_GetComponentsByClass` "/Game/Tech/Upgrades/BPC_ChainLightning.BPC_ChainLightning_C")))))
    (:`B`
      (bind _output_get_2 (set `self.ProjectileType` "/Game/Tech/Projectiles/NewProjectiles/BP_PiercingProjectile.BP_PiercingProjectile_C"))
      (for _array_element_2 (`self.K2_GetComponentsByClass` "/Game/Tech/Upgrades/BPC_BaseUpgrade.BPC_BaseUpgrade_C")
        (`/Game/Tech/Upgrades/BPC_BaseUpgrade.Upgrade_ProjectileShoot` _array_element_2 0.0 _output_get_2 (`self.F_GetDamage`) (`self.K2_GetComponentsByClass` "/Game/Tech/Upgrades/BPC_ChainLightning.BPC_ChainLightning_C"))))))

(fn `UserConstructionScript`
  (`parent.UserConstructionScript`))