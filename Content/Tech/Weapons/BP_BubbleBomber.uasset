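; Bubble Bomber weapon that fires more projectiles per shot the longer it stays active.
; Each shot loops over the current bubble count, telling every upgrade component to shoot an inaccurate projectile with the weapon's damage and any Chain Lightning components as shot upgrades.
; After a short delay the count rises up to a small cap, and deactivating the weapon resets it to one.
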(event `self.DeactivateWeapon`
  (params (`Weapon Switch?` :type Boolean))
  ;[0.9922 0.6667 1] Starting and stopping shooting
  (`parent.DeactivateWeapon` false)
  (set `self.Bubblecount` 1))

(event `self.WeaponFunctionality`
  ;[0.9922 0.6667 1] Starting and stopping shooting
  ;[0.9922 0.6667 1] Increases the amount of bubbles fired with each shot
  (for _ (range 1 (+ (`self.Bubblecount`) 1))
    (for _array_element (`self.K2_GetComponentsByClass` "/Game/Tech/Upgrades/BPC_BaseUpgrade.BPC_BaseUpgrade_C")
      (`/Game/Tech/Upgrades/BPC_BaseUpgrade.Upgrade_ProjectileShoot` _array_element 15.0 (`self.ProjectileType`) (`self.F_GetDamage`) (`self.K2_GetComponentsByClass` "/Game/Tech/Upgrades/BPC_ChainLightning.BPC_ChainLightning_C"))))
  (`KismetSystemLibrary.Delay` 1.0)
  (bind _result (`/Engine/EditorBlueprintResources/StandardMacros.IncrementInt` (`self.Bubblecount`))
    (:`  `
      (set `self.Bubblecount` (`KismetMathLibrary.Clamp` _result 1 3)))))

(fn `UserConstructionScript`
  (`parent.UserConstructionScript`))