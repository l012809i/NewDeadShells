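; Base weapon Blueprint that provides automatic firing, stats and damage for child weapons, which override WeaponFunctionality and alternate-fire events.
; The construction script finds the DT_Weapons row matching its own class to set WeaponInformation and mesh.
; Activation fires immediately and starts a looping FireRate timer; deactivation delays clearing it by the remaining interval, gating re-fire.
; FGetDamage rolls critical hits from those stats.
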(event `ActivateWeapon`
  ;[0 1 1] Activate Weapon - On activate start firing, if held down fully automatic fire will occur
  (if (== (`KismetSystemLibrary.K2_GetTimerRemainingTimeHandle` (`self.FireRateTimer`)) 0.0)
    (`self.WeaponFunctionality`)
    (bind _returnvalue (`KismetSystemLibrary.K2_SetTimerDelegate` (`|CreateDelegate` :!event `WeaponFunctionality`) (/ 1.0 (`.FireRate_27_CAE65EA0450609A315897D810B56FE4E` (break `/Game/Tech/Weapons/WeaponInfo/WeaponInformation` (`self.WeaponInformation`)))) true))
    (set `self.FireRateTimer` _returnvalue)))

(event `DeactivateWeapon`
  (params (`Weapon Switch?` :type Boolean))
  (bind _fireratetimer (`self.FireRateTimer`))
  ;[0 1 1] Deactivate Weapon - Stop fully automatic fire
  (`KismetSystemLibrary.Delay` (`KismetSystemLibrary.K2_GetTimerRemainingTimeHandle` _fireratetimer))
  (`KismetSystemLibrary.K2_ClearAndInvalidateTimerHandle` _fireratetimer))

(event `AlternateActivate`
  ;[0 1 1] Right click events for alternate fire
)

(event `AlternateDeactivate`
  ;[0 1 1] Right click events for alternate fire
)

(event `WeaponFunctionality`
  ;[0 1 1] WeaponFunctionality for child blueprints
)

(event `self.I_DestroyComponent`
  (params (Component :type "ActorComponent Object Reference"))
  (`ActorComponent.K2_DestroyComponent` Component))

(fn `F_GetDamage`
  (returns (Damage :type "Float (double-precision)"))
  (bind _weaponinformation (`self.WeaponInformation`))
  (bind ((`AttackPower_29_83DD24E64DC0231FDA6E81A1723EB3F5` _attackpower) (`CriticalDamage_16_C3B73A1D41CF74641D8A029EA31D2A61` _criticaldamage)) (break `/Game/Tech/Weapons/WeaponInfo/WeaponInformation` _weaponinformation))
  ;[0 1 1] Damage Calculation Function
  ; NON CRIT = ATK
  ; CRIT = ATK * CRIT DAMAGE
  (return (`KismetMathLibrary.SelectFloat` (* _attackpower (+ (/ _criticaldamage 100.0) 1.0)) _attackpower (>= (`.CriticalRate_15_045B7F2C4D91BCDF30C36D98417B5FFC` (break `/Game/Tech/Weapons/WeaponInfo/WeaponInformation` _weaponinformation)) (`KismetMathLibrary.RandomFloatInRange` 0.0 100.0)))))

(fn `UserConstructionScript`
  (bind _outrownames (`DataTableFunctionLibrary.GetDataTableRowNames` "/Game/Tech/Weapons/DT_Weapons.DT_Weapons"))
  (for _array_element _outrownames
    (bind _returnvalue (`|GetDataTableRow` "/Game/Tech/Weapons/DT_Weapons.DT_Weapons" _array_element)
      (:`then`
        (bind ((`WeaponMesh_17_79AEC6A248F23E731AEC6A8F2697B164` _weaponmesh) (`WeaponBlueprint_32_8A2FB0DD4C47CCCE3886D7BFCACBCC41` _weaponblueprint)) (break `/Game/Tech/Weapons/WeaponInfo/WeaponInformation` _returnvalue))
        (if (== _weaponblueprint (`GameplayStatics.GetObjectClass` self))
          (set `self.WeaponInformation` _returnvalue)
          (`StaticMeshComponent.SetStaticMesh` (`self.SM_Weapon`) _weaponmesh))))))