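; Fish sword melee weapon with a normal attack and a double-damage charged attack, gated by a fire-rate cooldown.
; Activation starts a one-second charge timer that auto-fires the charged attack on completion; early release gives a normal attack with sound, while weapon switching cancels the charge.
; Both attacks use a placeholder debug sphere trace around the owner, damaging each unique pawn once through an interface message.
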(event `self.ActivateWeapon`
  ;[0 1 1] Start Charging Weapon on Left click
  (if (== (`KismetSystemLibrary.K2_GetTimerRemainingTimeHandle` (`self.CooldownTimer`)) 0.0)
    (set `self.Released?` true)
    (`KismetSystemLibrary.PrintString` "charge started")
    (bind _returnvalue (`KismetSystemLibrary.K2_SetTimerDelegate` (delegate `AttackWithWeapon`) 1.0))
    (set `self.ChargeTimer` _returnvalue)
    (else
      (`KismetSystemLibrary.PrintString` "On Cooldown")
      (set `self.Released?` false))))

(event `AttackWithWeapon`
  ;[0 1 1] Start Charging Weapon on Left click
  (`self.DeactivateWeapon` false))

(event `self.DeactivateWeapon`
  (params (`Weapon Switch?` :type Boolean))
  ;[0 1 1] On Release - check if weapon isn't being swapped, button is held and if the weapon is on CD. If false - clear charge. If true - Attack and start cooldown.
  (if (and (not `Weapon Switch?`) (`self.Released?`) (== (`KismetSystemLibrary.K2_GetTimerRemainingTimeHandle` (`self.CooldownTimer`)) 0.0))
    (`self.WeaponFunctionality`)
    (bind _returnvalue (`KismetSystemLibrary.K2_SetTimerDelegate` (delegate `ClearCooldown`) (/ 1.0 (`.FireRate_27_CAE65EA0450609A315897D810B56FE4E` (break `/Game/Tech/Weapons/WeaponInfo/WeaponInformation` (`self.WeaponInformation`))))))
    (set `self.CooldownTimer` _returnvalue)
    (`KismetSystemLibrary.K2_ClearAndInvalidateTimerHandle` (`self.ChargeTimer`))
    (else
      (`KismetSystemLibrary.K2_ClearAndInvalidateTimerHandle` (`self.ChargeTimer`)))))

(event `ClearCooldown`
  ;[0 1 1] On Release - check if weapon isn't being swapped, button is held and if the weapon is on CD. If false - clear charge. If true - Attack and start cooldown.
  (`KismetSystemLibrary.K2_ClearAndInvalidateTimerHandle` (`self.CooldownTimer`)))

(event `ChargeAttack`
  ;[0 1 1] Charge Attack - 2x damage. Normal attack 1x damage
  (`KismetSystemLibrary.PrintString` "charge attack")
  (`self.DealDamage - Debug` 2.0))

(event `self.WeaponFunctionality`
  (bind _chargetimer (`self.ChargeTimer`))
  ;[0 1 1] WeaponFunc - check charge - If charged. Charge attack, else do normal attack
  (if (and (== (`KismetSystemLibrary.K2_GetTimerRemainingTimeHandle` _chargetimer) 0.0) (`KismetSystemLibrary.K2_IsValidTimerHandle` _chargetimer))
    (`self.ChargeAttack`)
    (set `self.Released?` false)
    (else
      (`self.NormalAttack`)
      (`GameplayStatics.PlaySound2D` "/Game/Tech/Sounds/FishSword/FishSword_cue.FishSword_cue" 1.0 1.0 0.0 null null))))

(event `NormalAttack`
  ;[0 1 1] Charge Attack - 2x damage. Normal attack 1x damage
  (`KismetSystemLibrary.PrintString` "normal attack")
  (`self.DealDamage - Debug` 1.0))

(event `DealDamage - Debug`
  (params (DamageMult :type "Float (double-precision)"))
  (bind _returnvalue (`self.GetOwner`))
  (bind _returnvalue_2 (`self.K2_GetActorLocation` _returnvalue))
  ;[1 0 0] Damage Sphere - Will be replaced soon when mesh and anims are implemented
  (`KismetArrayLibrary.Array_Clear` (`self.ActorsHit`))
  (bind _outhits (`KismetSystemLibrary.SphereTraceMultiForObjects` _returnvalue_2 _returnvalue_2 400.0 (`|MakeArray` "ObjectTypeQuery3" :!type "EObjectTypeQuery Enum") false (`|MakeArray` _returnvalue) "ForDuration"))
  (for _array_element _outhits
    (bind (_bblockinghit _binitialoverlap _time _distance _location _impactpoint _normal _impactnormal _physmat _hitactor) (`GameplayStatics.BreakHitResult` _array_element))
    (if (== (`KismetArrayLibrary.Array_Find` (`self.ActorsHit`) _hitactor) -1)
      (`KismetArrayLibrary.Array_AddUnique` (`self.ActorsHit`) _hitactor)
      (message `/Game/Tech/HealthSystem/BPI_DamageHandling.I_ApplyDamage` _hitactor (* DamageMult (`self.F_GetDamage`)) (`self.GetOwner`)))))

(fn `UserConstructionScript`
  (`parent.UserConstructionScript`))