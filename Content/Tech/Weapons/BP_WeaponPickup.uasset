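; Weapon pickup actor that offers its selected weapon to any actor overlapping its sphere.
; The construction script uses the weapon enum as a DT_Weapons row name to load the weapon data and set the mesh.
; On overlap it sends the weapon class to the other actor through a pickup interface call, destroying itself only on success.
; Its own inventory and pickup interface functions are stubs returning false.
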(event `SpawnInformation`
  (params (`Weapon Name` :type "/Game/Tech/Weapons/E_WeaponNames Enum" :default "NewEnumerator4"))
  (bind _returnvalue (`|GetDataTableRow` "/Game/Tech/Weapons/DT_Weapons.DT_Weapons" (`KismetStringLibrary.Conv_StringToName` (`|GetEnumeratorNameAsString` `Weapon Name`)))
    (:`then`
      (bind _output_get (set `self.Weapon Information` _returnvalue))
      (`StaticMeshComponent.SetStaticMesh` (`self.StaticMesh`) (`.WeaponMesh_17_79AEC6A248F23E731AEC6A8F2697B164` (break `/Game/Tech/Weapons/WeaponInfo/WeaponInformation` _output_get))))))

(event `self.Sphere.OnComponentBeginOverlap`
  (params (OverlappedComponent :type "PrimitiveComponent Object Reference") (OtherActor :type "Actor Object Reference") (OtherComp :type "PrimitiveComponent Object Reference") (OtherBodyIndex :type Integer) (bFromSweep :type Boolean) (SweepResult :type "HitResult Structure (by ref)"))
  ;[0 1 1] On Overlap - Make the target pick up the weapon - If success destroy self
  (bind _picked_up_ (message `/Game/Tech/Weapons/WeaponInfo/BPI_WeaponPickup.I_PickUpWeapon` OtherActor (`.WeaponBlueprint_32_8A2FB0DD4C47CCCE3886D7BFCACBCC41` (break `/Game/Tech/Weapons/WeaponInfo/WeaponInformation` (`self.Weapon Information`))) 0))
  (if _picked_up_
    (`self.K2_DestroyActor`)))

(fn `I_CheckDuplicateWeapon`
  (params (`Weapon Class` :type "/Game/Tech/Weapons/WeaponInfo/BP_BaseWeapon Class Reference"))
  (returns (`Duplicate?` :type Boolean))
  (return false))

(fn `I_CheckFullInventory`
  (returns (`Full?` :type Boolean))
  (return false))

(fn `I_PickUpWeapon`
  (params (`Weapon Class` :type "/Game/Tech/Weapons/WeaponInfo/BP_BaseWeapon Class Reference") (`Item Slot` :type Integer))
  (returns (`Picked Up?` :type Boolean))
  (return false))

(fn `UserConstructionScript`
  (`self.SpawnInformation` (`self.Weapon`)))