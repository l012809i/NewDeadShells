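; Shell Axe melee weapon that runs a combo of horizontal swings ending in a downward crush, which restarts the sequence.
; An attack counter picks Swing or Crush, each playing a montage on the owner's mesh at a rate scaled by relative attack speed.
; Each hands its attack class, damage and ChainLightning components to every BaseUpgrade component via UpgradeMeleeSwing, with Crush adding a short scaled delay.
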(event `self.WeaponFunctionality`
  ;[0 1 1] WeaponFunc - check sequence for what attack to do.
  (if (< (`self.AttackSequence`) 3)
    (`self.Swing`)
    (else
      (`self.Crush`))))

(event `Swing`
  (`/Engine/EditorBlueprintResources/StandardMacros.IncrementInt` (`self.AttackSequence`)
    (:`  `
      (bind _mesh (message `/Game/Tech/Character/BPI_GetCharacterMesh.GetPlayerMesh` (`self.GetOwner`)))
      (`|PlayMontage` _mesh "/Game/Tech/Character/FinalMainCharacter/Animations/MeleeAnimations/Melee_Attack_Horizontal_Montage.Melee_Attack_Horizontal_Montage" (/ 1.0 (`self.RelativeAtkSpd`)) 0.75
        (:`then`
          (for _array_element (`self.K2_GetComponentsByClass` "/Game/Tech/Upgrades/BPC_BaseUpgrade.BPC_BaseUpgrade_C")
            (`/Game/Tech/Upgrades/BPC_BaseUpgrade.Upgrade_MeleeSwing` _array_element "/Game/Tech/MeleeAttacks/BP_ShellAxeSwing.BP_ShellAxeSwing_C" (`self.F_GetDamage`) (`self.K2_GetComponentsByClass` "/Game/Tech/Upgrades/BPC_ChainLightning.BPC_ChainLightning_C"))))))))

(event `Crush`
  (set `self.AttackSequence` 1)
  (bind _mesh (message `/Game/Tech/Character/BPI_GetCharacterMesh.GetPlayerMesh` (`self.GetOwner`)))
  (`|PlayMontage` _mesh "/Game/Tech/Character/FinalMainCharacter/Animations/MeleeAnimations/Melee_Attack_Downward_Montage.Melee_Attack_Downward_Montage" (/ 1.15 (`self.RelativeAtkSpd`)) 0.55
    (:`then`
      (`KismetSystemLibrary.Delay` (/ 0.15 (`self.RelativeAtkSpd`)))
      (for _array_element (`self.K2_GetComponentsByClass` "/Game/Tech/Upgrades/BPC_BaseUpgrade.BPC_BaseUpgrade_C")
        (`/Game/Tech/Upgrades/BPC_BaseUpgrade.Upgrade_MeleeSwing` _array_element "/Game/Tech/MeleeAttacks/BP_ShellAxeCrush.BP_ShellAxeCrush_C" (`self.F_GetDamage`) (`self.K2_GetComponentsByClass` "/Game/Tech/Upgrades/BPC_ChainLightning.BPC_ChainLightning_C"))))))

(fn `UserConstructionScript`
  (`parent.UserConstructionScript`))