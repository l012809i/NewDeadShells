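; BP_Buckshot is a short-range projectile that destroys itself shortly after its projectile movement activates.
; When its collision sphere hits anything other than BP_Player, it sends damage and knockback interface messages along its forward direction, then destroys itself.
; If the damage message reports a hit target, it notifies each of its own BPC_BaseUpgrade components with damage and location.
; GetFreeze always returns false.
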(event `self.ProjectileMovement.OnComponentActivated`
  (params (Component :type "ActorComponent Object Reference") (bReset :type Boolean))
  (`KismetSystemLibrary.Delay` 0.2)
  (`self.K2_DestroyActor`))

(event `self.Sphere_Col.OnComponentHit`
  (params (HitComponent :type "PrimitiveComponent Object Reference") (OtherActor :type "Actor Object Reference") (OtherComp :type "PrimitiveComponent Object Reference") (NormalImpulse :type "Vector Structure") (Hit :type "HitResult Structure (by ref)"))
  (if (!= (`GameplayStatics.GetObjectClass` OtherActor) "/Game/Tech/Character/BP_Player.BP_Player_C")
    (bind _target_hit_ (message `/Game/Tech/HealthSystem/BPI_DamageHandling.I_ApplyDamage` OtherActor (`self.Damage`) (`self.GetOwner`)))
    (message `/Game/Tech/Projectiles/NewProjectiles/BPI_ProjectileInterface.ApplyKnockback` OtherActor (`SceneComponent.GetForwardVector` (`self.SM_projectile`)) 600.0)
    (if _target_hit_
      (for _array_element (`self.K2_GetComponentsByClass` "/Game/Tech/Upgrades/BPC_BaseUpgrade.BPC_BaseUpgrade_C")
        (`/Game/Tech/Upgrades/BPC_BaseUpgrade.Upgrade_HitEnemy` _array_element (`self.Damage`) (`self.K2_GetActorLocation`))))
    (`self.K2_DestroyActor`)))

(fn `Get freeze`
  (returns (Frozen :type Boolean))
  (return false))

(fn `UserConstructionScript`
  (`parent.UserConstructionScript`))