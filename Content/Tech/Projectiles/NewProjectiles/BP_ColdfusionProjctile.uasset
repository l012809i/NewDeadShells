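; Coldfusion projectile that freezes enemies on impact and deals bonus damage to targets that are already frozen.
; On a sphere hit with anything but the player, it queries the target's freeze state through interface messages, then either doubles damage or applies a timed freeze before dealing damage.
; A confirmed hit notifies the projectile's upgrade components with damage and location; the projectile then destroys itself.
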(event `self.Sphere_Col.OnComponentHit`
  (params (HitComponent :type "PrimitiveComponent Object Reference") (OtherActor :type "Actor Object Reference") (OtherComp :type "PrimitiveComponent Object Reference") (NormalImpulse :type "Vector Structure") (Hit :type "HitResult Structure (by ref)"))
  (if (!= (`GameplayStatics.GetObjectClass` OtherActor) "/Game/Tech/Character/BP_Player.BP_Player_C")
    (bind _frozen (message `/Game/Tech/Projectiles/NewProjectiles/BPI_ProjectileInterface.Get freeze` OtherActor))
    (if _frozen
      (bind _output_get (set `self.Damage` (* (`self.Damage`) 2.0)))
      (bind _target_hit_ (message `/Game/Tech/HealthSystem/BPI_DamageHandling.I_ApplyDamage` OtherActor _output_get null))
      (else
        (message `/Game/Tech/Projectiles/NewProjectiles/BPI_ProjectileInterface.Freeze enemies` OtherActor 2.0)
        (bind _target_hit__2 (message `/Game/Tech/HealthSystem/BPI_DamageHandling.I_ApplyDamage` OtherActor (`self.Damage`) null))))
    (if (or _target_hit_ _target_hit__2)
      (for _array_element (`self.K2_GetComponentsByClass` "/Game/Tech/Upgrades/BPC_BaseUpgrade.BPC_BaseUpgrade_C")
        (`/Game/Tech/Upgrades/BPC_BaseUpgrade.Upgrade_HitEnemy` _array_element (`self.Damage`) (`self.K2_GetActorLocation`))))
    (`self.K2_DestroyActor`)))

(fn `Get freeze`
  (returns (Frozen :type Boolean))
  (return false))

(fn `UserConstructionScript`
  (`parent.UserConstructionScript`))