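; BP_PiercingProjectile is a projectile that passes through damageable targets instead of stopping on the first hit.
; On sphere overlap it ignores actors of its own class and sends others a damage interface message, with its owner as instigator.
; A registered hit notifies every BPC_BaseUpgrade component on the projectile through UpgradeHitEnemy.
; Otherwise the projectile destroys itself, so only non-target overlaps end its flight here.
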(event `self.Sphere_Col.OnComponentBeginOverlap`
  (params (OverlappedComponent :type "PrimitiveComponent Object Reference") (OtherActor :type "Actor Object Reference") (OtherComp :type "PrimitiveComponent Object Reference") (OtherBodyIndex :type Integer) (bFromSweep :type Boolean) (SweepResult :type "HitResult Structure (by ref)"))
  (if (!= (`GameplayStatics.GetObjectClass` OtherActor) (`GameplayStatics.GetObjectClass` self))
    (bind _target_hit_ (message `/Game/Tech/HealthSystem/BPI_DamageHandling.I_ApplyDamage` OtherActor (`self.Damage`) (`self.GetOwner`)))
    (if _target_hit_
      (for _array_element (`self.K2_GetComponentsByClass` "/Game/Tech/Upgrades/BPC_BaseUpgrade.BPC_BaseUpgrade_C")
        (`/Game/Tech/Upgrades/BPC_BaseUpgrade.Upgrade_HitEnemy` _array_element (`self.Damage`)))
      (else
        (`self.K2_DestroyActor`)))))

(fn `UserConstructionScript`
  (`parent.UserConstructionScript`))