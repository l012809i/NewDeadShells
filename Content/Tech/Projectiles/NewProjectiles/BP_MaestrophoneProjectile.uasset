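; Maestrophone projectile that damages and displaces pawns around it as it travels.
; Once projectile movement activates, a looping timer runs a sphere trace at the collision sphere, ignoring the player and anything already hit.
; Each hit takes interface damage, notifies the projectile's upgrade components on success, and restarts one shared timeline that sweeps the hit actor from the sphere's location to a distance-based offset.
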(event `self.ProjectileMovement.OnComponentActivated`
  (params (Component :type "ActorComponent Object Reference") (bReset :type Boolean))
  (set `self.Array` (`self.Array`))
  (`KismetSystemLibrary.K2_SetTimerDelegate` (delegate `Trace`) 0.1 true))

(event `Trace`
  (bind _array (`self.Array`))
  (bind _returnvalue (`SceneComponent.K2_GetComponentLocation` (`self.Sphere_Col`)))
  (`KismetArrayLibrary.Array_Add` _array (`GameplayStatics.GetPlayerCharacter` 0))
  (bind _outhits (`KismetSystemLibrary.SphereTraceMultiForObjects` _returnvalue _returnvalue 200.0 (`|MakeArray` "ObjectTypeQuery3" :!type "EObjectTypeQuery Enum") false _array))
  (for _array_element _outhits
    (bind (_bblockinghit _binitialoverlap _time _distance _location _impactpoint _normal _impactnormal _physmat _hitactor) (`GameplayStatics.BreakHitResult` _array_element))
    (`KismetArrayLibrary.Array_Add` (`self.Array`) _hitactor)
    (bind _output_get (set `self.Hit Actor` _hitactor))
    (`self.Dmg`)
    (bind _output_get_2 (set `self.NewVar` (`SceneComponent.K2_GetComponentLocation` (`self.Sphere_Col`))))
    (bind (_direction __movement) (`Timeline|Timeline` :!via `PlayFromStart`)
      (:`Update`
        (`self.K2_SetActorRelativeLocation` _output_get (`KismetMathLibrary.VLerp` _output_get_2 (- _output_get_2 _distance) __movement) true false)))))

(event `Dmg`
  (bind _target_hit_ (message `/Game/Tech/HealthSystem/BPI_DamageHandling.I_ApplyDamage` (stale `Trace` _output_get) (`self.Damage`) (`self.GetOwner`)))
  (if _target_hit_
    (for _array_element (`self.K2_GetComponentsByClass` "/Game/Tech/Upgrades/BPC_BaseUpgrade.BPC_BaseUpgrade_C")
      (`/Game/Tech/Upgrades/BPC_BaseUpgrade.Upgrade_HitEnemy` _array_element (`self.Damage`) (`self.K2_GetActorLocation`)))))

(fn `UserConstructionScript`
  (`parent.UserConstructionScript`))