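; Bubble projectile actor that launches at a random speed and damages what its collision sphere overlaps.
; The speed is randomised when the movement component activates, and damage goes through an interface message with the owner as instigator.
; A confirmed hit triggers UpgradeOther on its upgrade components, then destroys the bubble.
; Slowing exists only as debug prints, partly in unreachable nodes.
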(event `self.ReceiveBeginPlay`
  (`parent.ReceiveBeginPlay`))

(event `self.ProjectileMovement.OnComponentActivated`
  (params (Component :type "ActorComponent Object Reference") (bReset :type Boolean))
  ;[0.9922 0.6667 1] Projectile starts move at a random speed then slows down and damages all enemies nearby
  (set `ProjectileMovementComponent.InitialSpeed` (`KismetMathLibrary.RandomFloatInRange` 450.0 700.0) (`self.ProjectileMovement`)))

(event `self.Sphere_Col.OnComponentBeginOverlap`
  (params (OverlappedComponent :type "PrimitiveComponent Object Reference") (OtherActor :type "Actor Object Reference") (OtherComp :type "PrimitiveComponent Object Reference") (OtherBodyIndex :type Integer) (bFromSweep :type Boolean) (SweepResult :type "HitResult Structure (by ref)"))
  (`KismetSystemLibrary.PrintString` "slow")
  (bind _target_hit_ (message `/Game/Tech/HealthSystem/BPI_DamageHandling.I_ApplyDamage` OtherActor (`self.Damage`) (`self.GetOwner`)))
  (if _target_hit_
    (for _array_element (`self.K2_GetComponentsByClass` "/Game/Tech/Upgrades/BPC_BaseUpgrade.BPC_BaseUpgrade_C")
      (`/Game/Tech/Upgrades/BPC_BaseUpgrade.Upgrade_Other` _array_element))
    (`self.K2_DestroyActor`)))

(fn `UserConstructionScript`
  (`parent.UserConstructionScript`))