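; Projectile actor that damages enemies and carries shot upgrades.
; On BeginPlay it adds a component of the same class as each ShotUpgrades entry.
; Sphere overlaps send damage through an interface message with the owner as instigator; a confirmed hit notifies every BPC_BaseUpgrade component of the damage, then destroys the projectile.
; A blocking sphere hit simply destroys it.
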(event `self.ReceiveBeginPlay`
  (for _array_element (`self.Shot Upgrades`)
    (`|AddComponentByClass` (`GameplayStatics.GetObjectClass` _array_element))))

(event `self.Sphere_Col.OnComponentBeginOverlap`
  (params (OverlappedComponent :type "PrimitiveComponent Object Reference") (OtherActor :type "Actor Object Reference") (OtherComp :type "PrimitiveComponent Object Reference") (OtherBodyIndex :type Integer) (bFromSweep :type Boolean) (SweepResult :type "HitResult Structure (by ref)"))
  ;[1 1 1] Applying Damage to the enemy and destroys on impact
  (bind _target_hit_ (message `/Game/Tech/HealthSystem/BPI_DamageHandling.I_ApplyDamage` OtherActor (`self.Damage`) (`self.GetOwner`)))
  (if _target_hit_
    (for _array_element (`self.K2_GetComponentsByClass` "/Game/Tech/Upgrades/BPC_BaseUpgrade.BPC_BaseUpgrade_C")
      (`/Game/Tech/Upgrades/BPC_BaseUpgrade.Upgrade_HitEnemy` _array_element (`self.Damage`)))
    (`self.K2_DestroyActor`)))

(event `self.Sphere_Col.OnComponentHit`
  (params (HitComponent :type "PrimitiveComponent Object Reference") (OtherActor :type "Actor Object Reference") (OtherComp :type "PrimitiveComponent Object Reference") (NormalImpulse :type "Vector Structure") (Hit :type "HitResult Structure (by ref)"))
  ;[1 1 1] Projectile destroys on object hit
  (`self.K2_DestroyActor`))

(fn `UserConstructionScript`)