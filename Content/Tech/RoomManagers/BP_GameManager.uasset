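; Game manager that moves the player through randomly chosen rooms and on to a boss room.
; On BeginPlay it caches the room manager, which supplies the room locations, and the player.
; Each SetLocation call increments a counter, picks one of nine rooms through a random, non-looping MultiGate so none repeats, then teleports the player there.
; The seventh call sends the player to the boss room instead.
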(event `self.ReceiveBeginPlay`
  (bind _returnvalue (`GameplayStatics.GetActorOfClass` "/Game/Tech/RoomManagers/BP_Room1Manager.BP_Room1Manager_C"))
  (set `self.Room1Man` _returnvalue)
  (bind _returnvalue_2 (`GameplayStatics.GetActorOfClass` "/Game/Tech/Character/BP_Player.BP_Player_C"))
  (set `self.PLayer` _returnvalue_2))

(event `Teleport Player`
  (`self.K2_TeleportTo` :`self` (`self.PLayer`) :`DestLocation` (`self.PlayerRoom Start`)))

(event `Set Location`
  (bind _room1man (`self.Room1Man`))
  (bind _output_get (set `self.TimesTeleported` (+ (`self.TimesTeleported`) 1)))
  (`KismetSystemLibrary.PrintString` (`KismetStringLibrary.Conv_IntToString` (`self.TimesTeleported`)))
  (if (== _output_get 7)
    (set `self.PlayerRoom Start` (`SceneComponent.K2_GetComponentLocation` (`/Game/Tech/RoomManagers/BP_Room1Manager.BossRoom` (`self.Room1Man`))))
    (`self.Teleport Player`)
    (else
      (`|MultiGate` true
        (:`Out 0`
          (set `self.PlayerRoom Start` (`SceneComponent.K2_GetComponentLocation` (`/Game/Tech/RoomManagers/BP_Room1Manager.Room1` _room1man))))
        (:`Out 1`
          (set `self.PlayerRoom Start` (`SceneComponent.K2_GetComponentLocation` (`/Game/Tech/RoomManagers/BP_Room1Manager.Room2` _room1man))))
        (:`Out 2`
          (set `self.PlayerRoom Start` (`SceneComponent.K2_GetComponentLocation` (`/Game/Tech/RoomManagers/BP_Room1Manager.Room3` _room1man))))
        (:`Out 3`
          (set `self.PlayerRoom Start` (`SceneComponent.K2_GetComponentLocation` (`/Game/Tech/RoomManagers/BP_Room1Manager.Room4` _room1man))))
        (:`Out 4`
          (set `self.PlayerRoom Start` (`SceneComponent.K2_GetComponentLocation` (`/Game/Tech/RoomManagers/BP_Room1Manager.Room5` _room1man))))
        (:`Out 5`
          (set `self.PlayerRoom Start` (`SceneComponent.K2_GetComponentLocation` (`/Game/Tech/RoomManagers/BP_Room1Manager.Room6` _room1man))))
        (:`Out 6`
          (set `self.PlayerRoom Start` (`SceneComponent.K2_GetComponentLocation` (`/Game/Tech/RoomManagers/BP_Room1Manager.Room7` _room1man))))
        (:`Out 7`
          (set `self.PlayerRoom Start` (`SceneComponent.K2_GetComponentLocation` (`/Game/Tech/RoomManagers/BP_Room1Manager.Room8` _room1man))))
        (:`Out 8`
          (set `self.PlayerRoom Start` (`SceneComponent.K2_GetComponentLocation` (`/Game/Tech/RoomManagers/BP_Room1Manager.Room9` _room1man)))))
      (`self.Teleport Player`))))

(fn `UserConstructionScript`)