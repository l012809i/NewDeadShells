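; BP_D_Room4 is a procedurally generated Depths room variant that declares where its doors, walls and corners can spawn.
; Its construction script fills the door spawn array with two door locations and one corner location.
; The two door locations also serve as wall positions, and the corner as a one-wide door position, before the parent construction script runs.
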(fn `UserConstructionScript`
  ;[1 1 1] Set array of possible Door Spawns
  (set `self.TestedDoorSpawns` (`|MakeArray` (`self.DoorLocation1`) (`self.DoorLocation2`) (`self.CornerLocation1`)))
  ;[1 1 1] Set array of possible Wall Spawns
  (set `self.WallPositions` (`|MakeArray` (`self.DoorLocation1`) (`self.DoorLocation2`)))
  ;[1 1 1] List of Corners/1 Wide Doors
  (set `self.CornerPositions` (`|MakeArray` (`self.CornerLocation1`)))
  (`parent.UserConstructionScript`))