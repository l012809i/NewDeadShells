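; Procedural Depths combat room (Room 4, NW) that supplies door, wall and corner candidate locations to its parent's construction script.
; BeginPlay spawns yellow melee grunts at cylinder markers, and player overlap raises the barriers while EnemyCount is nonzero.
; Any overlap starts a self-recalling Delay poll of EnemyCount.
; At zero, it increments the room manager's KilledEnemies once, restores the barriers and spawns a whirlpool teleporter if SpawnBossPortal is set.
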(event `self.ReceiveBeginPlay`
  ;[1 1 1] Spawns Enemies
  (for _array_element (`|MakeArray` (`self.Cylinder1`) (`self.Cylinder2`) (`self.Cylinder3`) (`self.Cylinder4`) (`self.Cylinder`) :!type "SceneComponent Object Reference")
    (`|SpawnActorFromClass` "/Game/Tech/Character/Enemies/NewAI/MeleeGrunt/BP_MeleeGrunt_Yellow.BP_MeleeGrunt_Yellow_C" (`SceneComponent.K2_GetComponentToWorld` _array_element) "Undefined" "OverrideRootScale" self null)))

(event `self.Box.OnComponentBeginOverlap`
  (params (OverlappedComponent :type "PrimitiveComponent Object Reference") (OtherActor :type "Actor Object Reference") (OtherComp :type "PrimitiveComponent Object Reference") (OtherBodyIndex :type Integer) (bFromSweep :type Boolean) (SweepResult :type "HitResult Structure (by ref)"))
  ;[1 1 1] Locks Room and spawns enemies
  (`self.D_Room_4_Loop`)
  (if (== (`GameplayStatics.GetObjectClass` OtherActor) "/Game/Tech/Character/BP_Player.BP_Player_C")
    (if (!= (`self.EnemyCount`) 0)
      (bind _output_get (set `self.BarrierOrigin` (`SceneComponent.K2_GetComponentLocation` (`self.RoomBarriers`))))
      (`SceneComponent.K2_SetWorldLocation` (`self.RoomBarriers`) (+ _output_get (0.0 0.0 400.0)) false false))))

(event `D_Room_4_Loop`
  ;[1 1 1] Room Completion Tracker
  (if (== (`self.EnemyCount`) 0)
    (`/Engine/EditorBlueprintResources/StandardMacros.DoOnce` false
      (:`Completed`
        (`/Engine/EditorBlueprintResources/StandardMacros.IncrementInt` (`/Game/Tech/ProcGen/BP_R_RoomManager.KilledEnemies` (`self.RoomManager Reference`))
          (:`  `
            (`SceneComponent.K2_SetWorldLocation` (`self.RoomBarriers`) (`self.BarrierOrigin`) false false)
            (`KismetSystemLibrary.Delay` 0.5)
            (if (`/Game/Tech/ProcGen/BP_R_RoomManager.SpawnBossPortal` (`self.RoomManager Reference`))
              (`|SpawnActorFromClass` "/Game/Tech/ProcGen/Whirlpool/Whirlpool_Teleporter.Whirlpool_Teleporter_C" (`SceneComponent.K2_GetComponentToWorld` (`self.DefaultSceneRoot`)) "Undefined" "OverrideRootScale" null null))))))
    (else
      (`KismetSystemLibrary.Delay` 0.5)
      (`self.D_Room_4_Loop`))))

(fn `D_Room_3_Loop`)

(fn `UserConstructionScript`
  ;[1 1 1] Set array of possible Door Spawns
  (set `self.TestedDoorSpawns` (`|MakeArray` (`self.DoorLocation1`) (`self.DoorLocation2`) (`self.CornerLocation1`)))
  ;[1 1 1] Set array of possible Wall Spawns
  (set `self.WallPositions` (`|MakeArray` (`self.DoorLocation1`) (`self.DoorLocation2`)))
  ;[1 1 1] List of Corners/1 Wide Doors
  (set `self.CornerPositions` (`|MakeArray` (`self.CornerLocation1`)))
  (`parent.UserConstructionScript`))