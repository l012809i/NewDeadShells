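; Base room for procedural map generation that grows the level by spawning neighbouring rooms at its doors.
; On BeginPlay it registers with BP_R_RoomManager and, until pregeneration completes, spawns random ReefDepthsRooms ahead of random doors, using collision-checked spawning with tick-delayed retries.
; It then sends remaining doors to the manager, whose wall event triggers spawning of walls and corners at marked positions.
; The boss-room spawner is unused legacy code.
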(event `self.ReceiveBeginPlay`
  (bind _outitem (`KismetArrayLibrary.Array_Random` (`self.TestedDoorSpawns`)))
  (bind _returnvalue (`KismetMathLibrary.RandomIntegerInRange` 2 (`KismetArrayLibrary.Array_Length` (`self.TestedDoorSpawns`))))
  (bind _returnvalue_2 (`GameplayStatics.GetActorOfClass` "/Game/Tech/ProcGen/BP_R_RoomManager.BP_R_RoomManager_C")) ; Selects the Room Manager
  (bind _output_get (set `self.RoomManager Reference` _returnvalue_2))
  ;[1 1 1] Selects Room Array
  (`KismetArrayLibrary.Array_Clear` (`self.RoomsToSpawn`)) ; Sanity Check
  (set `self.RoomsToSpawn` (`self.Reef+DepthsRooms`))
  (add `/Game/Tech/ProcGen/BP_R_RoomManager.E_WallSpawn` _output_get (delegate `Activate Walls`))
  (message `/Game/Tech/ProcGen/BPI_RoomManager.Map Size Tracker` (`self.RoomManager Reference`) (`self.Room Size`) self) ; Sends Room Size and Type to RoomManager
  (`/Engine/EditorBlueprintResources/StandardMacros.DoOnce` false
    (:`Completed`
      (if (not (`/Game/Tech/ProcGen/BP_R_RoomManager.Map Pregen complete?` (`self.RoomManager Reference`)))
        (`KismetSystemLibrary.DelayUntilNextTick`)
        (`KismetSystemLibrary.PrintString` (`KismetStringLibrary.Conv_IntToString` _returnvalue))
        (for _ (range (+ _returnvalue 1))
          (if (not (`/Game/Tech/ProcGen/BP_R_RoomManager.Map Pregen complete?` (`self.RoomManager Reference`)))
            ;[1 1 1] Room Spawner
            (bind _returnvalue_3 (`|SpawnActorFromClass` (`KismetArrayLibrary.Array_Random` (`self.RoomsToSpawn`)) (`KismetMathLibrary.Conv_VectorToTransform` (+ (* (`SceneComponent.GetForwardVector` _outitem) 2800.0) (`SceneComponent.K2_GetComponentLocation` _outitem))) "DontSpawnIfColliding" "OverrideRootScale" null null :!label _label)) ; Tries to spawn a Room
            (`/Engine/EditorBlueprintResources/StandardMacros.IsValid` _returnvalue_3
              (:`Is Valid`
                (`KismetArrayLibrary.Array_Add` (`self.ValidTeleports`) _outitem))
              (:`Is Not Valid`
                (bind _result (`/Engine/EditorBlueprintResources/StandardMacros.IncrementInt` (`self.Room Spawn Attempts`))
                  (:`  `
                    (if (== _result (/ (`KismetArrayLibrary.Array_Length` (`self.RoomsToSpawn`)) 2))
                      _
                      (else
                        (`KismetSystemLibrary.DelayUntilNextTick`)
                        (goto _label)))))))
            (`KismetArrayLibrary.Array_RemoveItem` (`self.TestedDoorSpawns`) _outitem)))
        (`KismetSystemLibrary.DelayUntilNextTick`)
        (for _array_element (`self.TestedDoorSpawns`)
          (message `/Game/Tech/ProcGen/BPI_EmptyDoors.Door Data Sender` (`self.RoomManager Reference`) _array_element))))))

(event `Activate Walls`
  (`/Engine/EditorBlueprintResources/StandardMacros.DoOnce` false
    (:`Completed`
      (for _array_element (`self.WallPositions`)
        (bind _returnvalue (`SceneComponent.K2_GetComponentToWorld` _array_element))
        (`|SpawnActorFromClass` "/Game/Tech/ProcGen/Walls/BP_BaseWall.BP_BaseWall_C" (`KismetMathLibrary.MakeTransform` (.location _returnvalue) (`KismetMathLibrary.MakeRotator` 0.0 0.0 (.yaw (.rotation _returnvalue))) (.scale _returnvalue)) "AlwaysSpawn" "OverrideRootScale" null true null))
      (for _array_element_2 (`self.CornerPositions`)
        (bind _returnvalue_2 (`SceneComponent.K2_GetComponentToWorld` _array_element_2))
        (`|SpawnActorFromClass` "/Game/Tech/ProcGen/Walls/BP_BaseDoubleCorner.BP_BaseDoubleCorner_C" (`KismetMathLibrary.MakeTransform` (.location _returnvalue_2) (`KismetMathLibrary.MakeRotator` 0.0 0.0 (.yaw (.rotation _returnvalue_2))) (.scale _returnvalue_2)) "Undefined" "OverrideRootScale" null true null)))))

(event `BossRoomSpawn`
  (bind _outitem (`KismetArrayLibrary.Array_Random` (`self.TestedDoorSpawns`)))
  ;[0.2656 0 0] Legacy Boss Room Code - Not used.
  (add `/Game/Tech/ProcGen/BP_R_RoomManager.E_StopBossRoomSpawn` (`self.RoomManager Reference`) (delegate `StopBossRoomSpawn`))
  (`/Engine/EditorBlueprintResources/StandardMacros.DoOnce` false
    (:`Completed`
      (for _ (range 4) :!label _label_2
        (bind _returnvalue (`|SpawnActorFromClass` "/Game/Tech/ProcGen/Rooms/BP_Room_Boss.BP_Room_Boss_C" (`KismetMathLibrary.Conv_VectorToTransform` (+ (* (`SceneComponent.GetForwardVector` _outitem) 2400.0) (`SceneComponent.K2_GetComponentLocation` _outitem))) "DontSpawnIfColliding" "OverrideRootScale" null null :!label _label_3)) ; Tries to spawn a Boss Room
        (`/Engine/EditorBlueprintResources/StandardMacros.IsValid` _returnvalue
          (:`Is Valid`
            (message `/Game/Tech/ProcGen/Rooms/BPI_BossRoom.Boss Room ID` (`self.RoomManager Reference`) _returnvalue))
          (:`Is Not Valid`
            (bind _result (`/Engine/EditorBlueprintResources/StandardMacros.IncrementInt` (`self.Room Spawn Attempts`))
              (:`  `
                (if (not (== _result (/ (`KismetArrayLibrary.Array_Length` (`self.ReefRooms`)) 2)))
                  (`KismetSystemLibrary.DelayUntilNextTick`)
                  (goto _label_3))))))))))

(event `StopBossRoomSpawn`
  ;[0.2656 0 0] Legacy Boss Room Code - Not used.
  (goto _label_2 :!via `Break`))

(fn `OnRep_EnemyCount`)

(fn `UserConstructionScript`)