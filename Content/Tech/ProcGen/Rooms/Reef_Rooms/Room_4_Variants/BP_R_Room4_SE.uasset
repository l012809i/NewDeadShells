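; BP_R_Room4_SE is a reef room variant (Room 4, SE) for procedural level generation.
; Its construction script fills both the possible door spawn and wall spawn arrays with the same eight door locations.
; It sets both arrays before calling the parent construction script, leaving any further setup to the parent class.
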(fn `UserConstructionScript`
  (bind _array (`|MakeArray` (`self.DoorLocation1`) (`self.DoorLocation2`) (`self.DoorLocation3`) (`self.DoorLocation4`) (`self.DoorLocation5`) (`self.DoorLocation6`) (`self.DoorLocation7`) (`self.DoorLocation8`)))
  ;[1 1 1] Set array of possible Door Spawns
  (set `self.TestedDoorSpawns` _array)
  ;[1 1 1] Set array of possible Wall Spawns
  (set `self.WallPositions` _array)
  (`parent.UserConstructionScript`))