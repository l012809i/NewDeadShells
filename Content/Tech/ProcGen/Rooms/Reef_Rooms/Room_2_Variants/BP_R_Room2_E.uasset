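; BP_R_Room2_E is a Room 2 variant, variant E, for the Reef rooms in the procedural room generation system.
; Its construction script fills the candidate arrays from placed location references: two corners serve as both tested door spawns and corner/one-wide door positions, and six locations serve as wall positions.
; It then calls the parent construction script, so the arrays are set before any inherited logic runs.
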(fn `UserConstructionScript`
  ;[1 1 1] Set array of possible Door Spawns
  (set `self.TestedDoorSpawns` (`|MakeArray` (`self.CornerLocation1`) (`self.CornerLocation2`)))
  ;[1 1 1] Set array of possible Wall Spawns
  (set `self.WallPositions` (`|MakeArray` (`self.WallLocation1`) (`self.WallLocation2`) (`self.WallLocation3`) (`self.WallLocation4`) (`self.WallLocation5`) (`self.WallLocation6`)))
  ;[1 1 1] List of Corners/1 Wide Doors
  (set `self.CornerPositions` (`|MakeArray` (`self.CornerLocation1`) (`self.CornerLocation2`)))
  (`parent.UserConstructionScript`))