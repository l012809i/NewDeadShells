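; BP_R_Room2_S is a Reef room variant for procedural generation, built on a parent room Blueprint.
; Its Construction Script fills the tested door spawn array with two door locations and the wall position array with six wall spawns plus those same door locations.
; It then runs the parent Construction Script, so both arrays are set before any inherited construction logic.
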(fn `UserConstructionScript`
  ;[1 1 1] Set array of possible Door Spawns
  (set `self.TestedDoorSpawns` (`|MakeArray` (`self.DoorLocation1`) (`self.DoorLocation2`)))
  ;[1 1 1] Set array of possible Wall Spawns
  (set `self.WallPositions` (`|MakeArray` (`self.WallSpawn1`) (`self.WallSpawn2`) (`self.WallSpawn3`) (`self.WallSpawn4`) (`self.WallSpawn5`) (`self.WallSpawn6`) (`self.DoorLocation1`) (`self.DoorLocation2`)))
  (`parent.UserConstructionScript`))