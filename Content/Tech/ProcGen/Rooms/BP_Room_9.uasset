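; BP_Room_9 is a procedural generation room variant that supplies its own spawn point layout to a parent room class.
; Its construction script fills TestedDoorSpawns with four movement locations for spawn and teleport points, and ArrowPositions with those plus two wall spawns for possible door spawns.
; Both arrays are set before the parent construction script runs, and the event graph holds only disabled default events.
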(fn `UserConstructionScript`
  ;[1 1 1] Set array of possible Spawn and Teleport spawnpoints
  (set `self.TestedDoorSpawns` (`|MakeArray` (`self.MovementLocation1`) (`self.MovementLocation2`) (`self.MovementLocation3`) (`self.MovementLocation4`)))
  ;[1 1 1] Set array of possible Door Spawns
  (set `self.ArrowPositions` (`|MakeArray` (`self.MovementLocation1`) (`self.MovementLocation2`) (`self.MovementLocation3`) (`self.MovementLocation4`) (`self.WallSpawn1`) (`self.WallSpawn2`)))
  (`parent.UserConstructionScript`))