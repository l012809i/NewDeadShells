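; BP_Room_1 is a procedural generation room Blueprint of size 1 with four door locations, built on a parent room class.
; Its construction script fills both the tested door spawn and arrow position arrays with those four locations, then runs the parent construction script.
; BeginPlay sets the room size, then calls the parent BeginPlay through a DoOnce.
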(event `self.ReceiveBeginPlay`
  (set `self.Room Size` 1)
  (`/Engine/EditorBlueprintResources/StandardMacros.DoOnce` false
    (:`Completed`
      (`parent.ReceiveBeginPlay`))))

(fn `UserConstructionScript`
  (bind _array (`|MakeArray` (`self.DoorLocation1`) (`self.DoorLocation2`) (`self.DoorLocation3`) (`self.DoorLocation4`)))
  ;[1 1 1] Set array of possible room positions
  (set `self.TestedDoorSpawns` _array)
  (set `self.ArrowPositions` _array)
  (`parent.UserConstructionScript`))