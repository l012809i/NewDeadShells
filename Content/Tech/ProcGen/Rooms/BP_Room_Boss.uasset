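; BP_Room_Boss is the boss room of the procedural room generator and fills its marked edge positions with walls.
; On BeginPlay it gathers its door location and wall spawn markers into an array, then binds to the wall spawn event of BP_R_RoomManager.
; When that event fires, a DoOnce lets it spawn a BP_BaseWall at every marker, door location included, using the marker's location, yaw and scale.
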(event `self.ReceiveBeginPlay`
  ;[1 1 1] Set array of possible Door Spawns
  (set `self.WallPositions` (`|MakeArray` (`self.DoorLocation1`) (`self.WallSpawn1`) (`self.WallSpawn2`) (`self.WallSpawn3`) (`self.WallSpawn4`) (`self.WallSpawn5`) (`self.WallSpawn6`) (`self.WallSpawn7`) (`self.WallSpawn8`) (`self.WallSpawn9`) (`self.WallSpawn10`) (`self.WallSpawn11`)))
  (bind _returnvalue (`GameplayStatics.GetActorOfClass` "/Game/Tech/ProcGen/BP_R_RoomManager.BP_R_RoomManager_C")) ; Selects the Room Manager
  (bind _output_get (set `self.RoomManager Reference` _returnvalue))
  (add `/Game/Tech/ProcGen/BP_R_RoomManager.E_WallSpawn` _output_get (delegate `Wall Spawn`)))

(event `Wall Spawn`
  (`/Engine/EditorBlueprintResources/StandardMacros.DoOnce` false
    (:`Completed`
      (for _array_element (`self.WallPositions`)
        (bind _returnvalue (`SceneComponent.K2_GetComponentToWorld` _array_element))
        (`|SpawnActorFromClass` "/Game/Tech/ProcGen/Walls/BP_BaseWall.BP_BaseWall_C" (`KismetMathLibrary.MakeTransform` (.location _returnvalue) (`KismetMathLibrary.MakeRotator` 0.0 0.0 (.yaw (.rotation _returnvalue))) (.scale _returnvalue)) "AlwaysSpawn" "OverrideRootScale" null true null)))))

(fn `UserConstructionScript`)