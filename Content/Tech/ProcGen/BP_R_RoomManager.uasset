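; Room manager for procedural map generation, spawning a normal or Depths starting room and tracking the pieces that grow from it.
; Pieces report their size toward a target, with a retriggerable delay acting as a stall timeout that destroys and regenerates undersized maps.
; At target size it triggers boss room spawning, then randomly culls extras down to two.
; With two, it triggers wall spawning and flags one as mini-boss; with fewer, it regenerates.
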(event `/Game/Tech/ProcGen/BPI_EmptyDoors.Door Data Sender`
  (params (EmptyDoors :type "ArrowComponent Object Reference"))
  ;[1 1 1] Stores Unused rooms for Boss Room spawning
  (`KismetArrayLibrary.Array_Add` (`self.Possible Boss Room Spawn`) EmptyDoors))

(event `self.ReceiveBeginPlay`
  ;[1 1 1] Spawns the inital starting room, and resets the map size
  (set `self.Map Pregen complete?` false :!label _label)
  (set `self.Boss Room Spawned?` false)
  (if (== (`self.IsDepths`) true)
    (set `self.Starting Room` "/Game/Tech/ProcGen/Rooms/Depths_Rooms/Depths_Starting_Room.Depths_Starting_Room_C")
    (else
      (set `self.Starting Room` "/Game/Tech/ProcGen/Rooms/Reef_Rooms/BP_R_StartingRoom.BP_R_StartingRoom_C")))
  (`|SpawnActorFromClass` (`self.Starting Room`) (`self.Starting Room Transform`) "AlwaysSpawn" "OverrideRootScale" null null)
  (set `self.Current Map Size` 0))

(event `Generate Rooms`
  ;[1 1 1] Spawns the inital starting room, and resets the map size
  (goto _label))

(event `/Game/Tech/ProcGen/BPI_RoomManager.Map Size Tracker`
  (params (RoomSize :type Integer) (MapPiece :type "/Game/Tech/ProcGen/Rooms/BP_BaseRoom Object Reference"))
  ;[1 1 1] Stores each spawned map segement into an array
  (`KismetArrayLibrary.Array_Add` (`self.Spawned Map Pieces`) MapPiece)
  ;[1 1 1] Adds together the map size
  (bind _output_get (set `self.Current Map Size` (+ RoomSize (`self.Current Map Size`))))
  (`KismetSystemLibrary.PrintString` (`KismetStringLibrary.Conv_IntToString` _output_get))
  ;[1 1 1] If Map Size generated is too small or too big, the map regenerates.
  (if (>= (`self.Current Map Size`) (`self.Target Map Size`))
    (set `self.Map Pregen complete?` true)
    (`self.E_BossRoomSpawn`)
    (else
      (`KismetSystemLibrary.RetriggerableDelay` 0.4)
      (if (not (`self.Map Pregen complete?`))
        (`self.K2_DestroyActor` (`self.Spawned Map Pieces`))
        (`KismetSystemLibrary.DelayUntilNextTick`)
        (`self.Generate Rooms`)
        (set `self.Map Pregen complete?` false)))))

(event `/Game/Tech/ProcGen/Rooms/BPI_BossRoom.Boss Room ID`
  (params (BossRoomID :type "/Game/Tech/ProcGen/Rooms/BP_Room_Boss Object Reference"))
  (bind _bossrooms (`self.BossRooms`))
  (bind _outitem (`KismetArrayLibrary.Array_Random` _bossrooms))
  ;[1 1 1] Spawns boss rooms in all possible locations, and then despawns unused ones if there is more than 2.
  (`KismetArrayLibrary.Array_Add` (`self.BossRooms`) BossRoomID)
  (`self.E_StopBossRoomSpawn`)
  (`/Engine/EditorBlueprintResources/StandardMacros.DoOnce` false
    (:`Completed`
      (`KismetSystemLibrary.Delay` 2.0 :!label _label_2)
      (if (<= (`KismetArrayLibrary.Array_Length` (`self.BossRooms`)) 2)
        ;[1 1 1] Tests if 2 boss rooms exist, if so, one is randomly assigned to be a boss room. If there are less than 2, the map regenerates.
        (if (== (`KismetArrayLibrary.Array_Length` (`self.BossRooms`)) 2)
          (`self.E_WallSpawn`)
          (set `/Game/Tech/ProcGen/Rooms/BP_Room_Boss.IsMiniBossRoom?` true (`KismetArrayLibrary.Array_Random` (`self.BossRooms`)))
          (else
            (`KismetSystemLibrary.RetriggerableDelay` 0.4)
            (if (`self.Map Pregen complete?`)
              _
              (else
                _))
            (`self.K2_DestroyActor` (`self.Spawned Map Pieces`))
            (`KismetSystemLibrary.DelayUntilNextTick`)
            (`self.Generate Rooms`)
            (set `self.Map Pregen complete?` false)))
        (else
          (`KismetArrayLibrary.Array_RemoveItem` _bossrooms _outitem)
          (`self.K2_DestroyActor` _outitem)
          (`KismetSystemLibrary.DelayUntilNextTick`)
          (goto _label_2))))))

(fn `UserConstructionScript`)