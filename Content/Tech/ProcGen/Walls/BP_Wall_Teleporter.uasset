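; BP_Wall_Teleporter is a procedural-generation wall that moves the player between rooms, noted in the graph as a messy stand-in for a corridor system.
; When BP_Player overlaps its box, it prints the offset and teleports the player a fixed distance along the box's forward vector, with zeroed rotation.
; A DoOnce that resets after a short delay gates repeat triggers, whichever actor overlaps.
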(event `self.Box_0.OnComponentBeginOverlap`
  (params (OverlappedComponent :type "PrimitiveComponent Object Reference") (OtherActor :type "Actor Object Reference") (OtherComp :type "PrimitiveComponent Object Reference") (OtherBodyIndex :type Integer) (bFromSweep :type Boolean) (SweepResult :type "HitResult Structure (by ref)"))
  (bind _returnvalue (* (`SceneComponent.GetForwardVector` (`self.Box_0`)) 3400.0))
  ;[1 0 0] This is a mess. It will move the player between rooms, but PLEASE do the corridor system. I hate this with a passion.
  (`/Engine/EditorBlueprintResources/StandardMacros.DoOnce` false :!label _label
    (:`Completed`
      (`|ExecutionSequence`
        (:`then_0`
          (if (== (`GameplayStatics.GetObjectClass` OtherActor) "/Game/Tech/Character/BP_Player.BP_Player_C")
            (`KismetSystemLibrary.PrintString` (`KismetStringLibrary.Conv_VectorToString` _returnvalue))
            (`self.K2_TeleportTo` :`self` OtherActor :`DestLocation` (+ (`SceneComponent.K2_GetComponentLocation` (`self.Box_0`)) _returnvalue))))
        (:`then_1`
          (`KismetSystemLibrary.Delay` 0.2)
          (goto _label :!via `Reset`))))))

(fn `UserConstructionScript`
  (`parent.UserConstructionScript`))