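; Procedural-generation wall corner piece that resolves itself into either a doorway or a closed corner.
; On BeginPlay it gathers its doorway meshes and floor tiles, waits briefly, then line-traces forward from an arrow component to set IsDoor.
; A hit removes the two coral corner components, while a miss removes the doorway set.
; An unconnected leftover graph would teleport the player forward between rooms, noted as a stopgap for a corridor system.
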(event `self.ReceiveBeginPlay`
  (bind _arrow (`self.Arrow`))
  (bind _returnvalue (`SceneComponent.K2_GetComponentLocation` _arrow))
  (set `self.DoorwayArray` (`|MakeArray` (`self.Coral Doorway`) (`self.Coral Doorway1`) (`self.StaticMesh`) (`self.StaticMesh1`) (`self.StaticMesh2`) (`self.StaticMesh3`) (`self.StaticMesh4`) (`self.StaticMesh5`) (`self.StaticMesh6`) (`self.StaticMesh7`) (`self.Floor_Tile`) (`self.Floor_Tile1`) (`self.Floor_Tile2`) (`self.Floor_Tile3`) :!type "ActorComponent Object Reference"))
  (`KismetSystemLibrary.Delay` 1.0)
  (bind (_outhit _returnvalue_2) (`KismetSystemLibrary.LineTraceSingle` :`Start` _returnvalue :`End` (+ _returnvalue (* (`SceneComponent.GetForwardVector` _arrow) 2300.0)) :`TraceChannel` "TraceTypeQuery3" :`DrawDebugType` "Persistent" :`bIgnoreSelf` false))
  (bind _output_get (set `self.IsDoor?` _returnvalue_2))
  (if _output_get
    (`ActorComponent.K2_DestroyComponent` (`self.Coral Corner`))
    (`ActorComponent.K2_DestroyComponent` (`self.Coral Corner1`))
    (else
      (`ActorComponent.K2_DestroyComponent` (`self.DoorwayArray`)))))

(fn `UserConstructionScript`)