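; Weapon upgrade component that performs single projectile or melee attacks and provides empty hook events, likely for child upgrade components.
; BeginPlay caches the owning weapon's mesh and its player.
; Shots spawn from the FirePoint socket, yawed toward a point ahead of the player with random inaccuracy; swings spawn at the player's Projectilespawn with flattened pitch.
; After spawning, it calls the matching hook on every BPC_SingleAttack on the weapon, passing trajectory, type, damage and upgrades.
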(event `ShotUpgrades`
  (params (Trajectory :type "Transform Structure") (ProjectileType :type "/Game/Tech/Projectiles/NewProjectiles/BP_BaseProjectile Class Reference") (Damage :type "Float (double-precision)") (`Shot Upgrades` :type "Array of /Game/Tech/Upgrades/BPC_ChainLightning Object Reference")))

(event `MeleeUpgrades`
  (params (Location :type "Transform Structure") (`Melee Type` :type "/Game/Tech/MeleeAttacks/BP_BaseMelee Class Reference") (Damage :type "Float (double-precision)") (`Shot Upgrades` :type "Array of /Game/Tech/Upgrades/BPC_ChainLightning Object Reference")))

(event `self.ReceiveBeginPlay`
  (bind _returnvalue (`self.GetOwner`))
  (bind _asbp_base_weapon (cast `/Game/Tech/Weapons/WeaponInfo/BP_BaseWeapon` _returnvalue :!pure true))
  (bind _asbp_player (cast `/Game/Tech/Character/BP_Player` (`Actor.GetOwner` _returnvalue) :!pure true))
  (`parent.ReceiveBeginPlay`)
  (`/Engine/EditorBlueprintResources/StandardMacros.IsValid` _asbp_base_weapon
    (:`Is Valid`
      (set `self.Weapon Mesh` (`/Game/Tech/Weapons/WeaponInfo/BP_BaseWeapon.SM_Weapon` _asbp_base_weapon))
      (`/Engine/EditorBlueprintResources/StandardMacros.IsValid` _asbp_player
        (:`Is Valid`
          (set `self.Player` _asbp_player))))))

(event `self.Upgrade_ProjectileShoot`
  (params (`Inaccuracy (half-degrees)` :type "Float (double-precision)") (`Projectile Type` :type "/Game/Tech/Projectiles/NewProjectiles/BP_BaseProjectile Class Reference") (Damage :type "Float (double-precision)") (`Shot Upgrades` :type "Array of /Game/Tech/Upgrades/BPC_ChainLightning Object Reference (by ref)"))
  ;[0 1 1] Single shot for projectiles
  (set `self.Projectile Type` `Projectile Type`)
  (set `self.Damage` Damage)
  (set `self.Shot Upgrades` `Shot Upgrades`)
  (bind _output_get (set `self.ProjectileTrajectory` (`self.F_Calculate Trajectory` `Inaccuracy (half-degrees)`)))
  (`|SpawnActorFromClass` (`self.Projectile Type`) (`KismetMathLibrary.MakeTransform` (+ (.location _output_get) (* (`SceneComponent.GetRightVector` (`self.Weapon Mesh`)) (`self.Location Offset - Projectile`))) (.rotation _output_get) (.scale _output_get)) "Undefined" "OverrideRootScale" (`Actor.GetOwner` (`self.GetOwner`)) (`self.Damage`) (`self.Shot Upgrades`) null)
  (for _array_element (`Actor.K2_GetComponentsByClass` (`self.GetOwner`) "BPC_SingleAttack_C")
    (`self.ShotUpgrades` _array_element (`self.ProjectileTrajectory`) (`self.Projectile Type`) (`self.Damage`) (`self.Shot Upgrades`))))

(event `self.Upgrade_MeleeSwing`
  (params (`Melee Attack` :type "/Game/Tech/MeleeAttacks/BP_BaseMelee Class Reference") (Damage :type "Float (double-precision)") (`Shot Upgrades` :type "Array of /Game/Tech/Upgrades/BPC_ChainLightning Object Reference (by ref)"))
  (bind (_meleetrajectory_location _meleetrajectory_rotation _meleetrajectory_scale) (`KismetMathLibrary.BreakTransform` (`self.MeleeTrajectory`)))
  ;[0 1 1] SingleShot for Melee
  (set `self.Melee Attack` `Melee Attack`)
  (set `self.MeleeDamage` Damage)
  (set `self.MeleeShotUpgrades` `Shot Upgrades`)
  (set `self.MeleeTrajectory` (`self.F_CalculateMelee`))
  (`|SpawnActorFromClass` (`self.Melee Attack`) (`KismetMathLibrary.MakeTransform` (+ _meleetrajectory_location (* (`SceneComponent.GetRightVector` (`/Game/Tech/Character/BP_Player.Projectilespawn` (`self.Player`))) (`self.Location Offset - Melee`))) _meleetrajectory_rotation _meleetrajectory_scale) "Undefined" "OverrideRootScale" (`Actor.GetOwner` (`self.GetOwner`)) (`self.MeleeDamage`) (`self.MeleeShotUpgrades`) null)
  (for _array_element (`Actor.K2_GetComponentsByClass` (`self.GetOwner`) "BPC_SingleAttack_C")
    (`self.MeleeUpgrades` _array_element (`self.MeleeTrajectory`) (`self.Melee Attack`) (`self.MeleeDamage`) (`self.MeleeShotUpgrades`))))

(fn `F_Calculate Trajectory`
  (params (`Inaccuracy (half-deg)` :type "Float (double-precision)"))
  (returns (ReturnValue :type "Transform Structure"))
  (bind _player (`self.Player`))
  (bind _weapon_mesh (`self.Weapon Mesh`))
  (bind _location (.location (`SceneComponent.GetSocketTransform` _weapon_mesh "FirePoint" "RTS_World")))
  (bind (_returnvalue_roll _returnvalue_pitch _returnvalue_yaw) (`KismetMathLibrary.BreakRotator` (`KismetMathLibrary.MakeRotator` 0.0 0.0 (`KismetMathLibrary.RandomFloatInRange` (* `Inaccuracy (half-deg)` -1.0) `Inaccuracy (half-deg)`))))
  (bind (_returnvalue_roll_2 _returnvalue_pitch_2 _returnvalue_yaw_2) (`KismetMathLibrary.BreakRotator` (`KismetMathLibrary.FindLookAtRotation` _location (+ (`Actor.K2_GetActorLocation` _player) (* (`SceneComponent.GetForwardVector` (`/Game/Tech/Character/BP_Player.Projectilespawn` _player)) 500.0)))))
  (`/Engine/EditorBlueprintResources/StandardMacros.IsValid` _weapon_mesh
    (:`Is Valid`
      (return (`KismetMathLibrary.MakeTransform` _location (`KismetMathLibrary.MakeRotator` 0.0 0.0 (+ _returnvalue_yaw_2 _returnvalue_yaw)))))))

(fn `F_CalculateMelee`
  (returns (ReturnValue :type "Transform Structure"))
  (return (`KismetMathLibrary.MakeTransform` (.location (`SceneComponent.K2_GetComponentToWorld` (`/Game/Tech/Character/BP_Player.Projectilespawn` (`self.Player`)))) (`KismetMathLibrary.MakeRotator` (.roll (.rotation (`SceneComponent.K2_GetComponentToWorld` (`/Game/Tech/Character/BP_Player.Projectilespawn` (`self.Player`))))) 0.0 (.yaw (.rotation (`SceneComponent.K2_GetComponentToWorld` (`/Game/Tech/Character/BP_Player.Projectilespawn` (`self.Player`)))))))))