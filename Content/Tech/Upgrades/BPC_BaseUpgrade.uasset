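; Base upgrade component that gives child upgrades empty hooks for projectile shots, melee swings, enemy hits, and player and weapon stats.
; On BeginPlay it finds the DT_Upgrades row whose blueprint matches its own class and caches it as UpgradeInformation.
; UpgradeInit checks the owner for another component of the same class and slot, and if one exists asks the owner via interface message to destroy this one.
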(event `Upgrade Init`
  (for _array_element (`Actor.K2_GetComponentsByClass` (`self.GetOwner`) (`GameplayStatics.GetObjectClass` self))
    (if (and (!= self _array_element) (== (`/Game/Tech/Upgrades/BPC_BaseUpgrade.Slot` _array_element) (`self.Slot`)))
      (message `/Game/Tech/Upgrades/BPI_upgradeComponents.I_DestroyComponent` (`self.GetOwner`) self))))

(event `Upgrade_ProjectileShoot`
  (params (`Inaccuracy (half-degrees)` :type "Float (double-precision)") (`Projectile Type` :type "/Game/Tech/Projectiles/NewProjectiles/BP_BaseProjectile Class Reference") (Damage :type "Float (double-precision)") (`Shot Upgrades` :type "Array of /Game/Tech/Upgrades/BPC_ChainLightning Object Reference")))

(event `Upgrade_MeleeSwing`
  (params (`Melee Attack` :type "/Game/Tech/MeleeAttacks/BP_BaseMelee Class Reference") (Damage :type "Float (double-precision)") (`Shot Upgrades` :type "Array of /Game/Tech/Upgrades/BPC_ChainLightning Object Reference")))

(event `Upgrade_HitEnemy`
  (params (Damage :type "Float (double-precision)") (Location :type "Vector Structure")))

(event `Upgrade_PlayerStat`)

(event `Upgrade_WeaponStat`)

(event `self.ReceiveBeginPlay`
  (bind _outrownames (`DataTableFunctionLibrary.GetDataTableRowNames` "/Game/Tech/Upgrades/DT_Upgrades.DT_Upgrades"))
  (for _array_element _outrownames
    (bind _returnvalue (`|GetDataTableRow` "/Game/Tech/Upgrades/DT_Upgrades.DT_Upgrades" _array_element)
      (:`then`
        (if (== (`.UpgradeBlueprint_6_FD1D87BD4F63A6ABAD2F1B9A84B7BE98` (break `/Game/Tech/Upgrades/S_Upgrades` _returnvalue)) (`GameplayStatics.GetObjectClass` self))
          (set `self.UpgradeInformation` _returnvalue))))))