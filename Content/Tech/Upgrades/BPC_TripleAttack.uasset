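; Upgrade component for a triple attack that spawns two projectiles angled to either side of a calculated trajectory.
; UpgradeProjectile gets the trajectory from the inaccuracy value, then spawns the given projectile class twice with mirrored yaw offsets, passing on owner, damage and shot upgrades.
; A DoOnce flips the offset's sign after the first spawn and is reset once the loop finishes.
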(event `/Game/Tech/Upgrades/BPC_BaseUpgrade.Upgrade_Projectile`
  (params (`Inaccuracy (half-degrees)` :type "Float (double-precision)") (`Projectile Type` :type "/Game/Tech/Projectiles/BP_Projectile Class Reference") (Damage :type "Float (double-precision)") (`Shot Upgrades` :type "Array of /Game/Tech/Upgrades/BPC_ChainLightning Object Reference (by ref)"))
  (bind _trajectory (`self.Trajectory`))
  (set `self.Direction Offset` 15.0)
  (set `self.Trajectory` (`self.F_Calculate Trajectory` `Inaccuracy (half-degrees)`))
  (for _ (range 1 3)
    (`|SpawnActorFromClass` `Projectile Type` (`KismetMathLibrary.MakeTransform` (.location _trajectory) (`KismetMathLibrary.MakeRotator` (.roll (.rotation _trajectory)) (.pitch (.rotation _trajectory)) (+ (.yaw (.rotation _trajectory)) (`self.Direction Offset`)))) "Undefined" "OverrideRootScale" (`self.GetOwner`) Damage `Shot Upgrades` null)
    (`/Engine/EditorBlueprintResources/StandardMacros.DoOnce` false :!label _label
      (:`Completed`
        (set `self.Direction Offset` (* (`self.Direction Offset`) -1.0)))))
  (`self.Reset`))

(event `Reset`
  (goto _label :!via `Reset`))