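; BPC_ChainLightning is an upgrade component that chains damage from a hit enemy to nearby pawns.
; BeginPlay finds the owning BP_Player up the owner chain and adds it to the ignore list.
; UpgradeHitEnemy sphere-traces around a stored location, line-traces to each pawn and applies a fifth of the damage.
; Successful hits move that location, join the never-cleared ignore list and recursively trigger the event with reduced damage.
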(event `self.ReceiveBeginPlay`
  (bind _returnvalue (`Actor.GetOwner` (`self.GetOwner`)))
  (bind (_asbp_player _bsuccess) (cast `/Game/Tech/Character/BP_Player` _returnvalue :!pure true))
  (bind (_asbp_player_2 _bsuccess_2) (cast `/Game/Tech/Character/BP_Player` (`Actor.GetOwner` _returnvalue) :!pure true))
  (`parent.ReceiveBeginPlay`)
  (if _bsuccess
    (set `self.Owner` _asbp_player)
    (`KismetArrayLibrary.Array_Add` (`self.Actors to Ignore`) (`self.Owner`) :!label _label)
    (elif _bsuccess_2
      (set `self.Owner` _asbp_player_2)
      (goto _label))))

(event `self.Upgrade_HitEnemy`
  (params (Damage :type "Float (double-precision)") (Location :type "Vector Structure"))
  (bind _location (`self.Location`))
  (set `self.Damage` Damage)
  (`|ExecutionSequence`
    (:`then_0`
      (`/Engine/EditorBlueprintResources/StandardMacros.DoOnce` false
        (:`Completed`
          (set `self.Location` Location))))
    (:`then_1`
      (bind _outhits (`KismetSystemLibrary.SphereTraceMultiForObjects` _location _location 250.0 (`|MakeArray` "ObjectTypeQuery3" :!type "EObjectTypeQuery Enum") false (`self.Actors to Ignore`)))
      (for _array_element _outhits
        (bind (_bblockinghit _binitialoverlap _time _distance _location_2 _impactpoint _normal _impactnormal _physmat _hitactor _hitcomponent _hitbonename _bonename _hititem _elementindex _faceindex _tracestart) (`GameplayStatics.BreakHitResult` _array_element))
        (bind _outhit (`KismetSystemLibrary.LineTraceSingle` _tracestart (`Actor.K2_GetActorLocation` _hitactor) "TraceTypeQuery1" false (`self.Actors to Ignore`) "ForDuration"))
        (bind (_bblockinghit_2 _binitialoverlap_2 _time_2 _distance_2 _location_3 _impactpoint_2 _normal_2 _impactnormal_2 _physmat_2 _hitactor_2) (`GameplayStatics.BreakHitResult` _outhit))
        (bind _target_hit_ (message `/Game/Tech/HealthSystem/BPI_DamageHandling.I_ApplyDamage` _hitactor_2 (* (`self.Damage`) 0.2) (`self.Owner`)))
        (if _target_hit_
          (set `self.Location` (`Actor.K2_GetActorLocation` _hitactor_2))
          (`KismetArrayLibrary.Array_Add` (`self.Actors to Ignore`) _hitactor_2)
          (`self.Upgrade_HitEnemy` (* (`self.Damage`) 0.2)))))))