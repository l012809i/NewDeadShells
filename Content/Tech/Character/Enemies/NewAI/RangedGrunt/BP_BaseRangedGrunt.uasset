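; Base ranged grunt enemy that shoots projectiles at the player and can be frozen, slowed or knocked back.
; Entering activation range starts a firing timer, with a reload pause gated by ShotCount, which is never incremented here.
; Looping timers drive AIMoveTo to chase the player, or retreat while the player overlaps the too-close hitbox.
; Damage and healing pass through a health component to update the overhead bar; death ragdolls, then destroys the actor.
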(event `self.ReceiveBeginPlay`
  (`self.Set References`)
  (`self.HealthBar`))

(event `/Game/Tech/Projectiles/NewProjectiles/BPI_ProjectileInterface.Freeze enemies`
  (params (`Freeze Length` :type "Float (double-precision)"))
  ;[0.9922 0.6667 1] Cold fusion freeze
  (`CharacterMovementComponent.DisableMovement` (`self.CharacterMovement`))
  (set `self.Frozen` true)
  (`KismetSystemLibrary.K2_SetTimerDelegate` (`|CreateDelegate` :!event `Unfreeze`) `Freeze Length`))

(event `Set References`
  (bind _returnvalue (`GameplayStatics.GetActorOfClass` "/Game/Tech/Character/BP_Player.BP_Player_C"))
  (set `self.Player` _returnvalue))

(event `Unfreeze`
  ;[0.9922 0.6667 1] Cold fusion unfreeze
  (`CharacterMovementComponent.SetMovementMode` (`self.CharacterMovement`) "MOVE_NavWalking" 0)
  (set `self.Frozen` false))

(event `/Game/Tech/Projectiles/NewProjectiles/BPI_ProjectileInterface.ApplyKnockback`
  (params (`Forward vector` :type "Vector Structure") (Amount :type "Float (double-precision)"))
  ;[0.9922 0.6667 1] Knockback
  (`CharacterMovementComponent.AddImpulse` (`self.CharacterMovement`) (* `Forward vector` Amount) true))

(event `/Game/Tech/Projectiles/NewProjectiles/BPI_ProjectileInterface.Slow`
  (bind _charactermovement (`self.CharacterMovement`))
  ;[0.9922 0.6667 1] Bubble slows
  (set `CharacterMovementComponent.MaxWalkSpeed` 300.0 _charactermovement)
  (`KismetSystemLibrary.Delay` 1.0)
  (set `CharacterMovementComponent.MaxWalkSpeed` 600.0 _charactermovement))

(event `self.TooCloseHitbox.OnComponentBeginOverlap`
  (params (OverlappedComponent :type "PrimitiveComponent Object Reference") (OtherActor :type "Actor Object Reference") (OtherComp :type "PrimitiveComponent Object Reference") (OtherBodyIndex :type Integer) (bFromSweep :type Boolean) (SweepResult :type "HitResult Structure (by ref)"))
  ;[1 1 1] Ranged Grunt Functionality
  (bind _asbp_player (cast `/Game/Tech/Character/BP_Player` OtherActor))
  (set `self.Player` _asbp_player)
  (bind _returnvalue (`KismetSystemLibrary.K2_SetTimerDelegate` (delegate `Move Away`) 0.01 true))
  (set `self.StopMoveAway` _returnvalue)
  (`KismetSystemLibrary.K2_ClearAndInvalidateTimerHandle` (`self.StopMoveTowards`)))

(event `Move Away`
  (bind _returnvalue (`self.K2_GetActorLocation`))
  ;[1 1 1] Ranged Grunt Functionality
  (`|AIMoveTo` self (+ _returnvalue (- _returnvalue (`self.K2_GetActorLocation` (`self.Player`)))) null 100.0))

(event `self.TooCloseHitbox.OnComponentEndOverlap`
  (params (OverlappedComponent :type "PrimitiveComponent Object Reference") (OtherActor :type "Actor Object Reference") (OtherComp :type "PrimitiveComponent Object Reference") (OtherBodyIndex :type Integer))
  ;[1 1 1] Ranged Grunt Functionality
  (bind _asbp_player (cast `/Game/Tech/Character/BP_Player` OtherActor))
  (set `self.Player` _asbp_player)
  (bind _returnvalue (`KismetSystemLibrary.K2_SetTimerDelegate` (delegate `Move Towards`) 0.01 true :!label _label))
  (set `self.StopMoveTowards` _returnvalue)
  (`KismetSystemLibrary.K2_ClearAndInvalidateTimerHandle` (`self.StopMoveAway`)))

(event `HealthBar`
  (bind (_health _maxhealth) (break `/Game/Tech/HealthSystem/S_Health` (`/Game/Tech/HealthSystem/BPC_HealthComponent.S_Health` (`self.BPC_HealthComponent`))))
  ;[1 1 1] HealthBar Updating
  (add `self.E_HealthUpdated` (delegate `Update HealthBar`))
  (bind _aswb_aihealth_bar (cast `/Game/Tech/UI/UI_Enemies/WB_AIHealthBar` (`WidgetComponent.GetUserWidgetObject` (`self.HealthBarWidget`)) :!label _label_2))
  (bind _output_get (set `/Game/Tech/UI/UI_Enemies/WB_AIHealthBar.Health` _health _aswb_aihealth_bar))
  (`ProgressBar.SetPercent` (`/Game/Tech/UI/UI_Enemies/WB_AIHealthBar.HealthBarProgress` _aswb_aihealth_bar) (/ _health _maxhealth))
  (`TextBlock.SetText` (`/Game/Tech/UI/UI_Enemies/WB_AIHealthBar.HealthText` _aswb_aihealth_bar) (`KismetTextLibrary.Conv_DoubleToText` _output_get "HalfToEven")))

(event `Move Towards`
  ;[1 1 1] Ranged Grunt Functionality
  (`|AIMoveTo` self (`self.K2_GetActorLocation` (`self.Player`)) null 100.0))

(event `Update HealthBar` :!signature `self.E_HealthUpdated`
  (params (Health :type "/Game/Tech/HealthSystem/S_Health Structure"))
  ;[1 1 1] HealthBar Updating
  (`KismetSystemLibrary.K2_SetTimerDelegate` (delegate `Update`) 0.01 true))

(event `self.ActivationRange.OnComponentBeginOverlap`
  (params (OverlappedComponent :type "PrimitiveComponent Object Reference") (OtherActor :type "Actor Object Reference") (OtherComp :type "PrimitiveComponent Object Reference") (OtherBodyIndex :type Integer) (bFromSweep :type Boolean) (SweepResult :type "HitResult Structure (by ref)"))
  ;[1 1 1] Ranged Grunt Functionality
  (cast `/Game/Tech/Character/BP_Player` OtherActor)
  (set `self.IsShooting` true)
  (bind _returnvalue (`KismetSystemLibrary.K2_SetTimerDelegate` (delegate `Shoot`) (`self.FireRate`) true))
  (set `self.ShootingHandler` _returnvalue)
  (goto _label))

(event `Update`
  ;[1 1 1] HealthBar Updating
  (goto _label_2))

(event `Shoot`
  (bind _shootinghandler (`self.ShootingHandler`))
  ;[1 1 1] Ranged Grunt Functionality
  (if (<= (`self.ShotCount`) (`self.ReloadCount`))
    (`self.LookAtPlayer`)
    (`|SpawnActorFromClass` :`Class` "/Game/Tech/Projectiles/NewProjectiles/BP_NormalProjectile.BP_NormalProjectile_C" :`SpawnTransform` (`SceneComponent.K2_GetComponentToWorld` (`self.Projectilespawn`)) :`CollisionHandlingOverride` "AdjustIfPossibleButAlwaysSpawn" :`TransformScaleMethod` "OverrideRootScale" :`Damage` (`self.Damage`) :`Instigator` null)
    (else
      (`KismetSystemLibrary.K2_PauseTimerHandle` _shootinghandler)
      (`KismetSystemLibrary.Delay` (`self.ReloadSpeed`))
      (`KismetSystemLibrary.K2_UnPauseTimerHandle` _shootinghandler))))

(fn `Death`
  (`self.K2_DestroyActor`))

(fn `Get freeze`
  (returns (Frozen :type Boolean))
  (return (`self.Frozen`)))

(fn `I Get BP Base Enemy`
  (returns (Enemy :type "Character Object Reference"))
  (return self))

(fn `I_ApplyDamage`
  (params (Damage :type "Float (double-precision)") (Instigator :type "Actor Object Reference"))
  (returns (`Target Hit?` :type Boolean) (`Target Dead?` :type Boolean))
  (bind _bpc_healthcomponent (`self.BPC_HealthComponent`))
  ;[0 1 1] Sending damage to health component and updating event dispatcher for UI
  (bind (_target_hit_ _target_dead_) (`/Game/Tech/HealthSystem/BPC_HealthComponent.I_ApplyDamage` _bpc_healthcomponent Damage Instigator))
  (`self.E_HealthUpdated` (`/Game/Tech/HealthSystem/BPC_HealthComponent.S_Health` _bpc_healthcomponent))
  (if _target_dead_
    (`PrimitiveComponent.SetSimulatePhysics` (`self.Mesh`) true) ; Enable Ragdoll
    (`PrimitiveComponent.SetCollisionEnabled` (`self.Mesh`) "NoCollision")
    (bind _returnvalue (`KismetSystemLibrary.K2_SetTimer` null "Death" 5.0)) ; 5 Second delay before Destroying Character
    (set `self.TimerHandler` _returnvalue)
    (return _target_hit_ _target_dead_)
    (else
      (return _target_hit_ _target_dead_))))

(fn `I_ApplyHealing`
  (params (Healing :type "Float (double-precision)") (Instigator :type "Actor Object Reference"))
  (returns (`Target Full?` :type Boolean))
  (bind _bpc_healthcomponent (`self.BPC_HealthComponent`))
  ;[0 1 1] Sending healing to health component and updating event dispatcher for UI
  (bind _target_full_ (`/Game/Tech/HealthSystem/BPC_HealthComponent.I_ApplyHealing` _bpc_healthcomponent Healing Instigator))
  (`self.E_HealthUpdated` (`/Game/Tech/HealthSystem/BPC_HealthComponent.S_Health` _bpc_healthcomponent))
  (return _target_full_))

(fn `I_ChangeMaxHealth`
  (params (`Max Health` :type "Float (double-precision)") (Instigator :type "Actor Object Reference"))
  (returns (`Return Value` :type Boolean))
  (return false))

(fn `I_GetHealthStruct`
  (returns (`Health Struct` :type "/Game/Tech/HealthSystem/S_Health Structure"))
  (return))

(fn `LookAtPlayer`
  (bind _returnvalue (`self.K2_GetActorLocation` (`self.Player`)))
  (bind _returnvalue_2 (`KismetAnimationLibrary.K2_LookAt` (`self.GetTransform`) _returnvalue _returnvalue))
  (`self.K2_SetActorTransform` (`KismetMathLibrary.MakeTransform` (.location _returnvalue_2) (`KismetMathLibrary.MakeRotator` 0.0 0.0 (+ (.yaw (.rotation _returnvalue_2)) 90.0)) (.scale _returnvalue_2))))

(fn `UserConstructionScript`)