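; BP_BaseEnemyRed is a red enemy Blueprint that inherits its construction, healing and damage behavior from a parent class.
; The healing and damage interface functions only forward to the parent implementations and return their results.
; The max-health change and health-struct getter are stubs that skip the parent, returning false and an empty result.
; The event graph holds no active logic.
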(fn `I_ApplyDamage`
  (params (Damage :type "Float (double-precision)") (Instigator :type "Actor Object Reference"))
  (returns (`Target Hit?` :type Boolean) (`Target Dead?` :type Boolean))
  (bind (_target_hit_ _target_dead_) (`parent.I_ApplyDamage` Damage Instigator))
  (return _target_hit_ _target_dead_))

(fn `I_ApplyHealing`
  (params (Healing :type "Float (double-precision)") (Instigator :type "Actor Object Reference"))
  (returns (`Target Full?` :type Boolean))
  (bind _target_full_ (`parent.I_ApplyHealing` Healing Instigator))
  (return _target_full_))

(fn `I_ChangeMaxHealth`
  (params (`Max Health` :type "Float (double-precision)") (Instigator :type "Actor Object Reference"))
  (returns (`Return Value` :type Boolean))
  (return false))

(fn `I_GetHealthStruct`
  (returns (`Health Struct` :type "/Game/Tech/HealthSystem/S_Health Structure"))
  (return))

(fn `UserConstructionScript`
  (`parent.UserConstructionScript`))