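; Base melee grunt enemy that chases the player on entering its activation range and periodically attacks.
; Looping timers drive AI movement and attack choice: a close-range montage swing, or a timeline dash with mesh spin, both using sphere traces to deal damage.
; A health component handles damage, feeding a timer-refreshed health bar and triggering ragdoll death with delayed removal.
; Events add freeze, knockback and slow; coin spawning is disconnected.
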(event `self.ReceiveBeginPlay`
  (bind (_health _maxhealth) (break `/Game/Tech/HealthSystem/S_Health` (`/Game/Tech/HealthSystem/BPC_HealthComponent.S_Health` (`self.BPC_HealthComponent`))))
  (bind _returnvalue (`GameplayStatics.GetActorOfClass` "/Game/Tech/Character/BP_Player.BP_Player_C"))
  ;[1 1 1] HealthBar Live Update Very messy code
  (set `self.Player` _returnvalue)
  (add `self.E_HealthUpdated` (delegate `Update HealthBar`))
  (bind _aswb_aihealth_bar (cast `/Game/Tech/UI/UI_Enemies/WB_AIHealthBar` (`WidgetComponent.GetUserWidgetObject` (`self.HealthBar`)) :!label _label))
  (bind _output_get (set `/Game/Tech/UI/UI_Enemies/WB_AIHealthBar.Health` _health _aswb_aihealth_bar))
  (`ProgressBar.SetPercent` (`/Game/Tech/UI/UI_Enemies/WB_AIHealthBar.HealthBarProgress` _aswb_aihealth_bar) (/ _health _maxhealth))
  (`TextBlock.SetText` (`/Game/Tech/UI/UI_Enemies/WB_AIHealthBar.HealthText` _aswb_aihealth_bar) (`KismetTextLibrary.Conv_DoubleToText` _output_get "HalfToEven")))

(event `Update HealthBar` :!signature `self.E_HealthUpdated`
  (params (Health :type "/Game/Tech/HealthSystem/S_Health Structure"))
  ;[1 1 1] HealthBar Live Update Very messy code
  (`KismetSystemLibrary.K2_SetTimerDelegate` (delegate `Update`) 0.01 true))

(event `Update`
  ;[1 1 1] HealthBar Live Update Very messy code
  (goto _label))

(event `/Game/Tech/Projectiles/NewProjectiles/BPI_ProjectileInterface.Freeze enemies`
  (params (`Freeze Length` :type "Float (double-precision)"))
  ;[0.9922 0.6667 1] Cold fusion freeze
  (`CharacterMovementComponent.DisableMovement` (`self.CharacterMovement`))
  (set `self.Frozen` true)
  (`KismetSystemLibrary.K2_SetTimerDelegate` (`|CreateDelegate` :!event `Unfreeze`) `Freeze Length`))

(event `Unfreeze`
  ;[0.9922 0.6667 1] Cold fusion unfreeze
  (`CharacterMovementComponent.SetMovementMode` (`self.CharacterMovement`) "MOVE_NavWalking" 0)
  (set `self.Frozen` false))

(event `/Game/Tech/Projectiles/NewProjectiles/BPI_ProjectileInterface.ApplyKnockback`
  (params (`Forward vector` :type "Vector Structure") (Amount :type "Float (double-precision)"))
  ;[0.9922 0.6667 1] Knockback
  (`CharacterMovementComponent.AddImpulse` (`self.CharacterMovement`) (* `Forward vector` Amount) true))

(event `/Game/Tech/Projectiles/NewProjectiles/BPI_ProjectileInterface.Slow`
  (bind _charactermovement (`self.CharacterMovement`))
  ;[0.9922 0.6667 1] Bubble slows
  (set `CharacterMovementComponent.MaxWalkSpeed` 300.0 _charactermovement)
  (`KismetSystemLibrary.Delay` 1.0)
  (set `CharacterMovementComponent.MaxWalkSpeed` 600.0 _charactermovement))

(event `Attack`
  (bind _mesh (`self.Mesh`))
  (bind _returnvalue (`KismetMathLibrary.MakeVector` (.x (`SceneComponent.K2_GetComponentLocation` _mesh)) (.y (`SceneComponent.K2_GetComponentLocation` _mesh)) (+ (.z (`SceneComponent.K2_GetComponentLocation` _mesh)) 89.0)))
  (`|PlayMontage` (`self.Mesh`) "/Game/Tech/Enemies/MeleeGrunt/Animation/Melee_Grunt_Attack_Montage.Melee_Grunt_Attack_Montage" 0.3
    (:`then`
      ;[1 1 1] Draw Line Trace
      (bind (_outhit _returnvalue_2) (`KismetSystemLibrary.SphereTraceSingle` _returnvalue (+ _returnvalue (* (`SceneComponent.GetRightVector` _mesh) 200.0)) 30.0 "TraceTypeQuery1" false (`self.IgnoreEnemies`) "ForDuration"))
      (if _returnvalue_2
        (bind (_bblockinghit _binitialoverlap _time _distance _location _impactpoint _normal _impactnormal _physmat _hitactor) (`GameplayStatics.BreakHitResult` _outhit))
        (`KismetSystemLibrary.PrintString` (`KismetSystemLibrary.GetDisplayName` _hitactor))
        ;[1 1 1] Apply Damage to the player
        (if (== (`GameplayStatics.GetObjectClass` _hitactor) "/Game/Tech/Character/BP_Player.BP_Player_C")
          (bind _asbp_player (cast `/Game/Tech/Character/BP_Player` _hitactor))
          (message `/Game/Tech/HealthSystem/BPI_DamageHandling.I_ApplyDamage` _asbp_player (`.Damage_49_A01B425145A12C889FD0F9848EDABD6D` (break `/Game/Tech/Enemies/MeleeGrunt/S_MeleeGrunt` (`self.Stats`))) null))))))

(event `self.Activation Range.OnComponentBeginOverlap`
  (params (OverlappedComponent :type "PrimitiveComponent Object Reference") (OtherActor :type "Actor Object Reference") (OtherComp :type "PrimitiveComponent Object Reference") (OtherBodyIndex :type Integer) (bFromSweep :type Boolean) (SweepResult :type "HitResult Structure (by ref)"))
  (bind _asbp_player (cast `/Game/Tech/Character/BP_Player` OtherActor))
  (set `self.Player` _asbp_player)
  (bind _returnvalue (`KismetSystemLibrary.K2_SetTimerDelegate` (delegate `Move Towards`) 0.05 true))
  (set `self.Stop Move Towards` _returnvalue)
  (`KismetSystemLibrary.K2_ClearAndInvalidateTimerHandle` (`self.Stop Move Away`))
  (`KismetSystemLibrary.Delay` (`self.Attack Delay+ on Start`))
  (bind _returnvalue_2 (`KismetSystemLibrary.K2_SetTimerDelegate` (delegate `Can Attack`) 3.0 true))
  (set `self.Can Attack Handler` _returnvalue_2))

(event `Can Attack`
  (bind _returnvalue (`self.K2_GetActorLocation`))
  (bind _startrotation (`self.StartRotation`))
  (bind _mesh (`self.Mesh`))
  (bind _returnvalue_2 (- (`self.K2_GetActorLocation` (`self.Player`)) _returnvalue))
  (bind _returnvalue_3 (`KismetMathLibrary.MakeVector` (.x (`SceneComponent.K2_GetComponentLocation` _mesh)) (.y (`SceneComponent.K2_GetComponentLocation` _mesh)) (+ (.z (`SceneComponent.K2_GetComponentLocation` _mesh)) 89.0)))
  (if (<= (`KismetMathLibrary.VSize` _returnvalue_2) 230.0)
    (`self.Attack`)
    (else
      (set `self.DashStart` _returnvalue)
      (set `self.DashEnd` (+ _returnvalue (* (`KismetMathLibrary.Normal` _returnvalue_2) 300.0)))
      (set `self.StartRotation` (`SceneComponent.RelativeRotation` (`self.Mesh`)))
      (`|PlayMontage` (`self.Mesh`) "/Game/Tech/Enemies/MeleeGrunt/Animation/Melee_Grunt_Attack_Montage.Melee_Grunt_Attack_Montage" 0.3
        (:`then`
          (bind (_direction _newtrack_0 _newtrack_1) (`Timeline|Dash` :!via `PlayFromStart`)
            (:`Update`
              (`self.K2_SetActorLocation` (`KismetMathLibrary.VLerp` (`self.DashStart`) (`self.DashEnd`) _newtrack_0))
              (`SceneComponent.K2_SetRelativeRotation` (`self.Mesh`) (`KismetMathLibrary.RLerp` _startrotation (`KismetMathLibrary.MakeRotator` (.roll _startrotation) (+ (.pitch _startrotation) 360.0) (.yaw _startrotation)) _newtrack_1) false false)
              (if (not (`self.Hit`))
                (bind (_outhit _returnvalue_4) (`KismetSystemLibrary.SphereTraceSingle` _returnvalue_3 (+ _returnvalue_3 (* (`SceneComponent.GetRightVector` _mesh) 200.0)) 30.0 "TraceTypeQuery1" false (`self.IgnoreEnemies`) "ForDuration"))
                (if _returnvalue_4
                  (bind (_bblockinghit _binitialoverlap _time _distance _location _impactpoint _normal _impactnormal _physmat _hitactor) (`GameplayStatics.BreakHitResult` _outhit))
                  (`KismetSystemLibrary.PrintString` (`KismetSystemLibrary.GetDisplayName` _hitactor))
                  (if (== (`GameplayStatics.GetObjectClass` _hitactor) "/Game/Tech/Character/BP_Player.BP_Player_C")
                    (bind _asbp_player (cast `/Game/Tech/Character/BP_Player` _hitactor))
                    (message `/Game/Tech/HealthSystem/BPI_DamageHandling.I_ApplyDamage` _asbp_player (`.Damage_49_A01B425145A12C889FD0F9848EDABD6D` (break `/Game/Tech/Enemies/MeleeGrunt/S_MeleeGrunt` (`self.Stats`))) null)
                    (set `self.Hit` true)))))))))))

(event `Move Towards`
  (`|AIMoveTo` self (`self.K2_GetActorLocation` (`self.Player`)) null 100.0))

(fn `Death`
  (`PrimitiveComponent.SetSimulatePhysics` (`self.Mesh`) true)
  (`PrimitiveComponent.SetCollisionEnabled` (`self.CapsuleComponent`) "NoCollision")
  (bind _asmelee_grunt_aicontroller (cast `/Game/Tech/Enemies/MeleeGrunt/MeleeGruntAIController` (`AIBlueprintHelperLibrary.GetAIController` null)))
  (`Controller.UnPossess` _asmelee_grunt_aicontroller)
  (`self.SpawnCoin`))

(fn `Get freeze`
  (returns (Frozen :type Boolean))
  (return (`self.Frozen`)))

(fn `I_ApplyDamage`
  (params (Damage :type "Float (double-precision)") (Instigator :type "Actor Object Reference"))
  (returns (`Target Hit?` :type Boolean) (`Target Dead?` :type Boolean))
  (bind (_target_hit_ _target_dead_) (`/Game/Tech/HealthSystem/BPI_DamageHandling.I_ApplyDamage` (`self.BPC_HealthComponent`) Damage Instigator))
  (`self.E_HealthUpdated` (`/Game/Tech/HealthSystem/BPC_HealthComponent.S_Health` (`self.BPC_HealthComponent`)))
  (if _target_dead_
    (`self.Death`)
    (bind _returnvalue (`KismetSystemLibrary.K2_SetTimer` null "Remove" 3.0))
    (set `self.TimeUntilDead` _returnvalue)
    (return _target_hit_ _target_dead_)
    (else
      (return _target_hit_ _target_dead_))))

(fn `I_ApplyHealing`
  (params (Healing :type "Float (double-precision)") (Instigator :type "Actor Object Reference"))
  (returns (`Target Full?` :type Boolean))
  (return false))

(fn `I_ChangeMaxHealth`
  (params (`Max Health` :type "Float (double-precision)") (Instigator :type "Actor Object Reference"))
  (returns (`Return Value` :type Boolean))
  (return false))

(fn `I_GetHealthStruct`
  (returns (`Health Struct` :type "/Game/Tech/HealthSystem/S_Health Structure"))
  (bind _health_struct (`/Game/Tech/HealthSystem/BPI_DamageHandling.I_GetHealthStruct` (`self.BPC_HealthComponent`)))
  (return _health_struct))

(fn `Remove`
  (`self.K2_DestroyActor`))

(fn `SpawnCoin`)

(fn `UserConstructionScript`)