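; Jellyfish enemy projectile that flies toward the player and bursts into a temporary electric damage field.
; A timeline sweeps it 1000 units toward the player's position at spawn, with capsule overlap dealing projectile damage.
; At travel's end it reveals the explosion, and a looping timer damages the player within range through IApplyDamage.
; After three seconds the timer clears and a second timeline shrinks the actor before destroying it.
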(event `self.ReceiveBeginPlay`
  (bind _returnvalue (`self.K2_GetActorLocation`))
  (bind _returnvalue_2 (`GameplayStatics.CreateSound2D` "/Game/Tech/Sounds/Enemies/Jellyfish/Jellyfish_Ball_Cue.Jellyfish_Ball_Cue" 1.0 1.0 0.0 null))
  (`AudioComponent.Play` _returnvalue_2 0.0)
  (bind _returnvalue_3 (`GameplayStatics.GetActorOfClass` "/Game/Tech/Character/BP_Player.BP_Player_C"))
  (bind _output_get (set `self.Player` _returnvalue_3))
  (set `self.StartLocation` _returnvalue)
  (set `self.EndLocation` (- _returnvalue (* (`KismetMathLibrary.Normal` (- _returnvalue (`self.K2_GetActorLocation` _output_get))) 1000.0)))
  (bind (_direction _newtrack_0) (`Timeline|Electroball Travel` :!via `PlayFromStart`)
    (:`Update`
      (`self.K2_SetActorLocation` (`KismetMathLibrary.VLerp` (`self.StartLocation`) (`self.EndLocation`) _newtrack_0) true))
    (:`Finished`
      (`SceneComponent.SetVisibility` (`self.Explosion`) true false)
      (`AudioComponent.Stop` _returnvalue_2)
      (`GameplayStatics.PlaySound2D` "/Game/Tech/Sounds/Enemies/Jellyfish/electric_ball_explosion.electric_ball_explosion" 1.0 1.0 0.0 null null)
      (bind _returnvalue_4 (`KismetSystemLibrary.K2_SetTimerDelegate` (delegate `Electric Damage`) 0.1 true))
      (set `self.ElectricDamageHandle` _returnvalue_4)
      (`KismetSystemLibrary.Delay` 3.0)
      (`KismetSystemLibrary.K2_ClearAndInvalidateTimerHandle` (`self.ElectricDamageHandle`))
      (set `self.Start Scale` (`self.GetActorScale3D`))
      (bind (_direction_2 _newtrack_0_2) (`Timeline|Shrink` :!via `PlayFromStart`)
        (:`Update`
          (`self.SetActorScale3D` (`KismetMathLibrary.VLerp` (`self.Start Scale`) (0.0 0.0 0.0) _newtrack_0_2)))
        (:`Finished`
          (`self.K2_DestroyActor`))))))

(event `Electric Damage`
  (if (<= (`KismetMathLibrary.VSize` (- (`self.K2_GetActorLocation`) (`self.K2_GetActorLocation` (`self.Player`)))) 400.0)
    (`/Game/Tech/HealthSystem/BPI_DamageHandling.I_ApplyDamage` (`self.Player`) (`self.ElectricfieldDPS/10`) null)))

(event `self.Capsule.OnComponentBeginOverlap`
  (params (OverlappedComponent :type "PrimitiveComponent Object Reference") (OtherActor :type "Actor Object Reference") (OtherComp :type "PrimitiveComponent Object Reference") (OtherBodyIndex :type Integer) (bFromSweep :type Boolean) (SweepResult :type "HitResult Structure (by ref)"))
  (bind _asbp_player (cast `/Game/Tech/Character/BP_Player` OtherActor))
  (`/Game/Tech/HealthSystem/BPI_DamageHandling.I_ApplyDamage` _asbp_player (`self.ProjectileDamage`) null))

(fn `UserConstructionScript`)