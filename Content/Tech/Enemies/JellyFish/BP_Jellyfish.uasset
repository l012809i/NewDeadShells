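; Jellyfish enemy that chases the player once they enter its activation range.
; Looping timers drive AI movement and attacks: a random chance of an electro ball, then a timeline-animated spin dealing radius damage, which re-arms the attack timer.
; It supports freeze and slow effects, while knockback is stubbed out.
; A health component handles damage and healing, feeding a health bar widget; death ragdolls the mesh before delayed destruction.
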(event `Unfreeze`
  (`CharacterMovementComponent.SetMovementMode` (`self.CharacterMovement`) "MOVE_NavWalking" 0)
  (set `self.Frozen` false))

(event `/Game/Tech/Projectiles/NewProjectiles/BPI_ProjectileInterface.Slow`
  (bind _charactermovement (`self.CharacterMovement`))
  (set `CharacterMovementComponent.MaxWalkSpeed` 300.0 _charactermovement)
  (`KismetSystemLibrary.Delay` 1.0)
  (set `CharacterMovementComponent.MaxWalkSpeed` 600.0 _charactermovement))

(event `/Game/Tech/Projectiles/NewProjectiles/BPI_ProjectileInterface.ApplyKnockback`
  (params (`Forward vector` :type "Vector Structure") (Amount :type "Float (double-precision)")))

(event `/Game/Tech/Projectiles/NewProjectiles/BPI_ProjectileInterface.Freeze enemies`
  (params (`Freeze Length` :type "Float (double-precision)"))
  (`CharacterMovementComponent.DisableMovement` (`self.CharacterMovement`))
  (set `self.Frozen` true)
  (`KismetSystemLibrary.K2_SetTimerDelegate` (`|CreateDelegate` :!event `Unfreeze`) `Freeze Length`))

(event `Move Towards`
  (`|AIMoveTo` self (`self.K2_GetActorLocation` (`self.Player`)) null 100.0
    (:`then`
      (`self.LookAtPlayer`))))

(event `self.ActivationRange.OnComponentBeginOverlap`
  (params (OverlappedComponent :type "PrimitiveComponent Object Reference") (OtherActor :type "Actor Object Reference") (OtherComp :type "PrimitiveComponent Object Reference") (OtherBodyIndex :type Integer) (bFromSweep :type Boolean) (SweepResult :type "HitResult Structure (by ref)"))
  (bind _asbp_player (cast `/Game/Tech/Character/BP_Player` OtherActor))
  (set `self.Player` _asbp_player)
  (bind _returnvalue (`KismetSystemLibrary.K2_SetTimerDelegate` (delegate `Move Towards`) 0.01 true))
  (set `self.StopMoveTowards` _returnvalue)
  (`KismetSystemLibrary.Delay` (`self.AttackDelay+OnStart`))
  (bind _returnvalue_2 (`KismetSystemLibrary.K2_SetTimerDelegate` (delegate `Can Attack`) 3.0 true :!label _label))
  (set `self.Can Attack Handler` _returnvalue_2))

(event `Can Attack`
  (if (not (`KismetMathLibrary.RandomBool`))
    (`|SpawnActorFromClass` "/Game/Tech/Enemies/JellyFish/BP_ElectroBall.BP_ElectroBall_C" (`KismetMathLibrary.MakeTransform` (`self.K2_GetActorLocation`)) "Undefined" "OverrideRootScale" null null))
  (`KismetSystemLibrary.K2_SetTimerDelegate` (delegate `Spin Attack`) 0.1)
  (`KismetSystemLibrary.K2_ClearAndInvalidateTimerHandle` (`self.Can Attack Handler`)))

(event `Spin Attack`
  (bind _mesh (`self.Mesh`))
  (bind (_orig_rotation_roll _orig_rotation_pitch _orig_rotation_yaw) (`KismetMathLibrary.BreakRotator` (`self.Orig Rotation`)))
  (bind (_relativelocation_x _relativelocation_y _relativelocation_z) (`KismetMathLibrary.BreakVector` (`SceneComponent.RelativeLocation` _mesh)))
  (bind (_relativerotation_roll _relativerotation_pitch _relativerotation_yaw) (`KismetMathLibrary.BreakRotator` (`SceneComponent.RelativeRotation` _mesh)))
  (`|PlayMontage` (`self.Mesh`) "/Game/Tech/Enemies/JellyFish/JellyFish_Attack_Montage.JellyFish_Attack_Montage" 0.6
    (:`then`
      (`|ExecutionSequence`
        (:`then_0`
          (set `self.OriginalHeight` (`KismetMathLibrary.MakeVector` _relativelocation_x _relativelocation_y _relativelocation_z))
          (set `self.SpinHeight` (`KismetMathLibrary.MakeVector` _relativelocation_x _relativelocation_y (- _relativelocation_z 250.0)))
          (set `self.Orig Rotation` (`KismetMathLibrary.MakeRotator` _relativerotation_roll _relativerotation_pitch _relativerotation_yaw))
          (set `self.New Rotation` (`KismetMathLibrary.MakeRotator` (- _relativerotation_roll -20.0) _relativerotation_pitch _relativerotation_yaw))
          (bind (_direction _spinmove) (`Timeline|Get into Spin Position` :!via `PlayFromStart` :!label _label_2)
            (:`Update`
              (`SceneComponent.K2_SetRelativeLocation` _mesh (`KismetMathLibrary.VLerp` (`self.OriginalHeight`) (`self.SpinHeight`) _spinmove) false false))
            (:`Finished`
              (if (`self.Done Spinning`)
                (`|PlayMontage` (`self.Mesh`) "/Game/Tech/Enemies/JellyFish/JellyFish_Attack_Montage.JellyFish_Attack_Montage" -1.0
                  (:`OnCompleted`
                    (set `self.Done Spinning` false)
                    (goto _label)))
                (else
                  (bind _returnvalue (`KismetSystemLibrary.K2_SetTimerDelegate` (delegate `Spin Deal Damage`) 0.1 true))
                  (set `self.Spin Damage Timer Handle` _returnvalue)
                  (bind (_direction_2 _newtrack_0) (`Timeline|Spin` :!via `PlayFromStart`)
                    (:`Update`
                      (`SceneComponent.K2_SetRelativeRotation` (`self.Mesh`) (`KismetMathLibrary.RLerp` (`KismetMathLibrary.MakeRotator` _orig_rotation_roll _orig_rotation_pitch _orig_rotation_yaw) (`KismetMathLibrary.MakeRotator` _orig_rotation_roll _orig_rotation_pitch (+ _orig_rotation_yaw 1800.0)) _newtrack_0) false false))
                    (:`Finished`
                      (`KismetSystemLibrary.K2_ClearAndInvalidateTimerHandle` (`self.Spin Damage Timer Handle`))
                      (set `self.Done Spinning` true)
                      (goto _label_2 :!via `Reverse`))))))))
        (:`then_1`
          (`KismetSystemLibrary.Delay` 1.5)
          (bind _returnvalue_2 (`GameplayStatics.CreateSound2D` "/Game/Tech/Sounds/Enemies/Jellyfish/jelly_spin.jelly_spin" 1.0 1.0 0.0 null false false))
          (`AudioComponent.Play` _returnvalue_2 0.0))))))

(event `Spin Deal Damage`
  (if (<= (`KismetMathLibrary.VSize` (- (`self.K2_GetActorLocation`) (`self.K2_GetActorLocation` (`self.Player`)))) 400.0)
    (`/Game/Tech/HealthSystem/BPI_DamageHandling.I_ApplyDamage` (`self.Player`) (`self.Spin DPS/10`) null)))

(event `self.ReceiveBeginPlay`
  (`self.Set References`)
  (`self.HealthBarUpdate`))

(event `Update HealthBar` :!signature `self.E_HealthUpdated`
  (params (Health :type "/Game/Tech/HealthSystem/S_Health Structure"))
  (`KismetSystemLibrary.K2_SetTimerDelegate` (delegate `Update`) 0.01 true))

(event `Update`
  (bind (_health _maxhealth) (break `/Game/Tech/HealthSystem/S_Health` (`/Game/Tech/HealthSystem/BPC_HealthComponent.S_Health` (`self.BPC_HealthComponent`))))
  (bind _aswb_aihealth_bar (cast `/Game/Tech/UI/UI_Enemies/WB_AIHealthBar` (`WidgetComponent.GetUserWidgetObject` (`self.HealthBar`)) :!label _label_3))
  (bind _output_get (set `/Game/Tech/UI/UI_Enemies/WB_AIHealthBar.Health` _health _aswb_aihealth_bar))
  (`ProgressBar.SetPercent` (`/Game/Tech/UI/UI_Enemies/WB_AIHealthBar.HealthBarProgress` _aswb_aihealth_bar) (/ _health _maxhealth))
  (`TextBlock.SetText` (`/Game/Tech/UI/UI_Enemies/WB_AIHealthBar.HealthText` _aswb_aihealth_bar) (`KismetTextLibrary.Conv_DoubleToText` _output_get "HalfToEven")))

(event `HealthBarUpdate`
  (add `self.E_HealthUpdated` (delegate `Update HealthBar`))
  (goto _label_3))

(event `Set References`
  (bind _returnvalue (`GameplayStatics.GetActorOfClass` "/Game/Tech/Character/BP_Player.BP_Player_C"))
  (set `self.Player` _returnvalue))

(fn `Death`
  (`self.K2_DestroyActor`))

(fn `Get freeze`
  (returns (Frozen :type Boolean))
  (return (`self.Frozen`)))

(fn `I_ApplyDamage`
  (params (Damage :type "Float (double-precision)") (Instigator :type "Actor Object Reference"))
  (returns (`Target Hit?` :type Boolean) (`Target Dead?` :type Boolean))
  (bind _bpc_healthcomponent (`self.BPC_HealthComponent`))
  ;[0 1 1] Sending damage to health component and updating event dispatcher for UI
  (bind (_target_hit_ _target_dead_) (`/Game/Tech/HealthSystem/BPC_HealthComponent.I_ApplyDamage` _bpc_healthcomponent Damage Instigator))
  (`self.E_HealthUpdated` (`/Game/Tech/HealthSystem/BPC_HealthComponent.S_Health` _bpc_healthcomponent))
  (if _target_dead_
    (`PrimitiveComponent.SetSimulatePhysics` (`self.Mesh`) true) ; Enable Ragdoll
    (`PrimitiveComponent.SetCollisionEnabled` (`self.Mesh`) "NoCollision")
    (`GameplayStatics.PlaySound2D` "/Game/Tech/Sounds/Enemies/Jellyfish/jelly_death.jelly_death" 1.0 1.0 0.0 null null)
    (bind _returnvalue (`KismetSystemLibrary.K2_SetTimer` null "Death" 5.0)) ; 5 Second delay before Destroying Character
    (set `self.TimerHandler` _returnvalue)
    (return _target_hit_ _target_dead_)
    (else
      (return _target_hit_ _target_dead_))))

(fn `I_ApplyHealing`
  (params (Healing :type "Float (double-precision)") (Instigator :type "Actor Object Reference"))
  (returns (`Target Full?` :type Boolean))
  (bind _bpc_healthcomponent (`self.BPC_HealthComponent`))
  ;[0 1 1] Sending healing to health component and updating event dispatcher for UI
  (bind _target_full_ (`/Game/Tech/HealthSystem/BPC_HealthComponent.I_ApplyHealing` _bpc_healthcomponent Healing Instigator))
  (`self.E_HealthUpdated` (`/Game/Tech/HealthSystem/BPC_HealthComponent.S_Health` _bpc_healthcomponent))
  (return _target_full_))

(fn `I_ChangeMaxHealth`
  (params (`Max Health` :type "Float (double-precision)") (Instigator :type "Actor Object Reference"))
  (returns (`Return Value` :type Boolean))
  (return false))

(fn `I_GetHealthStruct`
  (returns (`Health Struct` :type "/Game/Tech/HealthSystem/S_Health Structure"))
  (return))

(fn `LookAtPlayer`
  (bind _returnvalue (`self.K2_GetActorLocation` (`self.Player`)))
  (bind _returnvalue_2 (`KismetAnimationLibrary.K2_LookAt` (`self.GetTransform`) _returnvalue _returnvalue))
  (`self.K2_SetActorTransform` (`KismetMathLibrary.MakeTransform` (.location _returnvalue_2) (`KismetMathLibrary.MakeRotator` 0.0 0.0 (+ (.yaw (.rotation _returnvalue_2)) 90.0)) (.scale _returnvalue_2))))

(fn `UserConstructionScript`)