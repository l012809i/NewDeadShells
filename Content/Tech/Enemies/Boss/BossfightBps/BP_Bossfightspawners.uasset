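; Boss fight spawner actor that releases waves of melee grunt enemies.
; SpawnGrunts, not triggered within this Blueprint, spawns four grunts (green, base and two yellow) at fixed Billboard transforms when CanSpawn is true.
; It then clears CanSpawn and starts a 30-second timer to SpawnAgain, which re-enables the flag and calls SpawnGrunts, so waves repeat indefinitely once started.
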(event `self.ReceiveBeginPlay`)

(event `Spawn Grunts`
  (if (`self.Can Spawn?`)
    (`KismetSystemLibrary.PrintString` "spawning")
    (`|ExecutionSequence`
      (:`then_0`
        (`|SpawnActorFromClass` "/Game/Tech/Enemies/MeleeGrunt/BP_MeleeGrunt_Green.BP_MeleeGrunt_Green_C" (`SceneComponent.K2_GetComponentToWorld` (`self.Billboard`)) "Undefined" "OverrideRootScale" null null))
      (:`then_1`
        (`|SpawnActorFromClass` "/Game/Tech/Enemies/MeleeGrunt/BP_BaseMeleeGrunt.BP_BaseMeleeGrunt_C" (`SceneComponent.K2_GetComponentToWorld` (`self.Billboard1`)) "Undefined" "OverrideRootScale" null null))
      (:`then_2`
        (`|SpawnActorFromClass` "/Game/Tech/Enemies/MeleeGrunt/BP_MeleeGrunt_Yellow.BP_MeleeGrunt_Yellow_C" (`SceneComponent.K2_GetComponentToWorld` (`self.Billboard2`)) "Undefined" "OverrideRootScale" null null))
      (:`then_3`
        (`|SpawnActorFromClass` "/Game/Tech/Enemies/MeleeGrunt/BP_MeleeGrunt_Yellow.BP_MeleeGrunt_Yellow_C" (`SceneComponent.K2_GetComponentToWorld` (`self.Billboard3`)) "Undefined" "OverrideRootScale" null null)
        (set `self.Can Spawn?` false)
        (`KismetSystemLibrary.K2_SetTimerDelegate` (delegate `spawn again`) 30.0)))))

(event `spawn again`
  (set `self.Can Spawn?` true)
  (`self.Spawn Grunts`))

(fn `UserConstructionScript`)