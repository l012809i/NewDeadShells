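; Angler fish boss that spawns grunts, chases the player and ends the game when killed.
; A chomp on overlap starts a cooldown, which randomly unlocks a stationary line-traced water plume, enables a current pulling the player inward, or waits again.
; Damage goes through a health component, whose update event starts a looping timer that refreshes the health bar and also re-issues the chase.
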(event `self.ReceiveBeginPlay`
  (bind (_health _maxhealth) (break `/Game/Tech/HealthSystem/S_Health` (`/Game/Tech/HealthSystem/BPC_HealthComponent.S_Health` (`self.BPC_HealthComponent`))))
  (bind _returnvalue (`GameplayStatics.GetActorOfClass` "/Game/Tech/Character/BP_Player.BP_Player_C"))
  (set `self.Player` _returnvalue)
  (bind _returnvalue_2 (`GameplayStatics.GetActorOfClass` "/Game/Tech/Enemies/Boss/BossfightBps/BP_Bossfightspawners.BP_Bossfightspawners_C"))
  (bind _output_get (set `self.gruntSpawner` _returnvalue_2))
  (`/Game/Tech/Enemies/Boss/BossfightBps/BP_Bossfightspawners.Spawn Grunts` _output_get)
  ;[1 1 1] HealthBar Live Update Very messy code
  (add `self.E_HealthUpdated` (delegate `Update HealthBar`))
  (bind _aswb_aihealth_bar (cast `/Game/Tech/UI/UI_Enemies/WB_AIHealthBar` (`WidgetComponent.GetUserWidgetObject` (`self.HealthBar`)) :!label _label))
  (bind _output_get_2 (set `/Game/Tech/UI/UI_Enemies/WB_AIHealthBar.Health` _health _aswb_aihealth_bar))
  (`ProgressBar.SetPercent` (`/Game/Tech/UI/UI_Enemies/WB_AIHealthBar.HealthBarProgress` _aswb_aihealth_bar) (/ _health _maxhealth))
  (`TextBlock.SetText` (`/Game/Tech/UI/UI_Enemies/WB_AIHealthBar.HealthText` _aswb_aihealth_bar) (`KismetTextLibrary.Conv_DoubleToText` _output_get_2 "HalfToEven"))
  (`self.Start Boss Fight`))

(event `AI_Attack`)

(event `Update HealthBar` :!signature `self.E_HealthUpdated`
  (params (Health :type "/Game/Tech/HealthSystem/S_Health Structure"))
  ;[1 1 1] HealthBar Live Update Very messy code
  (`KismetSystemLibrary.K2_SetTimerDelegate` (delegate `Update`) 0.01 true))

(event `Update`
  ;[1 1 1] HealthBar Live Update Very messy code
  (goto _label))

(event `waterPlume`
  (`|SpawnActorFromClass` "/Game/Tech/Enemies/Boss/BossfightBps/BP_Bubbles.BP_Bubbles_C" (`SceneComponent.K2_GetComponentToWorld` (`self.Arrow1`)) "Undefined" "OverrideRootScale" null null))

(event `Start Boss Fight`
  (`self.Boss Move to Player`))

(event `self.ReceiveTick`
  (params (DeltaSeconds :type "Float (single-precision)"))
  (if (`self.facePlayer?`)
    (`self.K2_SetActorRotation` (`KismetMathLibrary.FindLookAtRotation` (`self.K2_GetActorLocation`) (`self.K2_GetActorLocation` (`self.Player`))))))

(event `Boss Move to Player`
  (bind _player (`self.Player`))
  (if (`self.facePlayer?`)
    (`|AIMoveTo` self (`self.K2_GetActorLocation` _player) _player
      (:`OnSuccess`
        (`self.Boss Move to Player`)))))

(event `Water Plume Attack`
  (bind _arrow1 (`self.Arrow1`))
  (bind _returnvalue (`SceneComponent.K2_GetComponentLocation` _arrow1))
  (if (`self.WaterPlumeattack`)
    (bind _returnvalue_2 (`GameplayStatics.CreateSound2D` "/Game/Tech/Sounds/Enemies/boss/water_plume.water_plume" 1.0 1.0 0.0 null))
    (`AudioComponent.Play` _returnvalue_2 0.0)
    (set `CharacterMovementComponent.MaxWalkSpeed` 0.0 (`self.CharacterMovement`))
    (`KismetSystemLibrary.PrintString` "Water Plume Attack" true true (struct :`R` 0.881954 :`G` 1.0 :`B` 0.420212 :`A` 1.0))
    (set `self.facePlayer?` false)
    (bind _outhit (`KismetSystemLibrary.LineTraceSingle` :`Start` _returnvalue :`End` (+ _returnvalue (* (`SceneComponent.GetForwardVector` _arrow1) 2000.0)) :`TraceChannel` "TraceTypeQuery1" :`DrawDebugType` "ForDuration"))
    (bind _asbp_player (cast `/Game/Tech/Character/BP_Player` (`.HitActor` (`GameplayStatics.BreakHitResult` _outhit))))
    (`/Game/Tech/Character/BP_Player.I_ApplyDamage` _asbp_player 10.0 null)
    (`KismetSystemLibrary.K2_SetTimerDelegate` (delegate `Water Plume Attack`) 1.0)
    (`KismetSystemLibrary.K2_SetTimerDelegate` (delegate `stop attack`) 4.0)))

(event `stop attack`
  (set `self.WaterPlumeattack` false)
  (set `self.facePlayer?` true)
  (`self.Boss Move to Player`)
  (set `CharacterMovementComponent.MaxWalkSpeed` 100.0 (`self.CharacterMovement`))
  (`AudioComponent.SetPaused` (stale `Water Plume Attack` _returnvalue_2) true))

(event `self.Sphere.OnComponentBeginOverlap`
  (params (OverlappedComponent :type "PrimitiveComponent Object Reference") (OtherActor :type "Actor Object Reference") (OtherComp :type "PrimitiveComponent Object Reference") (OtherBodyIndex :type Integer) (bFromSweep :type Boolean) (SweepResult :type "HitResult Structure (by ref)"))
  ;[1 1 1] Chomp Attack
  (bind _asbp_player (cast `/Game/Tech/Character/BP_Player` OtherActor))
  (if (`self.can attack?`)
    (`|PlayMontage` (`self.Mesh`) "/Game/Tech/Enemies/Boss/Animations/Angler_Attack_Montage.Angler_Attack_Montage" 2.0
      (:`then`
        (`/Game/Tech/Character/BP_Player.I_ApplyDamage` _asbp_player 10.0 null)
        (`GameplayStatics.PlaySound2D` "/Game/Tech/Sounds/Enemies/boss/chomp.chomp" 1.0 1.0 0.0 null null)
        (set `self.can attack?` false)
        (`KismetSystemLibrary.K2_SetTimerDelegate` (delegate `reset attack`) 3.0 :!label _label_2)))))

(event `reset attack`
  ;[1 1 1] Chomp Attack
  (set `self.can attack?` true)
  (`|MultiGate` true true
    (:`Out 0`
      (set `self.WaterPlumeattack` true)
      (`self.Water Plume Attack`))
    (:`Out 1`
      (set `self.current attack?` true))
    (:`Out 2`
      (goto _label_2))))

(event `current attack`)

(event `self.Sphere1.OnComponentBeginOverlap`
  (params (OverlappedComponent :type "PrimitiveComponent Object Reference") (OtherActor :type "Actor Object Reference") (OtherComp :type "PrimitiveComponent Object Reference") (OtherBodyIndex :type Integer) (bFromSweep :type Boolean) (SweepResult :type "HitResult Structure (by ref)"))
  (cast `/Game/Tech/Character/BP_Player` OtherActor)
  (if (`self.current attack?`)
    (bind _returnvalue (`KismetSystemLibrary.K2_SetTimerDelegate` (delegate `CustomEvent`) 0.04 true))
    (bind _returnvalue_2 (`GameplayStatics.CreateSound2D` "/Game/Tech/Sounds/Enemies/boss/boss_current.boss_current" 1.0 1.0 0.0 null))
    (`AudioComponent.Play` _returnvalue_2 0.0)))

(event `CustomEvent`
  (bind _player (`self.Player`))
  (bind _returnvalue (`KismetMathLibrary.GetDirectionUnitVector` (`self.K2_GetActorLocation` _player) (`self.K2_GetActorLocation`)))
  (bind (_returnvalue_x _returnvalue_y) (`KismetMathLibrary.BreakVector` (+ _returnvalue (* _returnvalue 4.0))))
  (`KismetSystemLibrary.PrintString` "in range")
  (`PawnMovementComponent.AddInputVector` (`Character.CharacterMovement` _player) (`KismetMathLibrary.MakeVector` _returnvalue_x _returnvalue_y) false))

(event `self.Sphere1.OnComponentEndOverlap`
  (params (OverlappedComponent :type "PrimitiveComponent Object Reference") (OtherActor :type "Actor Object Reference") (OtherComp :type "PrimitiveComponent Object Reference") (OtherBodyIndex :type Integer))
  (cast `/Game/Tech/Character/BP_Player` OtherActor)
  (`KismetSystemLibrary.PrintString` "OUT")
  (`KismetSystemLibrary.K2_PauseTimerHandle` (stale `self.Sphere1.OnComponentBeginOverlap` _returnvalue))
  (`AudioComponent.SetPaused` (stale `self.Sphere1.OnComponentBeginOverlap` _returnvalue_2) true))

(fn `I Get BP Base Enemy`
  (returns (Enemy :type "Character Object Reference"))
  (return null))

(fn `I_ApplyDamage`
  (params (Damage :type "Float (double-precision)") (Instigator :type "Actor Object Reference"))
  (returns (`Target Hit?` :type Boolean) (`Target Dead?` :type Boolean))
  (bind _bpc_healthcomponent (`self.BPC_HealthComponent`))
  (bind (_target_hit_ _target_dead_) (`self.I_ApplyDamage` _bpc_healthcomponent Damage Instigator))
  (`self.E_HealthUpdated` (`/Game/Tech/HealthSystem/BPC_HealthComponent.S_Health` _bpc_healthcomponent))
  (if _target_dead_
    (`self.K2_DestroyActor`)
    (`/Game/Tech/Blueprints/BP_TopDownGameMode.End-Game` (cast `/Game/Tech/Blueprints/BP_TopDownGameMode` (`GameplayStatics.GetGameMode`) :!pure true))
    (return _target_hit_ _target_dead_)
    (else
      (return _target_hit_ _target_dead_))))

(fn `I_ApplyHealing`
  (params (Healing :type "Float (double-precision)") (Instigator :type "Actor Object Reference"))
  (returns (`Target Full?` :type Boolean))
  (return false))

(fn `I_ChangeMaxHealth`
  (params (`Max Health` :type "Float (double-precision)") (Instigator :type "Actor Object Reference"))
  (returns (`Return Value` :type Boolean))
  (return false))

(fn `I_GetHealthStruct`
  (returns (`Health Struct` :type "/Game/Tech/HealthSystem/S_Health Structure"))
  (bind _health_struct (`self.I_GetHealthStruct` (`self.BPC_HealthComponent`)))
  (return _health_struct))

(fn `UserConstructionScript`)