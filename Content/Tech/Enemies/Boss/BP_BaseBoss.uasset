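; Base boss enemy that roams to random reachable points, damages the player on box overlap, and ends the game when killed.
; Roaming re-triggers after each successful AI move while IsRoaming is set.
; Damage and healing interface calls forward to the health component and broadcast updates for UI; death ragdolls the mesh and calls EndGame on the game mode.
; A looping timer draws debug health and name overhead; Death and max-health functions are stubs.
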(event `self.ReceiveBeginPlay`
  (`self.Display Debug Health`)
  (`self.Random Roam`))

(event `Random Roam`
  ;[1 1 1] AI Roaming - Roaming to itself (creating random location)
  (if (`self.isRoaming`)
    (`|AIMoveTo` self (`NavigationSystemV1.K2_GetRandomReachablePointInRadius` (`self.K2_GetActorLocation`) 2500.0 null null) null
      (:`OnSuccess`
        (`KismetSystemLibrary.Delay` 1.0) ; AI stops for 1 sec, can be customised
        (`self.Random Roam`)))))

(event `Display Debug Health`
  ;[1 1 1] Debug Health Temp - Displays health above enemies head for debugging purposes
  (`KismetSystemLibrary.K2_SetTimerDelegate` (delegate `DebugHealth`) 0.01 true) ; Better than Delay
)

(event `DebugHealth`
  (bind _returnvalue (`KismetMathLibrary.MakeVector` (.x (`SceneComponent.K2_GetComponentLocation` (`self.Mesh`))) (- (.y (`SceneComponent.K2_GetComponentLocation` (`self.Mesh`))) 35.0) (+ (.z (`SceneComponent.K2_GetComponentLocation` (`self.Mesh`))) 220.0)))
  ;[1 1 1] Debug Health Temp - Displays health above enemies head for debugging purposes
  (`KismetSystemLibrary.DrawDebugString` _returnvalue (`KismetStringLibrary.Conv_DoubleToString` (`.Health_4_D29B34A6447D561A7C4BF3AD8D470278` (break `/Game/Tech/HealthSystem/S_Health` (`/Game/Tech/HealthSystem/BPC_HealthComponent.S_Health` (`self.BPC_HealthComponent`))))) null (struct :`R` 1.0 :`B` 0.014804 :`A` 1.0))
  (`KismetSystemLibrary.DrawDebugString` (`KismetMathLibrary.MakeVector` (.x _returnvalue) (.y _returnvalue) (+ (.z _returnvalue) 30.0)) (`KismetSystemLibrary.GetDisplayName` self) null (struct :`R` 1.0 :`B` 0.014804 :`A` 1.0)))

(event `self.Box.OnComponentBeginOverlap`
  (params (OverlappedComponent :type "PrimitiveComponent Object Reference") (OtherActor :type "Actor Object Reference") (OtherComp :type "PrimitiveComponent Object Reference") (OtherBodyIndex :type Integer) (bFromSweep :type Boolean) (SweepResult :type "HitResult Structure (by ref)"))
  (bind _asbp_player (cast `/Game/Tech/Character/BP_Player` OtherActor))
  (`/Game/Tech/HealthSystem/BPI_DamageHandling.I_ApplyDamage` _asbp_player (`self.DamageToPlayer`) null))

(fn `Death`
  (params (`isBossDEAD?` :type Boolean)))

(fn `I Get BP Base Enemy`
  (returns (Enemy :type "Character Object Reference"))
  (return self))

(fn `I_ApplyDamage`
  (params (Damage :type "Float (double-precision)") (Instigator :type "Actor Object Reference"))
  (returns (`Target Hit?` :type Boolean) (`Target Dead?` :type Boolean))
  (bind _bpc_healthcomponent (`self.BPC_HealthComponent`))
  ;[0 1 1] Sending damage to health component and updating event dispatcher for UI
  (bind (_target_hit_ _target_dead_) (`/Game/Tech/HealthSystem/BPC_HealthComponent.I_ApplyDamage` _bpc_healthcomponent Damage Instigator))
  (`self.E_HealthUpdated` (`/Game/Tech/HealthSystem/BPC_HealthComponent.S_Health` _bpc_healthcomponent))
  (if _target_dead_
    (`PrimitiveComponent.SetSimulatePhysics` (`self.Mesh`) true) ; Enable Ragdoll
    (`PrimitiveComponent.SetCollisionEnabled` (`self.Box`) "NoCollision")
    (bind _asbp_top_down_game_mode (cast `/Game/Tech/Blueprints/BP_TopDownGameMode` (`GameplayStatics.GetGameMode`)))
    (`/Game/Tech/Blueprints/BP_TopDownGameMode.End-Game` _asbp_top_down_game_mode)
    (return _target_hit_ _target_dead_)
    (else
      (return _target_hit_ _target_dead_))))

(fn `I_ApplyHealing`
  (params (Healing :type "Float (double-precision)") (Instigator :type "Actor Object Reference"))
  (returns (`Target Full?` :type Boolean))
  (bind _bpc_healthcomponent (`self.BPC_HealthComponent`))
  ;[0 1 1] Sending healing to health component and updating event dispatcher for UI
  (bind _target_full_ (`/Game/Tech/HealthSystem/BPC_HealthComponent.I_ApplyHealing` _bpc_healthcomponent Healing Instigator))
  (`self.E_HealthUpdated` (`/Game/Tech/HealthSystem/BPC_HealthComponent.S_Health` _bpc_healthcomponent))
  (return _target_full_))

(fn `I_ChangeMaxHealth`
  (params (`Max Health` :type "Float (double-precision)") (Instigator :type "Actor Object Reference"))
  (returns (`Return Value` :type Boolean))
  (return false))

(fn `I_GetHealthStruct`
  (returns (`Health Struct` :type "/Game/Tech/HealthSystem/S_Health Structure"))
  (return))

(fn `UserConstructionScript`)