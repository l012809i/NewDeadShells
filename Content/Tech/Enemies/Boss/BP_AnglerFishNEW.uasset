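; Angler fish boss that chases the player after activation, summons grunts periodically, and ends the game when killed.
; Looping timers drive movement and attack choice: at range it randomly uses a pulling current or a slowly tracking water plume, up close a chomp.
; The chomp is a timeline lunge, also triggered when the current drags the player into bite range.
; Damage routes through a health component, with a timer-polled health bar widget.
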(event `self.ReceiveBeginPlay`
  (bind (_health _maxhealth) (break `/Game/Tech/HealthSystem/S_Health` (`/Game/Tech/HealthSystem/BPC_HealthComponent.S_Health` (`self.BPC_HealthComponent`))))
  (bind _returnvalue (`GameplayStatics.GetActorOfClass` "/Game/Tech/Character/BP_Player.BP_Player_C"))
  (set `self.Player` _returnvalue)
  (bind _returnvalue_2 (`GameplayStatics.GetActorOfClass` "/Game/Tech/Enemies/Boss/BossfightBps/BP_Bossfightspawners.BP_Bossfightspawners_C"))
  (bind _output_get (set `self.gruntSpawner` _returnvalue_2))
  (`/Game/Tech/Enemies/Boss/BossfightBps/BP_Bossfightspawners.Spawn Grunts` _output_get)
  ;[1 1 1] HealthBar Live Update Very messy code
  (add `self.E_HealthUpdated` (delegate `Update HealthBar`))
  (bind _aswb_aihealth_bar (cast `/Game/Tech/UI/UI_Enemies/WB_AIHealthBar` (`WidgetComponent.GetUserWidgetObject` (`self.HealthBar`)) :!label _label))
  (bind _output_get_2 (set `/Game/Tech/UI/UI_Enemies/WB_AIHealthBar.Health` _health _aswb_aihealth_bar))
  (`ProgressBar.SetPercent` (`/Game/Tech/UI/UI_Enemies/WB_AIHealthBar.HealthBarProgress` _aswb_aihealth_bar) (/ _health _maxhealth))
  (`TextBlock.SetText` (`/Game/Tech/UI/UI_Enemies/WB_AIHealthBar.HealthText` _aswb_aihealth_bar) (`KismetTextLibrary.Conv_DoubleToText` _output_get_2 "HalfToEven")))

(event `Update HealthBar` :!signature `self.E_HealthUpdated`
  (params (Health :type "/Game/Tech/HealthSystem/S_Health Structure"))
  ;[1 1 1] HealthBar Live Update Very messy code
  (`KismetSystemLibrary.K2_SetTimerDelegate` (delegate `Update`) 0.01 true))

(event `Update`
  ;[1 1 1] HealthBar Live Update Very messy code
  (goto _label))

(event `CurrentAttack`
  (bind _player (`self.Player`))
  (bind _returnvalue (`SceneComponent.K2_GetComponentLocation` (`self.CurentTraceSpawner`)))
  (bind _returnvalue_2 (`KismetMathLibrary.GetDirectionUnitVector` (`self.K2_GetActorLocation` _player) (`self.K2_GetActorLocation`)))
  (bind _returnvalue_3 (- _returnvalue (`self.CurrentAttackAimingPoint`)))
  (bind (_returnvalue_x _returnvalue_y) (`KismetMathLibrary.BreakVector` (+ _returnvalue_2 (* _returnvalue_2 3.0))))
  ;[1 1 1] Current Attack
  (set `self.PlayerFound` false)
  (bind _outhits (`KismetSystemLibrary.SphereTraceMultiForObjects` _returnvalue (* (`KismetMathLibrary.Normal` (+ _returnvalue (`KismetMathLibrary.GreaterGreater_VectorRotator` _returnvalue_3 (struct :`Yaw` 30.0)))) 1000.0) 1000.0 (`|MakeArray` "ObjectTypeQuery3" :!type "EObjectTypeQuery Enum")))
  (for _array_element _outhits
    (cast `/Game/Tech/Character/BP_Player` (`.HitActor` (`GameplayStatics.BreakHitResult` _array_element)))
    (set `self.PlayerFound` true))
  (if (not (`self.PlayerFound`))
    (bind _outhits_2 (`KismetSystemLibrary.SphereTraceMultiForObjects` _returnvalue (* (`KismetMathLibrary.Normal` (+ _returnvalue (`KismetMathLibrary.GreaterGreater_VectorRotator` _returnvalue_3 (struct :`Yaw` -30.0)))) 1000.0) 1000.0 (`|MakeArray` "ObjectTypeQuery3" :!type "EObjectTypeQuery Enum")))
    (for _array_element_2 _outhits_2
      (cast `/Game/Tech/Character/BP_Player` (`.HitActor` (`GameplayStatics.BreakHitResult` _array_element_2)))
      (set `self.PlayerFound` true))
    (if (not (`self.PlayerFound`))
      (`PawnMovementComponent.AddInputVector` (`Character.CharacterMovement` _player) (`KismetMathLibrary.MakeVector` _returnvalue_x _returnvalue_y) false))))

(event `self.ActivationRange.OnComponentBeginOverlap`
  (params (OverlappedComponent :type "PrimitiveComponent Object Reference") (OtherActor :type "Actor Object Reference") (OtherComp :type "PrimitiveComponent Object Reference") (OtherBodyIndex :type Integer) (bFromSweep :type Boolean) (SweepResult :type "HitResult Structure (by ref)"))
  (bind _asbp_player (cast `/Game/Tech/Character/BP_Player` OtherActor))
  (set `self.Player` _asbp_player)
  (bind _returnvalue (`GameplayStatics.GetActorOfClass` "/Game/Tech/Enemies/Boss/BossfightBps/BP_Bossfightspawners.BP_Bossfightspawners_C"))
  (set `self.Spawner` _returnvalue)
  (`KismetSystemLibrary.K2_SetTimerDelegate` (delegate `CustomEvent`) 30.0 true)
  (bind _returnvalue_2 (`KismetSystemLibrary.K2_SetTimerDelegate` (delegate `Move Towards`) 0.01 true :!label _label_2))
  (set `self.StopMoveTowards` _returnvalue_2)
  (`KismetSystemLibrary.Delay` (`self.Attack Delay+ on Start`))
  (bind _returnvalue_3 (`KismetSystemLibrary.K2_SetTimerDelegate` (delegate `Can Attack`) 3.0 true))
  (set `self.Can Attack Handler` _returnvalue_3))

(event `CustomEvent`
  (`KismetSystemLibrary.PrintString` "open")
  (`/Game/Tech/Enemies/Boss/BossfightBps/BP_Bossfightspawners.Spawn Grunts` (`self.Spawner`))
  (`KismetSystemLibrary.Delay` 0.2)
  (`KismetSystemLibrary.PrintString` "close"))

(event `Can Attack`
  (bind (_returnvalue_x _returnvalue_y _returnvalue_z) (`KismetMathLibrary.BreakVector` (`self.K2_GetActorLocation`)))
  (if (>= (`KismetMathLibrary.VSize` (- (`self.K2_GetActorLocation`) (`self.K2_GetActorLocation` (`self.Player`)))) 570.0)
    (`KismetSystemLibrary.K2_ClearAndInvalidateTimerHandle` (`self.StopMoveTowards`))
    (`KismetSystemLibrary.K2_ClearAndInvalidateTimerHandle` (`self.Can Attack Handler`))
    (if (`KismetMathLibrary.RandomBool`)
      ;[1 1 1] Current Attack
      (set `self.CurrentAttackAimingPoint` (`self.K2_GetActorLocation` (`self.Player`)))
      (bind _returnvalue (`KismetSystemLibrary.K2_SetTimerDelegate` (delegate `CurrentAttack`) 0.01 true))
      (set `self.CurrentAttackHandle` _returnvalue)
      (set `self.IsInCurrentAttack` true)
      (`KismetSystemLibrary.Delay` 6.0)
      (set `self.IsInCurrentAttack` false)
      (`KismetSystemLibrary.K2_ClearAndInvalidateTimerHandle` (`self.CurrentAttackHandle`))
      (set `self.Attack Delay+ on Start` 0.0)
      (`KismetSystemLibrary.PrintString` "close")
      (goto _label_2)
      (else
        ;[1 1 1] Water Plume Attack
        (`SceneComponent.SetVisibility` (`self.WaterPlumeMesh`) true false)
        (set `self.PlumeAim` (`KismetMathLibrary.MakeVector` (.x (`self.K2_GetActorLocation` (`self.Player`))) (.y (`self.K2_GetActorLocation` (`self.Player`))) _returnvalue_z))
        (bind _returnvalue_2 (`KismetSystemLibrary.K2_SetTimerDelegate` (delegate `Water Plume Attack`) 0.03 true))
        (set `self.PlumeAttackHandler` _returnvalue_2)
        (`KismetSystemLibrary.Delay` 4.0)
        (set `self.Attack Delay+ on Start` 0.0)
        (`KismetSystemLibrary.K2_ClearAndInvalidateTimerHandle` (`self.PlumeAttackHandler`))
        (`SceneComponent.SetVisibility` (`self.WaterPlumeMesh`) false false)
        (`KismetSystemLibrary.PrintString` "close")
        (goto _label_2)))
    (else
      ;[1 1 1] Chomp Attack
      (`KismetSystemLibrary.K2_SetTimerDelegate` (delegate `ChompAttack`) 0.1))))

(event `Move Towards`
  (bind (_returnvalue_x _returnvalue_y _returnvalue_z) (`KismetMathLibrary.BreakVector` (`self.K2_GetActorLocation`)))
  (bind _returnvalue (`self.K2_GetActorLocation`))
  (bind (_returnvalue_x_2 _returnvalue_y_2) (`KismetMathLibrary.BreakVector` (`self.K2_GetActorLocation` (`self.Player`))))
  (`|AIMoveTo` self (- _returnvalue (* (`KismetMathLibrary.Normal` (- _returnvalue (`self.K2_GetActorLocation` (`self.Player`)))) 10.0)) null 1.0
    (:`then`
      (`self.K2_SetActorRotation` (`KismetMathLibrary.FindLookAtRotation` (`KismetMathLibrary.MakeVector` _returnvalue_x _returnvalue_y _returnvalue_z) (`KismetMathLibrary.MakeVector` _returnvalue_x_2 _returnvalue_y_2 _returnvalue_z))))))

(event `Water Plume Attack`
  (bind (_returnvalue_x _returnvalue_y) (`KismetMathLibrary.BreakVector` (`self.K2_GetActorLocation`)))
  (bind (_returnvalue_roll _returnvalue_pitch _returnvalue_yaw) (`KismetMathLibrary.BreakRotator` (`self.K2_GetActorRotation`)))
  (bind (_plumeaim_x _plumeaim_y) (`KismetMathLibrary.BreakVector` (`self.PlumeAim`)))
  (bind (_returnvalue_x_2 _returnvalue_y_2) (`KismetMathLibrary.BreakVector` (`self.K2_GetActorLocation` (`self.Player`))))
  (bind _returnvalue (`SceneComponent.K2_GetComponentLocation` (`self.PlumeEnd`)))
  ;[1 1 1] Water Plume Attack
  (if (>= (- (* (- _returnvalue_x_2 _returnvalue_x) (- _plumeaim_y _returnvalue_y)) (* (- _returnvalue_y_2 _returnvalue_y) (- _plumeaim_x _returnvalue_x))) 0.0)
    (set `self.FlumeTurnSpeed` -0.7)
    (else
      (set `self.FlumeTurnSpeed` 0.7)))
  (`self.K2_SetActorTransform` (`KismetMathLibrary.MakeTransform` (`self.K2_GetActorLocation`) (`KismetMathLibrary.MakeRotator` _returnvalue_roll _returnvalue_pitch (+ _returnvalue_yaw (`self.FlumeTurnSpeed`)))))
  (set `self.PlumeAim` _returnvalue)
  (bind _outhits (`KismetSystemLibrary.SphereTraceMultiForObjects` (`self.K2_GetActorLocation`) _returnvalue 25.0 (`|MakeArray` "ObjectTypeQuery3" :!type "EObjectTypeQuery Enum")))
  (for _array_element _outhits
    (cast `/Game/Tech/Character/BP_Player` (`.HitActor` (`GameplayStatics.BreakHitResult` _array_element)))
    (`/Game/Tech/HealthSystem/BPI_DamageHandling.I_ApplyDamage` (`self.Player`) (`self.PlumeDPS/33`) null)))

(event `self.BiteRange.OnComponentBeginOverlap`
  (params (OverlappedComponent :type "PrimitiveComponent Object Reference") (OtherActor :type "Actor Object Reference") (OtherComp :type "PrimitiveComponent Object Reference") (OtherBodyIndex :type Integer) (bFromSweep :type Boolean) (SweepResult :type "HitResult Structure (by ref)"))
  (bind _returnvalue (`self.K2_GetActorLocation`))
  (bind _returnvalue_2 (- (`self.K2_GetActorLocation` (`self.Player`)) _returnvalue))
  ;[1 1 1] Chomp Attack
  (cast `/Game/Tech/Character/BP_Player` OtherActor)
  (if (`self.IsInCurrentAttack`)
    (`KismetSystemLibrary.K2_ClearAndInvalidateTimerHandle` (`self.CurrentAttackHandle`))
    (set `self.ChompStartLocation` _returnvalue :!label _label_3)
    (set `self.ChompEndLocation` (`KismetMathLibrary.MakeVector` (.x (+ _returnvalue (* (`KismetMathLibrary.Normal` _returnvalue_2) 300.0))) (.y (+ _returnvalue (* (`KismetMathLibrary.Normal` _returnvalue_2) 300.0))) (.z _returnvalue)))
    (`KismetSystemLibrary.PrintString` "close")
    (bind (_direction _newtrack_0) (`Timeline|ChompDash` :!via `PlayFromStart`)
      (:`Update`
        (`self.K2_SetActorLocation` (`KismetMathLibrary.VLerp` (`self.ChompStartLocation`) (`self.ChompEndLocation`) _newtrack_0) true)
        (if (<= (`KismetMathLibrary.VSize` _returnvalue_2) 300.0)
          (if (not (`self.Chomped`))
            (set `self.Chomped` true)
            (`/Game/Tech/HealthSystem/BPI_DamageHandling.I_ApplyDamage` (`self.Player`) (`self.ChompDamage`) null))))
      (:`Finished`
        (set `self.Chomped` false)))))

(event `ChompAttack`
  ;[1 1 1] Chomp Attack
  (bind _output_get (set `self.OpenMontage` "/Game/Tech/Enemies/Boss/Animations/Angler_Attack_Open_Montage.Angler_Attack_Open_Montage"))
  (`|PlayMontage` (`self.Mesh`) _output_get 0.5
    (:`then`
      (goto _label_3))))

(fn `I Get BP Base Enemy`
  (returns (Enemy :type "Character Object Reference"))
  (return null))

(fn `I_ApplyDamage`
  (params (Damage :type "Float (double-precision)") (Instigator :type "Actor Object Reference"))
  (returns (`Target Hit?` :type Boolean) (`Target Dead?` :type Boolean))
  (bind _bpc_healthcomponent (`self.BPC_HealthComponent`))
  (bind (_target_hit_ _target_dead_) (`/Game/Tech/HealthSystem/BPI_DamageHandling.I_ApplyDamage` _bpc_healthcomponent Damage Instigator))
  (`self.E_HealthUpdated` (`/Game/Tech/HealthSystem/BPC_HealthComponent.S_Health` _bpc_healthcomponent))
  (if _target_dead_
    (`self.K2_DestroyActor`)
    (`/Game/Tech/Blueprints/BP_TopDownGameMode.End-Game` (cast `/Game/Tech/Blueprints/BP_TopDownGameMode` (`GameplayStatics.GetGameMode`) :!pure true))
    (return _target_hit_ _target_dead_)
    (else
      (return _target_hit_ _target_dead_))))

(fn `I_ApplyHealing`
  (params (Healing :type "Float (double-precision)") (Instigator :type "Actor Object Reference"))
  (returns (`Target Full?` :type Boolean))
  (return false))

(fn `I_ChangeMaxHealth`
  (params (`Max Health` :type "Float (double-precision)") (Instigator :type "Actor Object Reference"))
  (returns (`Return Value` :type Boolean))
  (return false))

(fn `I_GetHealthStruct`
  (returns (`Health Struct` :type "/Game/Tech/HealthSystem/S_Health Structure"))
  (bind _health_struct (`/Game/Tech/HealthSystem/BPI_DamageHandling.I_GetHealthStruct` (`self.BPC_HealthComponent`)))
  (return _health_struct))

(fn `LookAtPlayer`)

(fn `UserConstructionScript`)