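; BP_MeleeGrunt_Yellow is a child Blueprint, named as the yellow variant of the melee grunt enemy.
; It adds no logic of its own: the construction script calls the parent, and BeginPlay, overlap and Tick are disabled placeholders.
; Its health-struct and apply-damage interface overrides pass straight through to the parent and return its results.
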(fn `I_ApplyDamage`
  (params (Damage :type "Float (double-precision)") (Instigator :type "Actor Object Reference"))
  (returns (`Target Hit?` :type Boolean) (`Target Dead?` :type Boolean))
  (bind (_target_hit_ _target_dead_) (`parent.I_ApplyDamage` Damage Instigator))
  (return _target_hit_ _target_dead_))

(fn `I_GetHealthStruct`
  (returns (`Health Struct` :type "/Game/Tech/HealthSystem/S_Health Structure"))
  (bind _health_struct (`parent.I_GetHealthStruct`))
  (return _health_struct))

(fn `UserConstructionScript`
  (`parent.UserConstructionScript`))