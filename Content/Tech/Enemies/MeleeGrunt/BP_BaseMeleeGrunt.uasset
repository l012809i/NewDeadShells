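; Base melee grunt enemy that attacks the player with a montage and sphere trace, applying its damage stat on hit.
; Damage runs through BPCHealthComponent, whose update event starts a looping timer that refreshes the health bar widget.
; Movement events handle timed freeze, knockback impulse and temporary slow.
; Death ragdolls the mesh, unpossesses the AI and removes the actor after a delay; SpawnCoin's pickup spawn is disconnected.
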(event `self.ReceiveBeginPlay`
  (bind (_health _maxhealth) (break `/Game/Tech/HealthSystem/S_Health` (`/Game/Tech/HealthSystem/BPC_HealthComponent.S_Health` (`self.BPC_HealthComponent`))))
  ;[1 1 1] HealthBar Live Update Very messy code
  (add `self.E_HealthUpdated` (delegate `Update HealthBar`))
  (bind _aswb_aihealth_bar (cast `/Game/Tech/UI/UI_Enemies/WB_AIHealthBar` (`WidgetComponent.GetUserWidgetObject` (`self.HealthBar`)) :!label _label))
  (bind _output_get (set `/Game/Tech/UI/UI_Enemies/WB_AIHealthBar.Health` _health _aswb_aihealth_bar))
  (`ProgressBar.SetPercent` (`/Game/Tech/UI/UI_Enemies/WB_AIHealthBar.HealthBarProgress` _aswb_aihealth_bar) (/ _health _maxhealth))
  (`TextBlock.SetText` (`/Game/Tech/UI/UI_Enemies/WB_AIHealthBar.HealthText` _aswb_aihealth_bar) (`KismetTextLibrary.Conv_DoubleToText` _output_get "HalfToEven")))

(event `Update HealthBar` :!signature `self.E_HealthUpdated`
  (params (Health :type "/Game/Tech/HealthSystem/S_Health Structure"))
  ;[1 1 1] HealthBar Live Update Very messy code
  (`KismetSystemLibrary.K2_SetTimerDelegate` (delegate `Update`) 0.01 true))

(event `Update`
  ;[1 1 1] HealthBar Live Update Very messy code
  (goto _label))

(event `SetRange`
  (cast `/Game/Tech/Enemies/MeleeGrunt/MeleeGruntAIController` (`AIBlueprintHelperLibrary.GetAIController` null)))

(event `CustomEvent_2`
  (params (`Freeze Length` :type "Float (double-precision)"))
  ;[0.9922 0.6667 1] Cold fusion freeze
  (`CharacterMovementComponent.DisableMovement` (`self.CharacterMovement`))
  (set `self.Frozen` true)
  (`KismetSystemLibrary.K2_SetTimerDelegate` (`|CreateDelegate` :!event `Unfreeze`) `Freeze Length`))

(event `Unfreeze`
  ;[0.9922 0.6667 1] Cold fusion unfreeze
  (`CharacterMovementComponent.SetMovementMode` (`self.CharacterMovement`) "MOVE_NavWalking" 0)
  (set `self.Frozen` false))

(event `CustomEvent_1`
  (params (`Forward vector` :type "Vector Structure") (Amount :type "Float (double-precision)"))
  ;[0.9922 0.6667 1] Knockback
  (`CharacterMovementComponent.AddImpulse` (`self.CharacterMovement`) (* `Forward vector` Amount) true))

(event `CustomEvent`
  (bind _charactermovement (`self.CharacterMovement`))
  ;[0.9922 0.6667 1] Bubble slows
  (set `CharacterMovementComponent.MaxWalkSpeed` 300.0 _charactermovement)
  (`KismetSystemLibrary.Delay` 1.0)
  (set `CharacterMovementComponent.MaxWalkSpeed` 600.0 _charactermovement))

(event `Attack`
  (bind _mesh (`self.Mesh`))
  (bind _returnvalue (`KismetMathLibrary.MakeVector` (.x (`SceneComponent.K2_GetComponentLocation` _mesh)) (.y (`SceneComponent.K2_GetComponentLocation` _mesh)) (+ (.z (`SceneComponent.K2_GetComponentLocation` _mesh)) 89.0)))
  (`|PlayMontage` (`self.Mesh`) "/Game/Tech/Enemies/MeleeGrunt/Animation/Melee_Grunt_Attack_Montage.Melee_Grunt_Attack_Montage" 0.3
    (:`then`
      ;[1 1 1] Draw Line Trace
      (bind (_outhit _returnvalue_2) (`KismetSystemLibrary.SphereTraceSingle` _returnvalue (+ _returnvalue (* (`SceneComponent.GetRightVector` _mesh) 100.0)) 30.0 "TraceTypeQuery1" false (`self.IgnoreEnemies`) "ForDuration"))
      (if _returnvalue_2
        (bind (_bblockinghit _binitialoverlap _time _distance _location _impactpoint _normal _impactnormal _physmat _hitactor) (`GameplayStatics.BreakHitResult` _outhit))
        (`KismetSystemLibrary.PrintString` (`KismetSystemLibrary.GetDisplayName` _hitactor))
        ;[1 1 1] Apply Damage to the player
        (if (== (`GameplayStatics.GetObjectClass` _hitactor) "/Game/Tech/Character/BP_Player.BP_Player_C")
          (bind _asbp_player (cast `/Game/Tech/Character/BP_Player` _hitactor))
          (message `/Game/Tech/HealthSystem/BPI_DamageHandling.I_ApplyDamage` _asbp_player (`.Damage_49_A01B425145A12C889FD0F9848EDABD6D` (break `/Game/Tech/Enemies/MeleeGrunt/S_MeleeGrunt` (`self.Stats`))) null))))))

(fn `Death`
  (`PrimitiveComponent.SetSimulatePhysics` (`self.Mesh`) true)
  (`PrimitiveComponent.SetCollisionEnabled` (`self.CapsuleComponent`) "NoCollision")
  (bind _asmelee_grunt_aicontroller (cast `/Game/Tech/Enemies/MeleeGrunt/MeleeGruntAIController` (`AIBlueprintHelperLibrary.GetAIController` null)))
  (`Controller.UnPossess` _asmelee_grunt_aicontroller)
  (`self.SpawnCoin`))

(fn `Get freeze`
  (returns (Frozen :type Boolean))
  (return false))

(fn `I_ApplyDamage`
  (params (Damage :type "Float (double-precision)") (Instigator :type "Actor Object Reference"))
  (returns (`Target Hit?` :type Boolean) (`Target Dead?` :type Boolean))
  (bind (_target_hit_ _target_dead_) (`/Game/Tech/HealthSystem/BPI_DamageHandling.I_ApplyDamage` (`self.BPC_HealthComponent`) Damage Instigator))
  (`self.E_HealthUpdated` (`/Game/Tech/HealthSystem/BPC_HealthComponent.S_Health` (`self.BPC_HealthComponent`)))
  (if _target_dead_
    (`self.Death`)
    (bind _returnvalue (`KismetSystemLibrary.K2_SetTimer` null "Remove" 3.0))
    (set `self.TimeUntilDead` _returnvalue)
    (return _target_hit_ _target_dead_)
    (else
      (return _target_hit_ _target_dead_))))

(fn `I_ApplyHealing`
  (params (Healing :type "Float (double-precision)") (Instigator :type "Actor Object Reference"))
  (returns (`Target Full?` :type Boolean))
  (return false))

(fn `I_ChangeMaxHealth`
  (params (`Max Health` :type "Float (double-precision)") (Instigator :type "Actor Object Reference"))
  (returns (`Return Value` :type Boolean))
  (return false))

(fn `I_GetHealthStruct`
  (returns (`Health Struct` :type "/Game/Tech/HealthSystem/S_Health Structure"))
  (bind _health_struct (`/Game/Tech/HealthSystem/BPI_DamageHandling.I_GetHealthStruct` (`self.BPC_HealthComponent`)))
  (return _health_struct))

(fn `Remove`
  (`self.K2_DestroyActor`))

(fn `SpawnCoin`)

(fn `UserConstructionScript`)