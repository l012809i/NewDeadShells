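; Fight director that takes turns sending the level's melee grunts in to attack, one at a time on a looping timer.
; On BeginPlay it gathers all BP_BaseMeleeGrunt actors once and gives each a random grade in a map.
; Each timer tick picks the highest-graded grunt, calls AIAttack on its MeleeGruntAIController, then re-rolls that grunt's grade to vary who attacks next.
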(event `self.ReceiveBeginPlay`
  (`GameplayStatics.GetAllActorsOfClass` "/Game/Tech/Enemies/MeleeGrunt/BP_BaseMeleeGrunt.BP_BaseMeleeGrunt_C")
  (bind _output_get (set `self.EnemyList` (`self.EnemyList`)))
  (for _array_element _output_get
    (`BlueprintMapLibrary.Map_Add` (`self.EnemyGrading`) _array_element (`KismetMathLibrary.RandomFloatInRange` 1.0 5.0)))
  (`KismetSystemLibrary.K2_SetTimerDelegate` (delegate `TriggerAttack`) 2.0 true))

(event `TriggerAttack`
  (bind (_l_highestvalue1 _l_highestgradeai1) (`self.FindHighestGrade`))
  (bind _asmelee_grunt_aicontroller (cast `/Game/Tech/Enemies/MeleeGrunt/MeleeGruntAIController` (`AIBlueprintHelperLibrary.GetAIController` _l_highestgradeai1)))
  (`/Game/Tech/Enemies/MeleeGrunt/MeleeGruntAIController.AIAttack` _asmelee_grunt_aicontroller)
  (`BlueprintMapLibrary.Map_Add` (`self.EnemyGrading`) _l_highestgradeai1 (`KismetMathLibrary.RandomFloatInRange` 1.0 5.0)))

(fn `FindHighestGrade`
  (returns (L_HighestValue1 :type "Float (double-precision)") (L_HighestGradeAI1 :type "/Game/Tech/Enemies/MeleeGrunt/BP_BaseMeleeGrunt Object Reference"))
  (locals (L_HighestValue :type "Float (double-precision)") (L_HighestGradeAI :type "/Game/Tech/Enemies/MeleeGrunt/BP_BaseMeleeGrunt Object Reference"))
  (bind _keys (`BlueprintMapLibrary.Map_Keys` (`self.EnemyGrading`)))
  (for _array_element _keys
    (bind _value (`BlueprintMapLibrary.Map_Find` (`self.EnemyGrading`) _array_element))
    (if (> _value (`local.L_HighestValue`))
      (set `local.L_HighestValue` _value)
      (set `local.L_HighestGradeAI` _array_element)))
  (return (`local.L_HighestValue`) (`local.L_HighestGradeAI`)))

(fn `UserConstructionScript`)