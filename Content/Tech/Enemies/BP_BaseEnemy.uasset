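; Base enemy character that roams to random navigable points and damages the player when its box overlaps them.
; Damage and healing interface calls forward to a health component and fire a health-updated dispatcher for UI, while lethal damage triggers ragdoll and delayed destruction.
; Events provide timed freeze, impulse knockback and a brief slow for player abilities.
; A looping timer draws debug health text above its head.
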(event `self.ReceiveBeginPlay`
  (`self.Display Debug Health`)
  (`self.Random Roam`))

(event `Random Roam`
  ;[1 1 1] AI Roaming - Roaming to itself (creating random location)
  (if (`self.isRoaming`)
    (`|AIMoveTo` self (`NavigationSystemV1.K2_GetRandomReachablePointInRadius` (`self.K2_GetActorLocation`) 2500.0 null null) null
      (:`OnSuccess`
        (`KismetSystemLibrary.Delay` 1.0) ; AI stops for 1 sec, can be customised
        (`self.Random Roam`)))))

(event `Display Debug Health`
  ;[1 1 1] Debug Health Temp - Displays health above enemies head for debugging purposes
  (`KismetSystemLibrary.K2_SetTimerDelegate` (delegate `DebugHealth`) 0.01 true) ; Better than Delay
)

(event `DebugHealth`
  ;[1 1 1] Debug Health Temp - Displays health above enemies head for debugging purposes
  (`KismetSystemLibrary.DrawDebugString` (`KismetMathLibrary.MakeVector` (.x (`SceneComponent.K2_GetComponentLocation` (`self.Mesh`))) (- (.y (`SceneComponent.K2_GetComponentLocation` (`self.Mesh`))) 35.0) (+ (.z (`SceneComponent.K2_GetComponentLocation` (`self.Mesh`))) 220.0)) (`KismetStringLibrary.Conv_DoubleToString` (`.Health_4_D29B34A6447D561A7C4BF3AD8D470278` (break `/Game/Tech/HealthSystem/S_Health` (`/Game/Tech/HealthSystem/BPC_HealthComponent.S_Health` (`self.BPC_HealthComponent`))))) null (struct :`R` 1.0 :`B` 0.014804 :`A` 1.0)))

(event `self.Box.OnComponentBeginOverlap`
  (params (OverlappedComponent :type "PrimitiveComponent Object Reference") (OtherActor :type "Actor Object Reference") (OtherComp :type "PrimitiveComponent Object Reference") (OtherBodyIndex :type Integer) (bFromSweep :type Boolean) (SweepResult :type "HitResult Structure (by ref)"))
  (bind _asbp_player (cast `/Game/Tech/Character/BP_Player` OtherActor))
  (`self.I_ApplyDamage` _asbp_player (`self.DamageToPlayer`) null))

(event `/Game/Tech/Projectiles/NewProjectiles/BPI_ProjectileInterface.Freeze enemies`
  (params (`Freeze Length` :type "Float (double-precision)"))
  ;[0.9922 0.6667 1] Cold fusion freeze
  (`CharacterMovementComponent.DisableMovement` (`self.CharacterMovement`))
  (set `self.Frozen` true)
  (`KismetSystemLibrary.K2_SetTimerDelegate` (`|CreateDelegate` :!event `Unfreeze`) `Freeze Length`))

(event `Unfreeze`
  ;[0.9922 0.6667 1] Cold fusion unfreeze
  (`CharacterMovementComponent.SetMovementMode` (`self.CharacterMovement`) "MOVE_NavWalking" 0)
  (set `self.Frozen` false))

(event `/Game/Tech/Projectiles/NewProjectiles/BPI_ProjectileInterface.ApplyKnockback`
  (params (`Forward vector` :type "Vector Structure") (Amount :type "Float (double-precision)"))
  ;[0.9922 0.6667 1] Knockback
  (`CharacterMovementComponent.AddImpulse` (`self.CharacterMovement`) (* `Forward vector` Amount) true))

(event `/Game/Tech/Projectiles/NewProjectiles/BPI_ProjectileInterface.Slow`
  (bind _charactermovement (`self.CharacterMovement`))
  ;[0.9922 0.6667 1] Bubble slows
  (set `CharacterMovementComponent.MaxWalkSpeed` 300.0 _charactermovement)
  (`KismetSystemLibrary.Delay` 1.0)
  (set `CharacterMovementComponent.MaxWalkSpeed` 600.0 _charactermovement))

(fn `Death`
  (`self.K2_DestroyActor`))

(fn `Get freeze`
  (returns (Frozen :type Boolean))
  (bind _frozen (`self.Frozen`))
  (`KismetSystemLibrary.PrintString` (`KismetStringLibrary.Conv_BoolToString` _frozen))
  (return _frozen))

(fn `I Get BP Base Enemy`
  (returns (Enemy :type "Character Object Reference"))
  (return self))

(fn `I_ApplyDamage`
  (params (Damage :type "Float (double-precision)") (Instigator :type "Actor Object Reference"))
  (returns (`Target Hit?` :type Boolean) (`Target Dead?` :type Boolean))
  (bind _bpc_healthcomponent (`self.BPC_HealthComponent`))
  ;[0 1 1] Sending damage to health component and updating event dispatcher for UI
  (bind (_target_hit_ _target_dead_) (`/Game/Tech/HealthSystem/BPC_HealthComponent.I_ApplyDamage` _bpc_healthcomponent Damage Instigator))
  (`self.E_HealthUpdated` (`/Game/Tech/HealthSystem/BPC_HealthComponent.S_Health` _bpc_healthcomponent))
  (if _target_dead_
    (`PrimitiveComponent.SetSimulatePhysics` (`self.Mesh`) true) ; Enable Ragdoll
    (`PrimitiveComponent.SetCollisionEnabled` (`self.Box`) "NoCollision")
    (bind _returnvalue (`KismetSystemLibrary.K2_SetTimer` null "Death" 5.0)) ; 5 Second delay before Destroying Character
    (set `self.TimerHandler` _returnvalue)
    (return _target_hit_ _target_dead_)
    (else
      (return _target_hit_ _target_dead_))))

(fn `I_ApplyHealing`
  (params (Healing :type "Float (double-precision)") (Instigator :type "Actor Object Reference"))
  (returns (`Target Full?` :type Boolean))
  (bind _bpc_healthcomponent (`self.BPC_HealthComponent`))
  ;[0 1 1] Sending healing to health component and updating event dispatcher for UI
  (bind _target_full_ (`/Game/Tech/HealthSystem/BPC_HealthComponent.I_ApplyHealing` _bpc_healthcomponent Healing Instigator))
  (`self.E_HealthUpdated` (`/Game/Tech/HealthSystem/BPC_HealthComponent.S_Health` _bpc_healthcomponent))
  (return _target_full_))

(fn `I_ChangeMaxHealth`
  (params (`Max Health` :type "Float (double-precision)") (Instigator :type "Actor Object Reference"))
  (returns (`Return Value` :type Boolean))
  (return false))

(fn `I_GetHealthStruct`
  (returns (`Health Struct` :type "/Game/Tech/HealthSystem/S_Health Structure"))
  (return))

(fn `UserConstructionScript`)