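; BP_CheckBoss is a watcher that ends the game when no boss is present in the level.
; On BeginPlay it starts a looping one-second timer that searches for actors tagged EnemyBoss.
; When the first result is not valid, it casts the game mode to BP_TopDownGameMode and calls EndGame.
; The timer is never cleared, so the check keeps repeating after that call.
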(event `self.ReceiveBeginPlay`
  (`self.StartCheckBoss`))

(event `StartCheckBoss`
  (`KismetSystemLibrary.K2_SetTimerDelegate` (delegate `CheckingBoss`) 1.0 true))

(event `CheckingBoss`
  (bind _outactors (`GameplayStatics.GetAllActorsWithTag` "EnemyBoss"))
  (if (not (!= (`KismetSystemLibrary.IsValid` (`|GetArrayItem` _outactors)) false))
    (bind _asbp_top_down_game_mode (cast `/Game/Tech/Blueprints/BP_TopDownGameMode` (`GameplayStatics.GetGameMode`)))
    (`/Game/Tech/Blueprints/BP_TopDownGameMode.End-Game` _asbp_top_down_game_mode)))

(fn `UserConstructionScript`)