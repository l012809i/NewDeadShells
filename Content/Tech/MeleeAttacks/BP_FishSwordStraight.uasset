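; Straight melee attack actor for a fish sword that deals damage in a line when spawned.
; On BeginPlay it sweeps a sphere trace for Pawns forward from its owner, ignoring the owner and drawing debug shapes.
; Each hit receives damage through an interface message; confirmed hits notify the actor's BPC_BaseUpgrade components.
; A hit that does not confirm destroys the attack actor.
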(event `self.ReceiveBeginPlay`
  (bind _returnvalue (`self.GetOwner`))
  (bind _returnvalue_2 (`self.K2_GetActorLocation` _returnvalue))
  (`parent.ReceiveBeginPlay`)
  (`KismetArrayLibrary.Array_AddUnique` (`self.Actors to Ignore`) _returnvalue)
  (bind _outhits (`KismetSystemLibrary.SphereTraceMultiForObjects` _returnvalue_2 (+ _returnvalue_2 (* (`self.GetActorForwardVector` _returnvalue) 250.0)) 50.0 (`|MakeArray` "ObjectTypeQuery3" :!type "EObjectTypeQuery Enum") false (`self.Actors to Ignore`) "ForDuration"))
  (for _array_element _outhits
    (bind (_bblockinghit _binitialoverlap _time _distance _location _impactpoint _normal _impactnormal _physmat _hitactor) (`GameplayStatics.BreakHitResult` _array_element))
    (bind _target_hit_ (message `/Game/Tech/HealthSystem/BPI_DamageHandling.I_ApplyDamage` _hitactor (`self.Damage`) (`self.GetOwner`)))
    (`KismetArrayLibrary.Array_AddUnique` (`self.Actors to Ignore`) _hitactor)
    (if _target_hit_
      (for _array_element_2 (`self.K2_GetComponentsByClass` "/Game/Tech/Upgrades/BPC_BaseUpgrade.BPC_BaseUpgrade_C")
        (`/Game/Tech/Upgrades/BPC_BaseUpgrade.Upgrade_HitEnemy` _array_element_2 (`self.Damage`)))
      (else
        (`self.K2_DestroyActor`)))))

(fn `UserConstructionScript`
  (`parent.UserConstructionScript`))