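; Long-range katana melee attack actor that damages pawns in front of it as soon as it spawns.
; BeginPlay runs a forward multi-sphere object trace, ignoring its owner and briefly drawing debug, then sends each hit actor an interface damage message with the owner as instigator.
; Confirmed hits notify the attack's BPC_BaseUpgrade components with damage and location.
; An unconfirmed hit destroys the attack actor.
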(event `self.ReceiveBeginPlay`
  (bind _returnvalue (`self.K2_GetActorLocation`))
  (`parent.ReceiveBeginPlay`)
  (bind _outhits (`KismetSystemLibrary.SphereTraceMultiForObjects` _returnvalue (+ _returnvalue (* (`SceneComponent.GetForwardVector` (`self.DefaultSceneRoot`)) 500.0)) 125.0 (`|MakeArray` "ObjectTypeQuery3" :!type "EObjectTypeQuery Enum") false (`|MakeArray` (`self.GetOwner`)) "ForDuration" true (struct :`R` 1.0 :`A` 1.0) (struct :`G` 1.0 :`A` 1.0) 0.5))
  (for _array_element _outhits
    (bind (_bblockinghit _binitialoverlap _time _distance _location _impactpoint _normal _impactnormal _physmat _hitactor) (`GameplayStatics.BreakHitResult` _array_element))
    (bind _target_hit_ (message `/Game/Tech/HealthSystem/BPI_DamageHandling.I_ApplyDamage` _hitactor (`self.Damage`) (`self.GetOwner`)))
    (if _target_hit_
      (for _array_element_2 (`self.K2_GetComponentsByClass` "/Game/Tech/Upgrades/BPC_BaseUpgrade.BPC_BaseUpgrade_C")
        (`/Game/Tech/Upgrades/BPC_BaseUpgrade.Upgrade_HitEnemy` _array_element_2 (`self.Damage`) _location))
      (else
        (`self.K2_DestroyActor`)))))

(fn `UserConstructionScript`
  (`parent.UserConstructionScript`))