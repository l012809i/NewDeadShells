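; Short-lived melee sword sweep actor that damages pawns in an arc in front of its owner.
; On BeginPlay a fast timeline fans multi line traces from the actor to points along a forward-offset spline, end to start.
; Each pawn hit receives damage through an interface and is then ignored; successful hits notify the actor's upgrade components.
; The actor destroys itself when damage fails to land or the sweep finishes.
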(event `self.ReceiveBeginPlay`
  (bind _spline (`self.Spline`))
  (`parent.ReceiveBeginPlay`)
  (`KismetArrayLibrary.Array_AddUnique` (`self.Actors to Ignore`) (`self.GetOwner`))
  (`TimelineComponent.SetPlayRate` (`self.AttackTimeline`) (/ 1.0 0.3))
  (bind (_direction _alpha) (`Timeline|AttackTimeline` :!via `PlayFromStart`)
    (:`Update`
      (bind _outhits (`KismetSystemLibrary.LineTraceMultiForObjects` (`self.K2_GetActorLocation`) (`SplineComponent.GetLocationAtDistanceAlongSpline` _spline (`KismetMathLibrary.Lerp` (`SplineComponent.GetSplineLength` _spline) 0.0 _alpha) "World") (`|MakeArray` "ObjectTypeQuery3" :!type "EObjectTypeQuery Enum") false (`self.Actors to Ignore`) "ForDuration"))
      (for _array_element _outhits
        (bind (_bblockinghit _binitialoverlap _time _distance _location _impactpoint _normal _impactnormal _physmat _hitactor) (`GameplayStatics.BreakHitResult` _array_element))
        (bind _target_hit_ (message `/Game/Tech/HealthSystem/BPI_DamageHandling.I_ApplyDamage` _hitactor (`self.Damage`) (`self.GetOwner`)))
        (`KismetArrayLibrary.Array_AddUnique` (`self.Actors to Ignore`) _hitactor)
        (if _target_hit_
          (for _array_element_2 (`self.K2_GetComponentsByClass` "/Game/Tech/Upgrades/BPC_BaseUpgrade.BPC_BaseUpgrade_C")
            (`/Game/Tech/Upgrades/BPC_BaseUpgrade.Upgrade_HitEnemy` _array_element_2 (`self.Damage`)))
          (else
            (`self.K2_DestroyActor`)))))
    (:`Finished`
      (`self.K2_DestroyActor`))))

(fn `UserConstructionScript`
  (`SceneComponent.K2_SetWorldLocation` (`self.Spline`) (+ (`self.K2_GetActorLocation`) (* (`SceneComponent.GetForwardVector` (`self.DefaultSceneRoot`)) (`self.DistanceFromPlayer`))) false true))