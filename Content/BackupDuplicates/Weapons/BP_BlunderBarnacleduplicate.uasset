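; Blunder Barnacle weapon Blueprint (a backup duplicate) that alternates between a six-projectile scatter blast and one full-damage shot.
; Primary and alternate inputs set SingleShot and share parent activation and cooldown-starting deactivation, but a FlipFlop picks the shot type, not that flag.
; Shots route through every BPC_BaseUpgrade component, passing chain-lightning components as shot upgrades; the scatter splits damage evenly and adds inaccuracy.
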(event `self.ActivateWeapon`
  ;[0 1 1] On fire - do shot type
  (set `self.SingleShot?` true)
  (`parent.ActivateWeapon` :!label _label))

(event `self.DeactivateWeapon`
  (params (`Weapon Switch?` :type Boolean))
  ;[0 1 1] Deactivate to start cooldown
  (`parent.DeactivateWeapon` false :!label _label_2))

(event `self.AlternateDeactivate`
  ;[0 1 1] Deactivate to start cooldown
  (goto _label_2))

(event `self.AlternateActivate`
  ;[0 1 1] On fire - do shot type
  (set `self.SingleShot?` false)
  (goto _label))

(event `self.WeaponFunctionality`
  (`/Engine/EditorBlueprintResources/StandardMacros.FlipFlop`
    (:`A`
      (set `self.ProjectileType` null)
      (for _ (range 1 7)
        (for _array_element (`self.K2_GetComponentsByClass` "/Game/Tech/Upgrades/BPC_BaseUpgrade.BPC_BaseUpgrade_C")
          (`/Game/Tech/Upgrades/BPC_BaseUpgrade.Upgrade_ProjectileShoot` _array_element 15.0 (`self.ProjectileType`) (/ (`self.F_GetDamage`) 6.0) (`self.K2_GetComponentsByClass` "/Game/Tech/Upgrades/BPC_ChainLightning.BPC_ChainLightning_C")))))
    (:`B`
      (set `self.ProjectileType` null)
      (for _array_element_2 (`self.K2_GetComponentsByClass` "/Game/Tech/Upgrades/BPC_BaseUpgrade.BPC_BaseUpgrade_C")
        (`/Game/Tech/Upgrades/BPC_BaseUpgrade.Upgrade_ProjectileShoot` _array_element_2 0.0 (`self.ProjectileType`) (`self.F_GetDamage`) (`self.K2_GetComponentsByClass` "/Game/Tech/Upgrades/BPC_ChainLightning.BPC_ChainLightning_C"))))))

(fn `UserConstructionScript`
  (`parent.UserConstructionScript`))