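; Rusty pistol weapon Blueprint, a backup duplicate, that extends a parent weapon and delegates its shot to attached upgrade components.
; WeaponFunctionality calls UpgradeProjectileWeapon on each BPC_BaseUpgrade, passing projectile type, damage and any BPC_ChainLightning components as shot upgrades.
; The gunshot sound plays inside that loop, once per upgrade component.
; Activation, deactivation and construction only call the parent; alternate fire is empty, and the damage and healing nodes are unconnected.
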(event `self.ActivateWeapon`
  ;[0 1 1] Add custom firing mechanics here
  (`parent.ActivateWeapon`))

(event `self.WeaponFunctionality`
  ;[0 1 1] Add Weapon Functionality Here!
  (for _array_element (`self.K2_GetComponentsByClass` "/Game/Tech/Upgrades/BPC_BaseUpgrade.BPC_BaseUpgrade_C")
    (`/Game/Tech/Upgrades/BPC_BaseUpgrade.Upgrade_ProjectileWeapon` _array_element 0.0 (`self.ProjectileType`) (`self.F_GetDamage`) (`self.K2_GetComponentsByClass` "/Game/Tech/Upgrades/BPC_ChainLightning.BPC_ChainLightning_C"))
    (`GameplayStatics.PlaySound2D` "/Game/Tech/Sounds/RustyPistol/Gunshot_Cue.Gunshot_Cue" 1.0 1.0 0.0 null null)))

(event `self.DeactivateWeapon`
  (params (`Weapon Switch?` :type Boolean))
  ;[0 1 1] Add custom firing mechanics here
  (`parent.DeactivateWeapon` `Weapon Switch?`))

(event `self.AlternateActivate`
  ;[0 1 1] Alternate Firing nodes
)

(event `self.AlternateDeactivate`
  ;[0 1 1] Alternate Firing nodes
)

(fn `UserConstructionScript`
  (`parent.UserConstructionScript`))