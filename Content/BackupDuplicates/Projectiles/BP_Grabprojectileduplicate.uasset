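; Grab projectile that repositions nearby pawns relative to itself and destroys itself five seconds after its movement component activates.
; A fast looping timer runs a debug-drawn sphere trace around the ball, ignoring the player and pawns already caught.
; Each hit starts a timeline that sweeps the actor from the ball's position to that position minus the hit distance.
; Damage is stored but never applied, and the collision events are empty.
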(event `Set Damage`
  (params (Damage :type "Float (double-precision)"))
  (set `self.Damage` Damage))

(event `self.Sphere_Col.OnComponentBeginOverlap`
  (params (OverlappedComponent :type "PrimitiveComponent Object Reference") (OtherActor :type "Actor Object Reference") (OtherComp :type "PrimitiveComponent Object Reference") (OtherBodyIndex :type Integer) (bFromSweep :type Boolean) (SweepResult :type "HitResult Structure (by ref)")))

(event `self.Sphere_Col.OnComponentHit`
  (params (HitComponent :type "PrimitiveComponent Object Reference") (OtherActor :type "Actor Object Reference") (OtherComp :type "PrimitiveComponent Object Reference") (NormalImpulse :type "Vector Structure") (Hit :type "HitResult Structure (by ref)")))

(event `self.ProjectileMovement.OnComponentActivated`
  (params (Component :type "ActorComponent Object Reference") (bReset :type Boolean))
  (set `self.Array` (`self.Array`))
  (`KismetSystemLibrary.K2_SetTimerDelegate` (delegate `Trace`) 0.01 true)
  (`KismetSystemLibrary.Delay` 5.0)
  (`self.K2_DestroyActor`))

(event `Trace`
  (bind _array (`self.Array`))
  (bind _returnvalue (`SceneComponent.K2_GetComponentLocation` (`self.Sphere_Col`)))
  (`KismetArrayLibrary.Array_Add` _array (`GameplayStatics.GetPlayerCharacter` 0))
  (bind _outhits (`KismetSystemLibrary.SphereTraceMultiForObjects` _returnvalue _returnvalue 200.0 (`|MakeArray` "ObjectTypeQuery3" :!type "EObjectTypeQuery Enum") false _array "ForDuration"))
  (for _array_element _outhits
    (bind (_bblockinghit _binitialoverlap _time _distance _location _impactpoint _normal _impactnormal _physmat _hitactor) (`GameplayStatics.BreakHitResult` _array_element))
    (`KismetArrayLibrary.Array_Add` (`self.Array`) _hitactor)
    (bind _output_get (set `self.Hit Actor` _hitactor))
    (bind _output_get_2 (set `self.Ballposition` (`SceneComponent.K2_GetComponentLocation` (`self.Sphere_Col`))))
    (bind (_direction __movement) (`Timeline|Timeline_0`)
      (:`Update`
        (`self.K2_SetActorRelativeLocation` _output_get (`KismetMathLibrary.VLerp` _output_get_2 (- _output_get_2 _distance) __movement) true false)))))

(fn `UserConstructionScript`)