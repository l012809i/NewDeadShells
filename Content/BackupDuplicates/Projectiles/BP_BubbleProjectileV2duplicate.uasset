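; Bubble projectile Blueprint that slows what it hits and deals area damage after a short flight.
; On movement activation it picks a random initial speed, then stops after a delay and sphere-traces nearby pawns, ignoring the player, with debug drawing on.
; Damage and slow go through message calls; confirmed damage hits notify its upgrade components before the projectile destroys itself.
; GetFreeze always returns false.
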(event `self.ReceiveBeginPlay`
  (`parent.ReceiveBeginPlay`))

(event `self.Sphere_Col.OnComponentHit`
  (params (HitComponent :type "PrimitiveComponent Object Reference") (OtherActor :type "Actor Object Reference") (OtherComp :type "PrimitiveComponent Object Reference") (NormalImpulse :type "Vector Structure") (Hit :type "HitResult Structure (by ref)"))
  ;[0.9922 0.6667 1] Slows enemy On hit
  (message `/Game/Tech/Projectiles/BPI_ProjectileInterface.Slow` OtherActor))

(event `self.ProjectileMovement.OnComponentActivated`
  (params (Component :type "ActorComponent Object Reference") (bReset :type Boolean))
  (bind _returnvalue (`SceneComponent.K2_GetComponentLocation` (`self.Sphere_Col`)))
  ;[0.9922 0.6667 1] Projectile starts move at a random speed then slows down and damages all enemies nearby
  (set `ProjectileMovementComponent.InitialSpeed` (`KismetMathLibrary.RandomFloatInRange` 200.0 400.0) (`self.ProjectileMovement`))
  (`KismetSystemLibrary.Delay` 1.5)
  (`ProjectileMovementComponent.SetVelocityInLocalSpace` (`self.ProjectileMovement`) (0.0 0.0 0.0))
  (bind _outhits (`KismetSystemLibrary.SphereTraceMultiForObjects` _returnvalue _returnvalue 50.0 (`|MakeArray` "ObjectTypeQuery3" :!type "EObjectTypeQuery Enum") false (`|MakeArray` (`GameplayStatics.GetPlayerCharacter` 0) :!type "Actor Object Reference") "ForDuration"))
  (for _array_element _outhits
    (bind _target_hit_ (message `/Game/Tech/HealthSystem/BPI_DamageHandling.I_ApplyDamage` (`.HitActor` (`GameplayStatics.BreakHitResult` _array_element)) (`self.Damage`) null))
    (if _target_hit_
      (for _array_element_2 (`self.K2_GetComponentsByClass` "/Game/Tech/Upgrades/BPC_BaseUpgrade.BPC_BaseUpgrade_C")
        (`/Game/Tech/Upgrades/BPC_BaseUpgrade.Upgrade_Hit` _array_element_2 (`self.Damage`)))))
  (`self.K2_DestroyActor`))

(fn `Get freeze`
  (returns (Frozen :type Boolean))
  (return false))

(fn `UserConstructionScript`
  (`parent.UserConstructionScript`))