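; Weapon upgrade component for a single attack, spawning one projectile each time its UpgradeProjectileWeapon event fires.
; It caches the mesh of its owning BP_BaseWeapon on BeginPlay and builds the spawn transform from the FireOrigin socket, shifted sideways by LocationOffset with random yaw-only inaccuracy.
; The projectile receives the damage and shot upgrades, with the weapon's owner as its owner.
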(event `self.ReceiveBeginPlay`
  (bind _asbp_base_weapon (cast `/Game/Tech/Weapons/WeaponInfo/BP_BaseWeapon` (`self.GetOwner`) :!pure true))
  (`/Engine/EditorBlueprintResources/StandardMacros.IsValid` _asbp_base_weapon
    (:`Is Valid`
      (set `self.SM Weapon` (`/Game/Tech/Weapons/WeaponInfo/BP_BaseWeapon.SM_Weapon` _asbp_base_weapon)))))

(event `self.Upgrade_ProjectileWeapon`
  (params (`Inaccuracy (half-degrees)` :type "Float (double-precision)") (`Projectile Type` :type "/Game/Tech/Projectiles/BP_BaseProjectile Class Reference") (Damage :type "Float (double-precision)") (`Shot Upgrades` :type "Array of /Game/Tech/Upgrades/BPC_ChainLightning Object Reference (by ref)"))
  (`|SpawnActorFromClass` `Projectile Type` (`self.F_Calculate Trajectory` `Inaccuracy (half-degrees)`) "Undefined" "OverrideRootScale" (`Actor.GetOwner` (`self.GetOwner`)) Damage `Shot Upgrades` null))

(fn `F_Calculate Trajectory`
  (params (`Inaccuracy (half-deg)` :type "Float (double-precision)"))
  (returns (ReturnValue :type "Transform Structure"))
  (bind _sm_weapon (`self.SM Weapon`))
  (`/Engine/EditorBlueprintResources/StandardMacros.IsValid` _sm_weapon
    (:`Is Valid`
      (return (`KismetMathLibrary.MakeTransform` (+ (.location (`SceneComponent.GetSocketTransform` _sm_weapon "FireOrigin" "RTS_World")) (* (`SceneComponent.GetRightVector` (`self.SM Weapon`)) (`self.LocationOffset`))) (`KismetMathLibrary.ComposeRotators` (.rotation (`SceneComponent.GetSocketTransform` _sm_weapon "FireOrigin" "RTS_World")) (`KismetMathLibrary.MakeRotator` 0.0 0.0 (`KismetMathLibrary.RandomFloatInRange` (* `Inaccuracy (half-deg)` -1.0) `Inaccuracy (half-deg)`))))))))