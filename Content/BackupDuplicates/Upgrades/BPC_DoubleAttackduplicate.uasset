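; Weapon upgrade component, kept under BackupDuplicates, that adds a second, side-by-side projectile to attacks.
; UpgradeWeaponStat sets a sideways offset on the owner's BPC_SingleAttack component.
; UpgradeProjectile calculates a trajectory from the inaccuracy angle and spawns the given projectile type, offset the opposite way along the weapon mesh's right vector.
; The spawned projectile receives the owner, damage and shot upgrades.
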(event `self.Upgrade_WeaponStat`
  (set `/Game/Tech/Upgrades/BPC_SingleAttack.LocationOffset` 20.0 (`Actor.GetComponentByClass` (`self.GetOwner`) "/Game/Tech/Upgrades/BPC_SingleAttack.BPC_SingleAttack_C")))

(event `/Game/Tech/Upgrades/BPC_BaseUpgrade.Upgrade_Projectile`
  (params (`Inaccuracy (half-degrees)` :type "Float (double-precision)") (`Projectile Type` :type "/Game/Tech/Projectiles/BP_Projectile Class Reference") (Damage :type "Float (double-precision)") (`Shot Upgrades` :type "Array of /Game/Tech/Upgrades/BPC_ChainLightning Object Reference (by ref)"))
  (bind (_trajectory_location _trajectory_rotation) (`KismetMathLibrary.BreakTransform` (`self.Trajectory`)))
  (set `self.LocationOffset_Double` -20.0)
  (set `self.Trajectory` (`self.F_Calculate Trajectory` `Inaccuracy (half-degrees)`))
  (`|SpawnActorFromClass` `Projectile Type` (`KismetMathLibrary.MakeTransform` (+ _trajectory_location (* (`SceneComponent.GetRightVector` (`self.Weapon Mesh`)) (`self.LocationOffset_Double`))) _trajectory_rotation) "Undefined" "OverrideRootScale" (`self.GetOwner`) Damage `Shot Upgrades` null))