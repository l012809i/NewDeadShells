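; Glass Cannon upgrade component, a duplicate in a backup folder, that trades maximum health for attack power.
; UpgradePlayer reads the owner's health struct through an interface message and sends back a max health cut to a third.
; UpgradeWeaponStat casts the owner to BP_BaseWeapon and triples AttackPower in its WeaponInformation.
; Each event sits behind its own DoOnce, so neither change stacks on repeat calls.
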(event `self.Upgrade_Player`
  (`/Engine/EditorBlueprintResources/StandardMacros.DoOnce` false
    (:`Completed`
      (bind _health_struct (message `/Game/Tech/HealthSystem/BPI_DamageHandling.I_GetHealthStruct` (`self.GetOwner`)))
      (message `/Game/Tech/HealthSystem/BPI_DamageHandling.I_ChangeMaxHealth` (`self.GetOwner`) (/ (`.MaxHealth_5_66D911EB4E67FC9A695B02A3D74B2773` (break `/Game/Tech/HealthSystem/S_Health` _health_struct)) 3.0) null))))

(event `self.Upgrade_WeaponStat`
  (bind _weaponinformation (`/Game/Tech/Weapons/WeaponInfo/BP_BaseWeapon.WeaponInformation` (cast `/Game/Tech/Weapons/WeaponInfo/BP_BaseWeapon` (`self.GetOwner`) :!pure true)))
  (`/Engine/EditorBlueprintResources/StandardMacros.DoOnce` false
    (:`Completed`
      (setmembers `/Game/Tech/Weapons/WeaponInfo/WeaponInformation` :`StructRef` _weaponinformation :`Attack Power` (* (`.AttackPower_29_83DD24E64DC0231FDA6E81A1723EB3F5` (break `/Game/Tech/Weapons/WeaponInfo/WeaponInformation` _weaponinformation)) 3.0)))))