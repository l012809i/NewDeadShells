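; Weapon pickup actor that spins in place and shows an interact icon widget while overlapped.
; The construction script loads the Weapon enum's row from DT_Weapons, setting the mesh and centering it on its MidPoint socket.
; Interact sends the weapon's name, description and pickup reference to the player for UI.
; Addweapon passes the weapon class and slot to the player, destroying the pickup on success.
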(event `SpawnInformation`
  (params (`Weapon Name` :type "/Game/Tech/Weapons/E_WeaponNames Enum" :default "NewEnumerator4"))
  (bind _staticmesh (`self.StaticMesh`))
  (bind _returnvalue_location (`KismetMathLibrary.BreakTransform` (`SceneComponent.GetSocketTransform` _staticmesh "MidPoint" "RTS_Component")))
  (bind _returnvalue (`|GetDataTableRow` "/Game/Tech/Weapons/DT_Weapons.DT_Weapons" (`KismetStringLibrary.Conv_StringToName` (`|GetEnumeratorNameAsString` `Weapon Name`)))
    (:`then`
      (bind _output_get (set `self.Weapon Information` _returnvalue))
      (`StaticMeshComponent.SetStaticMesh` _staticmesh (`.WeaponMesh_17_79AEC6A248F23E731AEC6A8F2697B164` (break `/Game/Tech/Weapons/WeaponInfo/WeaponInformation` _output_get)))
      (`SceneComponent.K2_AddRelativeLocation` _staticmesh (* _returnvalue_location -1.0) false false))))

(event `self.Box.OnComponentBeginOverlap`
  (params (OverlappedComponent :type "PrimitiveComponent Object Reference") (OtherActor :type "Actor Object Reference") (OtherComp :type "PrimitiveComponent Object Reference") (OtherBodyIndex :type Integer) (bFromSweep :type Boolean) (SweepResult :type "HitResult Structure (by ref)"))
  ;[0.9922 0.6353 1] When the player gets near the pick up the interactable icon will appear
  (`SceneComponent.SetVisibility` (`self.Widget`) true false))

(event `/Game/Tech/Pickups/BPI_CharacterInteract.Interact`
  (params (Player :type "Actor Object Reference"))
  (bind ((`WeaponName_34_C3694ECA427C22994D707E9D808D1F6C` _weaponname) (`WeaponBlueprint_32_8A2FB0DD4C47CCCE3886D7BFCACBCC41` _weaponblueprint) (`WeaponDescription_37_B1D323954BAE511904601994C5853D22` _weapondescription)) (break `/Game/Tech/Weapons/WeaponInfo/WeaponInformation` (`self.Weapon Information`)))
  ;[0.9922 0.6353 1 0.9412] Sends to UI
  (message `/Game/Tech/Pickups/BPI_CharacterInteract.WeaponUIInteract` Player _weaponname self _weapondescription))

(event `/Game/Tech/Pickups/BPI_CharacterInteract.Addweapon`
  (params (Slot :type Integer))
  (bind _picked_up_ (message `/Game/Tech/Weapons/WeaponInfo/Test-BPI_Inventory.I_PickUpWeapon` (stale `/Game/Tech/Pickups/BPI_CharacterInteract.Interact` Player) (`.WeaponBlueprint_32_8A2FB0DD4C47CCCE3886D7BFCACBCC41` (break `/Game/Tech/Weapons/WeaponInfo/WeaponInformation` (`self.Weapon Information`))) Slot))
  (if _picked_up_
    (`self.K2_DestroyActor`)))

(event `self.Box.OnComponentEndOverlap`
  (params (OverlappedComponent :type "PrimitiveComponent Object Reference") (OtherActor :type "Actor Object Reference") (OtherComp :type "PrimitiveComponent Object Reference") (OtherBodyIndex :type Integer))
  ;[0.9922 0.6353 1] When the player gets near the pick up the interactable icon will appear
  (`SceneComponent.SetVisibility` (`self.Widget`) false false))

(event `self.ReceiveBeginPlay`
  (bind (_direction _alpha) (`Timeline|Rotation Timeline`)
    (:`Update`
      (`self.K2_SetActorRotation` (`KismetMathLibrary.RLerp` (struct) (struct :`Yaw` 360.0) _alpha)))))

(fn `I_CheckDuplicateWeapon`
  (params (`Weapon Class` :type "/Game/Tech/Weapons/WeaponInfo/BP_BaseWeapon Class Reference"))
  (returns (`Duplicate?` :type Boolean))
  (return false))

(fn `I_CheckFullInventory`
  (returns (`Full?` :type Boolean))
  (return false))

(fn `I_PickUpWeapon`
  (params (`Weapon Class` :type "/Game/Tech/Weapons/WeaponInfo/BP_BaseWeapon Class Reference") (Itemslot :type Integer))
  (returns (`Picked Up?` :type Boolean))
  (return false))

(fn `UserConstructionScript`
  (`self.SpawnInformation` (`self.Weapon`)))